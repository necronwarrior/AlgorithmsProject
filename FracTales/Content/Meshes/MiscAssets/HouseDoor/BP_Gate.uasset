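; BP_Gate is a double gate that swings open when its PuzzleSolved event fires.
; OpenGate plays the SwingOpen timeline, lerping the left and right hinges from their current relative rotation toward opposite 90-degree yaws.
; CloseDoors uses a separate SwingClosed timeline to lerp both hinges between zero and their current rotation, though nothing in this Blueprint calls it.
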(event `OpenGate`
  (bind _hingeleft (`self.HingeLeft`))
  (bind _hingeright (`self.HingeRight`))
  (bind (_returnvalue_location _returnvalue_rotation) (`KismetMathLibrary.BreakTransform` (`SceneComponent.GetRelativeTransform` _hingeright)))
  (bind (_returnvalue_location_2 _returnvalue_rotation_2) (`KismetMathLibrary.BreakTransform` (`SceneComponent.GetRelativeTransform` _hingeleft)))
  ;[1 1 1] Door Open away from player
  (bind (_direction _rotation) (`Timeline|Swing Open` :!via `PlayFromStart`)
    (:`Update`
      (`|ExecutionSequence`
        (:`then_0`
          (`SceneComponent.K2_SetRelativeRotation` _hingeleft (`KismetMathLibrary.RLerp` _returnvalue_rotation_2 (struct :`Yaw` 90.0) _rotation true) false false))
        (:`then_1`
          (`SceneComponent.K2_SetRelativeRotation` _hingeright (`KismetMathLibrary.RLerp` _returnvalue_rotation (struct :`Yaw` -90.0) _rotation true) false false))))))

(event `CloseDoors`
  (bind _hingeleft (`self.HingeLeft`))
  (bind _hingeright (`self.HingeRight`))
  (bind (_returnvalue_location _returnvalue_rotation) (`KismetMathLibrary.BreakTransform` (`SceneComponent.GetRelativeTransform` _hingeright)))
  (bind (_returnvalue_location_2 _returnvalue_rotation_2) (`KismetMathLibrary.BreakTransform` (`SceneComponent.GetRelativeTransform` _hingeleft)))
  ;[1 1 1] Door close when player away
  (bind (_direction _rotation) (`Timeline|Swing Closed` :!via `PlayFromStart`)
    (:`Update`
      (`|ExecutionSequence`
        (:`then_0`
          (`SceneComponent.K2_SetRelativeRotation` _hingeleft (`KismetMathLibrary.RLerp` (struct) _returnvalue_rotation_2 _rotation true) false false))
        (:`then_1`
          (`SceneComponent.K2_SetRelativeRotation` _hingeright (`KismetMathLibrary.RLerp` (struct) _returnvalue_rotation _rotation true) false false))))))

(event `/Game/Mechanics/CodeInjection/BPI_CodeInjectionInterface.PuzzleSolved`
  ;[1 1 1] Comment
  (`self.OpenGate`))

(fn `UserConstructionScript`)
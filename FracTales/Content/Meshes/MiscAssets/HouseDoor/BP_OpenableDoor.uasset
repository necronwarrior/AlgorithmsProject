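; A house door actor that swings open away from the first-person player and closes again when the player leaves.
; Box overlaps from the character's components tagged CanOpenDoors play Wwise open/close events and start the matching timeline, stopping the opposite one.
; The player's side in door-local space picks a ±90° yaw.
; Timelines blend from the hinge's current rotation each update, so interrupted swings continue from their present angle.
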(event `self.Box.OnComponentBeginOverlap`
  (params (OverlappedComponent :type "PrimitiveComponent Object Reference") (OtherActor :type "Actor Object Reference") (OtherComp :type "PrimitiveComponent Object Reference") (OtherBodyIndex :type Integer) (bFromSweep :type Boolean) (SweepResult :type "HitResult Structure (by ref)"))
  (bind _returnvalue (`self.K2_GetActorLocation`))
  (bind _hinge (`self.Hinge`))
  (bind (_returnvalue_location _returnvalue_rotation) (`KismetMathLibrary.BreakTransform` (`SceneComponent.GetRelativeTransform` _hinge)))
  (bind (_returnvalue_x _returnvalue_y) (`KismetMathLibrary.BreakVector` (`KismetMathLibrary.LessLess_VectorRotator` (- _returnvalue (`self.K2_GetActorLocation` OtherActor)) (`self.K2_GetActorRotation`))))
  ;[1 1 1] Door Open away from player
  (cast `/Game/Character/FirstPersonCharacter` OtherActor)
  (if (`ActorComponent.ComponentHasTag` OtherComp "CanOpenDoors")
    (`TimelineComponent.Stop` (`self.Swing Closed`))
    (set `self.OpenDirection` (< _returnvalue_y 0.0))
    ;;[1 1 1] Insert Audio functionality here
    (`AkGameplayStatics.PostEventAtLocation` "/Game/Audio/Wwise/Events/sfx/objects/non-destructable/door/door_open_start.door_open_start" _returnvalue)
    (bind (_direction _rotation) (`Timeline|Swing Open` :!via `PlayFromStart`)
      (:`Update`
        (`SceneComponent.K2_SetRelativeRotation` _hinge (`KismetMathLibrary.RLerp` _returnvalue_rotation (`KismetMathLibrary.MakeRotator` 0.0 0.0 (`KismetMathLibrary.SelectFloat` -90.0 90.0 (`self.OpenDirection`))) _rotation true) false false)))))

(event `self.Box.OnComponentEndOverlap`
  (params (OverlappedComponent :type "PrimitiveComponent Object Reference") (OtherActor :type "Actor Object Reference") (OtherComp :type "PrimitiveComponent Object Reference") (OtherBodyIndex :type Integer))
  (bind _hinge (`self.Hinge`))
  (bind (_returnvalue_location _returnvalue_rotation) (`KismetMathLibrary.BreakTransform` (`SceneComponent.GetRelativeTransform` _hinge)))
  ;[1 1 1] Door close when player away
  (cast `/Game/Character/FirstPersonCharacter` OtherActor)
  (if (`ActorComponent.ComponentHasTag` OtherComp "CanOpenDoors")
    (`TimelineComponent.Stop` (`self.Swing Open`))
    ;;[1 1 1] Insert Audio functionality here
    (`AkGameplayStatics.PostEventAtLocation` "/Game/Audio/Wwise/Events/sfx/objects/non-destructable/door/door_close_start.door_close_start" (`self.K2_GetActorLocation`))
    (bind (_direction _rotation) (`Timeline|Swing Closed` :!via `PlayFromStart`)
      (:`Update`
        (`SceneComponent.K2_SetRelativeRotation` _hinge (`KismetMathLibrary.RLerp` (struct) _returnvalue_rotation _rotation true) false false)))))

(fn `UserConstructionScript`)
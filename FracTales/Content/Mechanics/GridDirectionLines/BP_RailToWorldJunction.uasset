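; Rail-to-world junction that switches the first-person player between moving on rails and moving off them.
; An arrival event, or a player capsule overlap while active and flagged off-rails, toggles the mode from the RailCollider's collision state, repeating the off-rails enable after a short delay.
; Returning to rails clears the off-rails flag on all tagged junctions, but the call setting it is unwired.
; Solving a puzzle activates the junction.
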(event `self.ReceiveActorBeginOverlap`
  (params (OtherActor :type "Actor Object Reference"))
  (`parent.ReceiveActorBeginOverlap` OtherActor))

(event `RailToWorldArrived`
  ;[1 1 1] Take player on and off rails
  (bind _asfirst_person_character (cast `/Game/Character/FirstPersonCharacter` (`GameplayStatics.GetPlayerCharacter` 0) :!label _label))
  (switch `ECollisionEnabled` (`PrimitiveComponent.GetCollisionEnabled` (`/Game/Character/FirstPersonCharacter.RailCollider` _asfirst_person_character))
    (:`NoCollision`
      (`/Game/Character/FirstPersonCharacter.DisableOffRails` _asfirst_person_character self)
      (`self.SetIsPlayerOffRails?` false))
    (:`QueryOnly`
      (`/Game/Character/FirstPersonCharacter.EnableOffRails` _asfirst_person_character :!label _label_2)
      (`KismetSystemLibrary.Delay` 0.5)
      (`/Game/Character/FirstPersonCharacter.EnableOffRails` _asfirst_person_character))
    (:`PhysicsOnly`
      (goto _label_2))
    (:`QueryAndPhysics`
      (goto _label_2))))

(event `self.Capsule.OnComponentBeginOverlap`
  (params (OverlappedComponent :type "PrimitiveComponent Object Reference") (OtherActor :type "Actor Object Reference") (OtherComp :type "PrimitiveComponent Object Reference") (OtherBodyIndex :type Integer) (bFromSweep :type Boolean) (SweepResult :type "HitResult Structure (by ref)"))
  ;[1 1 1] Take player on and off rails
  (if (and (`ActorComponent.ComponentHasTag` OtherComp "Player") (`self.bPlayerIsOffRails`) (`self.bIsActive?`))
    (goto _label)))

(event `/Game/Mechanics/CodeInjection/BPI_CodeInjectionInterface.PuzzleSolved`
  (set `self.bIsActive?` true))

(fn `UserConstructionScript`
  (`parent.UserConstructionScript`))
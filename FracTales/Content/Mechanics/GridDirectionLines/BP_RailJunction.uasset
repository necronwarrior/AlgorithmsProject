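; Rail junction node that carries the player along a grid of linked junctions.
; On arrival it recalculates the player's beam layout and enables input; W picks one of four neighbours by relative yaw, if active.
; Tick lerps the player there at constant speed, then hands control to that junction.
; Character events reactivate junctions each new day and swap materials to show deactivated ones.
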(event `self.ReceiveBeginPlay`
  ;[1 1 1] Bind events and create failsafes for input management
  (`self.DisableInput` (`GameplayStatics.GetPlayerController` 0))
  (`self.SetActorTickEnabled` false)
  (bind _asfirst_person_character (cast `/Game/Character/FirstPersonCharacter` (`GameplayStatics.GetPlayerCharacter` 0)))
  (add `/Game/Character/FirstPersonCharacter.CallNextDay` _asfirst_person_character (delegate `SetActiveOnNewDay`))
  (add `/Game/Character/FirstPersonCharacter.JunctionsDeactivated` _asfirst_person_character (delegate `DeactivatedChanges`)))

(event `SetActiveOnNewDay`
  ;[1 1 1] Set all junctions active
  (set `self.bIsActive?` true))

(event `DeactivatedChanges`
  (bind _cylinder (`self.Cylinder`))
  ;[1 1 1] Make changes based on which rails are active or inactive
  (if (`self.bIsActive?`)
    (`PrimitiveComponent.SetMaterial` _cylinder 0 "/Engine/BasicShapes/BasicShapeMaterial.BasicShapeMaterial")
    (else
      (`PrimitiveComponent.SetMaterial` _cylinder 0 "/Engine/VREditor/LaserPointer/LaserPointerMaterialInst.LaserPointerMaterialInst"))))

(event `Arrived`
  ;[1 1 1] Place player onto rails on clollision or when passed too
  (`/Game/Character/FirstPersonCharacter.RecalculateBeamLayout` (stale `self.Box.OnComponentBeginOverlap` _asfirst_person_character) :!label _label)
  (`self.EnableInput` (`GameplayStatics.GetPlayerController` 0))
  (goto _label_2 :!via `Reset`))

(event `self.Box.OnComponentBeginOverlap`
  (params (OverlappedComponent :type "PrimitiveComponent Object Reference") (OtherActor :type "Actor Object Reference") (OtherComp :type "PrimitiveComponent Object Reference") (OtherBodyIndex :type Integer) (bFromSweep :type Boolean) (SweepResult :type "HitResult Structure (by ref)"))
  ;[1 1 1] Place player onto rails on clollision or when passed too
  (if (`ActorComponent.ComponentHasTag` OtherComp "Player")
    (bind _asfirst_person_character (cast `/Game/Character/FirstPersonCharacter` OtherActor))
    (set `self.PlayerCharacter` _asfirst_person_character)
    (set `/Game/Character/FirstPersonCharacter.CurrentJunction` self _asfirst_person_character)
    (if (`self.bIsFirstPoint?`)
      (goto _label))))

(event `Key|W`
  (params (Key :type "Key Structure" :default "AnyKey"))
  (bind (_returnvalue_roll _returnvalue_pitch _returnvalue_yaw) (`KismetMathLibrary.BreakRotator` (`SceneComponent.K2_GetComponentRotation` (`self.DefaultSceneRoot`))))
  (bind (_returnvalue_roll_2 _returnvalue_pitch_2 _returnvalue_yaw_2) (`KismetMathLibrary.BreakRotator` (`SceneComponent.K2_GetComponentRotation` (`Actor.RootComponent` (`self.PlayerCharacter`)))))
  (bind _returnvalue (- _returnvalue_yaw _returnvalue_yaw_2))
  ;[1 1 1] Junction Selection
  (:`Pressed`
    (if (`KismetMathLibrary.InRange_FloatFloat` _returnvalue -135.0 -45.0 false)
      (`self.IsThisJunctionActive?` 0
        (:`Out`
          (`/Engine/EditorBlueprintResources/StandardMacros.DoOnce` false :!label _label_2
            (:`Completed`
              (set `self.JunctionChoice` (`self.JunctionPreChoice`))
              (`self.SetActorTickEnabled` true)))))
      (elif (or (`KismetMathLibrary.InRange_FloatFloat` _returnvalue -180.0 -135.0) (`KismetMathLibrary.InRange_FloatFloat` _returnvalue 135.0 360.0))
        (`self.IsThisJunctionActive?` 1
          (:`Out`
            (goto _label_2)))
        (elif (`KismetMathLibrary.InRange_FloatFloat` _returnvalue 45.0 135.0 true false)
          (`self.IsThisJunctionActive?` 2
            (:`Out`
              (goto _label_2)))
          (elif (or (`KismetMathLibrary.InRange_FloatFloat` _returnvalue 0.0 45.0 true false) (`KismetMathLibrary.InRange_FloatFloat` _returnvalue -45.0 0.0 false))
            (`self.IsThisJunctionActive?` 3
              (:`Out`
                (goto _label_2)))))))))

(event `self.ReceiveTick`
  (params (DeltaSeconds :type "Float (single-precision)"))
  (bind (_returnvalue_x _returnvalue_y) (`KismetMathLibrary.BreakVector` (`self.K2_GetActorLocation`)))
  (bind (_returnvalue_x_2 _returnvalue_y_2 _returnvalue_z) (`KismetMathLibrary.BreakVector` (`self.K2_GetActorLocation` (`self.PlayerCharacter`))))
  (bind _output (`|GetArrayItem` (`self.JunctionList`) (`self.JunctionChoice`)))
  (bind _output_2 (`|GetArrayItem` (`self.JunctionList`) (`self.JunctionChoice`)))
  ;[1 1 1] Move the player from junction to junction
  (set `self.DeltaTime` DeltaSeconds)
  (set `self.PlayerZ` _returnvalue_z)
  (if (`PrimitiveComponent.IsOverlappingComponent` (`/Game/Mechanics/GridDirectionLines/BP_RailJunction.Box` _output_2) (`|GetArrayItem` (`self.GetComponentsByTag` (`self.PlayerCharacter`) "/Script/Engine.PrimitiveComponent" "RailBase")))
    (`self.K2_SetActorLocation` (`self.PlayerCharacter`) (`KismetMathLibrary.MakeVector` (.x (`self.K2_GetActorLocation` _output_2)) (.y (`self.K2_GetActorLocation` _output_2)) (`self.PlayerZ`)) false false)
    (`self.SetActorTickEnabled` false)
    (`self.Arrived` (`|GetArrayItem` (`self.JunctionList`) (`self.JunctionChoice`)))
    (set `self.bIsFirstPoint?` false)
    (set `self.DeltaTimeBuildup` 0.0)
    (`self.DisableInput` (`GameplayStatics.GetPlayerController` 0))
    (else
      (set `self.DeltaTimeBuildup` (+ (* (`self.DeltaTime`) 700.0) (`self.DeltaTimeBuildup`)))
      (`self.K2_SetActorLocation` (`self.PlayerCharacter`) (`KismetMathLibrary.VLerp` (`KismetMathLibrary.MakeVector` _returnvalue_x _returnvalue_y (`self.PlayerZ`)) (`KismetMathLibrary.MakeVector` (.x (`self.K2_GetActorLocation` _output)) (.y (`self.K2_GetActorLocation` _output)) (`self.PlayerZ`)) (`KismetMathLibrary.FClamp` (/ (`self.DeltaTimeBuildup`) (`KismetMathLibrary.VSize` (- (`self.K2_GetActorLocation` _output) (`self.K2_GetActorLocation`)))))) false false))))

(fn `UserConstructionScript`)
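; BP_HighlightedObject is a static mesh object that can show a highlight while the player looks at it from close range.
; Every Tick it runs its own short Visibility line trace from slightly above the player character's location along the control rotation.
; When OutlineOnFocus is set, it turns the mesh's Render Custom Depth on if the trace hits this actor and off otherwise.
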(event `self.ReceiveTick`
  (params (DeltaSeconds :type "Float (single-precision)"))
  (bind _returnvalue (`GameplayStatics.GetPlayerCharacter` 0))
  (bind _returnvalue_2 (`KismetMathLibrary.MakeVector` (.x (`self.K2_GetActorLocation` _returnvalue)) (.y (`self.K2_GetActorLocation` _returnvalue)) (+ (.z (`self.K2_GetActorLocation` _returnvalue)) 50.0)))
  (bind _outhit (`KismetSystemLibrary.LineTraceSingle` :`Start` _returnvalue_2 :`End` (+ _returnvalue_2 (* (`KismetMathLibrary.GetForwardVector` (`Pawn.GetControlRotation` _returnvalue)) 250.0)) :`TraceChannel` "TraceTypeQuery1" :`bIgnoreSelf` false))
  (if (== (`.HitActor` (`GameplayStatics.BreakHitResult` _outhit)) self)
    ;[1 1 1] Comment
    (if (`self.bOutlineOnFocus`)
      (`PrimitiveComponent.SetRenderCustomDepth` (`self.StaticMeshComponent`) true))
    (elif (`self.bOutlineOnFocus`)
      (`PrimitiveComponent.SetRenderCustomDepth` (`self.StaticMeshComponent`) false))))

(fn `UserConstructionScript`)
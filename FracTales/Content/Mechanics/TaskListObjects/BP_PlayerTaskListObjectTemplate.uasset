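; Base template Blueprint for a world object that represents a task on the player's task list.
; At BeginPlay and on the character's next-day event it resets text visibility and collision from per-task start flags, then finds the closest BP_RailJunction with an expanding sphere overlap.
; Clicks store the player behind a DoOnce, which reopens when TaskFinished marks the task complete in the player's list.
; Text labels can be toggled by tag.
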(event `self.ReceiveBeginPlay`
  (bind _bisactiveatstart_ (`self.bIsActiveAtStart?`))
  (bind _asfirst_person_character (cast `/Game/Character/FirstPersonCharacter` (`GameplayStatics.GetPlayerCharacter` 0)))
  (add `/Game/Character/FirstPersonCharacter.CallNextDay` _asfirst_person_character (delegate `NextDayReset`))
  (for (_array_element _array_index) (`SceneComponent.GetChildrenComponents` (`self.DefaultSceneRoot`) false) :!label _label
    (if (== (`GameplayStatics.GetObjectClass` _array_element) "/Script/Engine.TextRenderComponent")
      (`SceneComponent.SetVisibility` _array_element (`|GetArrayItem` _bisactiveatstart_ _array_index) true)
      (`self.SetActorEnableCollision` (`|GetArrayItem` _bisactiveatstart_))))
  (bind (_outactors _returnvalue) (`KismetSystemLibrary.SphereOverlapActors` (`self.K2_GetActorLocation` self) (`self.SphereSize`) (`|MakeArray` "ObjectTypeQuery2" :!type "EObjectTypeQuery Enum") "/Game/Mechanics/GridDirectionLines/BP_RailJunction.BP_RailJunction_C" :!label _label_2))
  (if _returnvalue
    (if (== (`KismetArrayLibrary.Array_Length` _outactors) 1)
      (bind _asbp_rail_junction (cast `/Game/Mechanics/GridDirectionLines/BP_RailJunction` (`|GetArrayItem` _outactors)))
      (set `self.ClosestRailJunction` _asbp_rail_junction)
      (else
        (for _array_element_2 _outactors
          (bind _returnvalue_2 (`KismetMathLibrary.VSize` (- (`self.K2_GetActorLocation` _array_element_2) (`self.K2_GetActorLocation` self))))
          (if (< _returnvalue_2 (`self.ClosestJunctionMagnitude`))
            (set `self.ClosestJunctionMagnitude` _returnvalue_2)
            (bind _asbp_rail_junction_2 (cast `/Game/Mechanics/GridDirectionLines/BP_RailJunction` _array_element_2))
            (set `self.ClosestRailJunction` _asbp_rail_junction_2)))))
    (else
      (`/Engine/EditorBlueprintResources/StandardMacros.IncrementFloat` (`self.SphereSize`)
        (:`  `
          (goto _label_2))))))

(event `NextDayReset`
  (goto _label))

(event `PlayerClick`
  (params (PlayerCharacter :type "/Game/Character/FirstPersonCharacter Object Reference") (TagFunctionality :type Name))
  ;[1 1 1] Check that this task is the next task to perform - at least compared to the last task
  (set `self.PlayerCharacterReference` PlayerCharacter)
  (`/Engine/EditorBlueprintResources/StandardMacros.DoOnce` false :!label _label_3))

(event `TaskFinished`
  ;[1 1 1] When task is completed set its corresponding value in the player's checklist to true and change colour
  (`/Game/Character/FirstPersonCharacter.SetTaskListComlpeteIndex` (`self.PlayerCharacterReference`) (`self.PositionInTaskList`))
  (goto _label_3 :!via `Reset`))

(event `ToggleTextVisibility`
  (params (TaskName :type Name))
  (for _array_element (`self.K2_GetComponentsByClass` self "/Script/Engine.TextRenderComponent")
    (if (`KismetArrayLibrary.Array_Contains` (`ActorComponent.ComponentTags` _array_element) TaskName)
      (`SceneComponent.ToggleVisibility` _array_element false))))

(fn `UserConstructionScript`)
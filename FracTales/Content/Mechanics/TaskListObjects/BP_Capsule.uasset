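; BP_Capsule is a clickable task-list object whose two beams cycle through four blue and red color combinations.
; A click advances a wrapping state counter, which picks both beam materials and applies them to two material slots on the static mesh.
; Each click also stops delayed dialogue on the first partner dialogue manager found in the level.
; BeginPlay caches the initial beam materials, and GetMaterials exposes the current pair.
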(event `self.ReceiveBeginPlay`
  (bind _returnvalue (`MeshComponent.GetMaterials` (`self.StaticMeshComponent`)))
  (set `self.Beam1Material` (`|GetArrayItem` _returnvalue 1))
  (set `self.Beam2Material` (`|GetArrayItem` _returnvalue 2)))

(event `SetBeamMaterials`
  (bind _staticmeshcomponent (`self.StaticMeshComponent`))
  (`PrimitiveComponent.SetMaterial` _staticmeshcomponent 1 (`self.Beam1Material`))
  (`PrimitiveComponent.SetMaterial` _staticmeshcomponent 2 (`self.Beam2Material`)))

(event `NextState`
  (bind _result (`/Engine/EditorBlueprintResources/StandardMacros.IncrementInt` (`self.CurrentState`))
    (:`  `
      (bind _output_get (set `self.CurrentState` _result))
      (if (> _output_get 3)
        (set `self.CurrentState` 0))
      (switch `int` (`self.CurrentState`)
        (:`0`
          (set `self.Beam1Material` "/Game/Assets/Lamp/BlueBeam.BlueBeam")
          (set `self.Beam2Material` "/Game/Assets/Lamp/BlueBeam.BlueBeam"))
        (:`1`
          (set `self.Beam1Material` "/Game/Assets/Lamp/RedBeam.RedBeam")
          (set `self.Beam2Material` "/Game/Assets/Lamp/BlueBeam.BlueBeam"))
        (:`2`
          (set `self.Beam1Material` "/Game/Assets/Lamp/BlueBeam.BlueBeam")
          (set `self.Beam2Material` "/Game/Assets/Lamp/RedBeam.RedBeam"))
        (:`3`
          (set `self.Beam1Material` "/Game/Assets/Lamp/RedBeam.RedBeam")
          (set `self.Beam2Material` "/Game/Assets/Lamp/RedBeam.RedBeam")))
      (`self.SetBeamMaterials`))))

(event `PlayerClick`
  (`self.NextState`)
  (bind _outactors (`GameplayStatics.GetAllActorsOfClass` "/Game/DialogueSystem/PartnerConversations/BP_PartnerDialogueManager.BP_PartnerDialogueManager_C"))
  (`/Game/DialogueSystem/PartnerConversations/BP_PartnerDialogueManager.StopDelayedDialogue` (`|GetArrayItem` _outactors)))

(fn `GetMaterials`
  (returns (Beam1Material :type "MaterialInterface Object Reference") (Beam2Material :type "MaterialInterface Object Reference"))
  (return (`self.Beam1Material`) (`self.Beam2Material`)))

(fn `UserConstructionScript`)
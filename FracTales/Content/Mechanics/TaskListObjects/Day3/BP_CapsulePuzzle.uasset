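; BP_CapsulePuzzle is a Day 3 task-list puzzle that completes when three capsules show the correct beam color combination.
; BeginPlay casts three child actors to BP_Capsule and caches the references.
; Tick polls each capsule's two beam materials against a fixed red/blue pattern and calls TaskFinished every frame they all match, with no one-shot guard.
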(event `self.ReceiveBeginPlay`
  (`parent.ReceiveBeginPlay`)
  (bind _asbp_capsule (cast `/Game/BP_Capsule` (`ChildActorComponent.ChildActor` (`self.ChildActor`))))
  (set `self.Capsule1` _asbp_capsule)
  (bind _asbp_capsule_2 (cast `/Game/BP_Capsule` (`ChildActorComponent.ChildActor` (`self.ChildActor1`))))
  (set `self.Capsule2` _asbp_capsule_2)
  (bind _asbp_capsule_3 (cast `/Game/BP_Capsule` (`ChildActorComponent.ChildActor` (`self.ChildActor2`))))
  (set `self.Capsule3` _asbp_capsule_3))

(event `self.ReceiveTick`
  (params (DeltaSeconds :type "Float (single-precision)"))
  (bind (_beam1material _beam2material) (`/Game/BP_Capsule.GetMaterials` (`self.Capsule1`)))
  (if (and (== _beam1material "/Game/Assets/Lamp/RedBeam.RedBeam") (== _beam2material "/Game/Assets/Lamp/RedBeam.RedBeam"))
    (bind (_beam1material_2 _beam2material_2) (`/Game/BP_Capsule.GetMaterials` (`self.Capsule2`)))
    (if (and (== _beam1material_2 "/Game/Assets/Lamp/BlueBeam.BlueBeam") (== _beam2material_2 "/Game/Assets/Lamp/RedBeam.RedBeam"))
      (bind (_beam1material_3 _beam2material_3) (`/Game/BP_Capsule.GetMaterials` (`self.Capsule3`)))
      (if (and (== _beam1material_3 "/Game/Assets/Lamp/BlueBeam.BlueBeam") (== _beam2material_3 "/Game/Assets/Lamp/BlueBeam.BlueBeam"))
        (`self.TaskFinished`)))))

(fn `UserConstructionScript`
  (`parent.UserConstructionScript`))
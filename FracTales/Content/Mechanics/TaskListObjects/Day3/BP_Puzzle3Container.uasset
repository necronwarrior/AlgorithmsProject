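; Day 3 puzzle container that tracks terminal clicks, which must arrive in numbered order.
; A correct click advances a counter and a wrong one resets all terminals.
; Completion disables widget input, finishes the task, plays a Wwise event, reactivates tagged laser fences and starts EndingObject's ending.
; An older endgame sequence with red screen fade and player slowdown remains, but is unwired, with Tick disabled.
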(event `self.ReceiveBeginPlay`
  (`parent.ReceiveBeginPlay`)
  (`self.SetActorTickEnabled` false))

(event `self.ReceiveTick`
  (params (DeltaSeconds :type "Float (single-precision)"))
  (bind _charactermovement (`Character.CharacterMovement` (cast `/Game/Character/FirstPersonCharacter` (`GameplayStatics.GetPlayerCharacter` 0) :!pure true)))
  (if (`self.EndgameBool`)
    (bind _output_get (set `self.DeltaTime` (+ (/ DeltaSeconds 8.0) (`self.DeltaTime`))))
    (`MaterialInstanceDynamic.SetScalarParameterValue` (`self.EndgameRedStatic`) "Opacity" _output_get)
    (set `CharacterMovementComponent.MaxWalkSpeed` (- (`CharacterMovementComponent.MaxWalkSpeed` _charactermovement) (* 10 (`self.DeltaTime`))) _charactermovement)))

(event `TerminalClicked`
  (params (NumberInList :type Integer))
  (if (== NumberInList (`self.AdditiveList`))
    (bind _result (`/Engine/EditorBlueprintResources/StandardMacros.IncrementInt` (`self.AdditiveList`))
      (:`  `
        (if (== _result 5)
          (`self.DisableWidgetInput`)
          (`self.TaskFinished`)
          (`AkGameplayStatics.PostEventAtLocation` "/Game/Audio/Wwise/Events/sfx/objects/non-destructable/puzzles/puzzle_03/puzzle03_complete.puzzle03_complete" (`self.K2_GetActorLocation`))
          (bind _outactors (`GameplayStatics.GetAllActorsWithTag` "LaserFence"))
          (for _array_element _outactors
            (bind _asbp_laser_fence_new (cast `/Game/Mechanics/TaskListObjects/BP_LaserFenceNew` _array_element))
            (`/Game/Mechanics/TaskListObjects/BP_LaserFenceNew.Reactivate` _asbp_laser_fence_new))
          ;[1 1 1] Begin ending sequence
          (`/Game/EndgameSequence/BP_signpost.PlayEnding` (`self.EndingObject`)))))
    (else
      (`self.ResetTerminals`)
      (set `self.AdditiveList` 1))))

(fn `UserConstructionScript`)
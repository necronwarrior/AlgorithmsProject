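; BP_Radio is a Day 1 task-list object representing a radio that the player clicks to complete a task.
; Its PlayerClick event runs the parent behavior, then calls TaskFinished.
; Every tick, it rotates its TextRender to face the first-person character's camera, so the label always points at the player.
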(event `self.PlayerClick`
  (params (PlayerCharacter :type "/Game/Character/FirstPersonCharacter Object Reference") (TagFunctionality :type Name))
  (`parent.PlayerClick` PlayerCharacter TagFunctionality)
  (`self.TaskFinished`))

(event `self.ReceiveTick`
  (params (DeltaSeconds :type "Float (single-precision)"))
  (bind _textrender (`self.TextRender`))
  (bind _asfirst_person_character (cast `/Game/Character/FirstPersonCharacter` (`GameplayStatics.GetPlayerCharacter` 0)))
  (`SceneComponent.K2_SetWorldRotation` _textrender (`KismetMathLibrary.FindLookAtRotation` (`SceneComponent.K2_GetComponentLocation` _textrender) (`SceneComponent.K2_GetComponentLocation` (`/Game/Character/FirstPersonCharacter.FirstPersonCamera` _asfirst_person_character))) false false))

(fn `UserConstructionScript`
  (`parent.UserConstructionScript`))
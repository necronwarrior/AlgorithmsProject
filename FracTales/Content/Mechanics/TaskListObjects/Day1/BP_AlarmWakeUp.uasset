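; Day 1 alarm clock task object that rings through Wwise on BeginPlay and handles the player's wake-up, sleep-alarm and day-reset interactions.
; PlayerClick branches on a functionality tag, finishing tasks, playing wake or sleep level sequences, and moving the player between sleep and wake points.
; Waking stops the alarm and restores input after a fixed delay; resetting waits out the sleep sequence, calls ResetDay and restarts the alarm.
; Tick turns its text render toward the first-person camera.
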(event `self.ReceiveBeginPlay`
  (bind _returnvalue (`self.K2_GetActorLocation`))
  (`parent.ReceiveBeginPlay`)
  (`AkGameplayStatics.PostEventAtLocation` "/Game/Audio/Wwise/Events/sfx/objects/non-destructable/alarm_clock/alarm_clock_start.alarm_clock_start" _returnvalue)
  (`AkGameplayStatics.SetRTPCValue` "alarm_clock_volume" 1.0)
  (`AkGameplayStatics.PostEventAtLocation` "/Game/Audio/Wwise/Events/UI/Prompts/complete_all_tasks.complete_all_tasks" _returnvalue))

(event `self.PlayerClick`
  (params (PlayerCharacter :type "/Game/Character/FirstPersonCharacter Object Reference") (TagFunctionality :type Name))
  (bind _returnvalue (`GameplayStatics.GetPlayerCharacter` 0))
  (bind _returnvalue_2 (`GameplayStatics.GetPlayerController` 0))
  (bind _sequenceplayer (`LevelSequenceActor.SequencePlayer` (`self.SleepSequence`)))
  (bind _sequenceplayer_2 (`LevelSequenceActor.SequencePlayer` (`self.WakeUpSequence`)))
  (bind _sequenceplayer_3 (`LevelSequenceActor.SequencePlayer` (`self.SleepSequence`)))
  ;[1 1 1] Check If this is next task, space for any other checks
  (`parent.PlayerClick` PlayerCharacter TagFunctionality)
  (switch `name` TagFunctionality
    (:`WakeUpAlarmClock`
      ;[1 1 1] Waking Up Functionality
      (`|ExecutionSequence`
        (:`then_0`
          (`/Engine/EditorBlueprintResources/StandardMacros.DoOnce` false
            (:`Completed`
              (`SceneComponent.K2_AddWorldOffset` (`/Game/Character/FirstPersonCharacter.FirstPersonCamera` PlayerCharacter) (0.0 0.0 40.0) false true))))
        (:`then_1`
          (`AkGameplayStatics.SetRTPCValue` "alarm_clock_volume")
          (`AkGameplayStatics.PostEventAtLocation` "/Game/Audio/Wwise/Events/sfx/objects/non-destructable/alarm_clock/alarm_clock_stop.alarm_clock_stop" (`self.K2_GetActorLocation`))
          (`AkGameplayStatics.PostEventAtLocation` "/Game/Audio/Wwise/Events/UI/Tasks/task_updated.task_updated" (`self.K2_GetActorLocation` (`GameplayStatics.GetPlayerCharacter` 0)))
          (`self.K2_SetActorRotation` :`self` PlayerCharacter)
          (`/Game/Character/FirstPersonCharacter.SetControlStructure` PlayerCharacter "NewEnumerator3")
          (`self.TaskFinished`)
          (`AkGameplayStatics.SetState` "location" "inside")
          (`self.DisableInput` PlayerCharacter _returnvalue_2)
          (`MovieSceneSequencePlayer.SetPlaybackPosition` _sequenceplayer_2 0.0)
          (`MovieSceneSequencePlayer.Play` _sequenceplayer_2)
          (`KismetSystemLibrary.Delay` 5.0)
          (`self.K2_SetActorLocation` _returnvalue (.location (`self.GetTransform` (`self.WakeupPoint`))) false false)
          (`Controller.SetControlRotation` _returnvalue_2 (.rotation (`self.GetTransform` (`self.WakeupPoint`))))
          (bind _asfirst_person_character (cast `/Game/Character/FirstPersonCharacter` _returnvalue))
          (set `/Game/Character/FirstPersonCharacter.bIsLyingDown?` false _asfirst_person_character)
          (`self.EnableInput` _asfirst_person_character _returnvalue_2)
          (`PrimitiveComponent.SetCollisionEnabled` (`/Game/Character/FirstPersonCharacter.RailCollider` _asfirst_person_character) "QueryOnly"))))
    (:`SetSleepAlarm`
      ;[1 1 1] Set alarm for falling asleep in the bed without resetting the day
      (`self.TaskFinished`)
      (`MovieSceneSequencePlayer.SetPlaybackPosition` _sequenceplayer_3 0.0)
      (`MovieSceneSequencePlayer.Play` _sequenceplayer_3)
      (`/Game/Character/FirstPersonCharacter.Change Task List` PlayerCharacter))
    (:`ResetDay`
      ;[1 1 1] Fall asleep in the bed and reset the day
      (`self.K2_TeleportTo` :`self` PlayerCharacter :`DestLocation` (`self.K2_GetActorLocation` (`self.SleepPoint`)))
      (`MovieSceneSequencePlayer.SetPlaybackPosition` _sequenceplayer 0.0)
      (`MovieSceneSequencePlayer.Play` _sequenceplayer)
      (`self.K2_SetActorLocation` PlayerCharacter (.location (`self.GetTransform` (`self.SleepPoint`))) false false)
      (`Controller.SetControlRotation` (`GameplayStatics.GetPlayerController` 0) (.rotation (`self.GetTransform` (`self.SleepPoint`))))
      (set `/Game/Character/FirstPersonCharacter.bIsLyingDown?` true PlayerCharacter)
      (`KismetSystemLibrary.Delay` (`MovieSceneSequencePlayer.GetLength` _sequenceplayer))
      (`/Game/Character/FirstPersonCharacter.Reset Day` PlayerCharacter)
      (`AkGameplayStatics.PostEventAtLocation` "/Game/Audio/Wwise/Events/sfx/objects/non-destructable/alarm_clock/alarm_clock_start.alarm_clock_start" (`self.K2_GetActorLocation`))
      (`AkGameplayStatics.SetRTPCValue` "alarm_clock_volume" 1.0))))

(event `self.ReceiveTick`
  (params (DeltaSeconds :type "Float (single-precision)"))
  (bind _textrender (`self.TextRender`))
  (bind _asfirst_person_character (cast `/Game/Character/FirstPersonCharacter` (`GameplayStatics.GetPlayerCharacter` 0)))
  (bind (_returnvalue_roll _returnvalue_pitch _returnvalue_yaw) (`KismetMathLibrary.BreakRotator` (`KismetMathLibrary.FindLookAtRotation` (`SceneComponent.K2_GetComponentLocation` _textrender) (`SceneComponent.K2_GetComponentLocation` (`/Game/Character/FirstPersonCharacter.FirstPersonCamera` _asfirst_person_character)))))
  (`SceneComponent.K2_SetWorldRotation` _textrender (`KismetMathLibrary.MakeRotator` 90.0 _returnvalue_pitch _returnvalue_yaw) false false))

(fn `UserConstructionScript`
  (`parent.UserConstructionScript`))
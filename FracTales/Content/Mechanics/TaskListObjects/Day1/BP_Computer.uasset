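; Task-list computer that the player clicks to do a Computer task, then a Mail task, on in-world screen widgets.
; Clicking blends to a fixed camera with mouse input, while Tick polls widget completion and faces text at the player.
; Finishing Mail respawns the actor with the Day 142 report, restores first-person control and, on day 1, updates a rail junction.
; OnDayReset restores the first screen and re-arms the click gates.
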(event `OnDayReset`
  (bind _returnvalue (`GameplayStatics.GetPlayerController` 0))
  (bind _returnvalue_2 (`GameplayStatics.GetPlayerController` 0))
  (bind _tasklistw (`self.TaskListW`))
  (bind _widget (`self.Widget`))
  (bind (_returnvalue_x _returnvalue_y _returnvalue_z) (`KismetMathLibrary.BreakVector` (`SceneComponent.K2_GetComponentLocation` _widget)))
  (`KismetSystemLibrary.PrintString` "Hello")
  (`ActorComponent.SetActive` _widget true false)
  (`SceneComponent.SetVisibility` _widget true false)
  (`SceneComponent.K2_SetWorldLocation` _widget (`KismetMathLibrary.MakeVector` _returnvalue_x _returnvalue_y (- _returnvalue_z 300.0)) false false)
  (bind _asbp_task_list_widget_day_141 (cast `/Game/HUD/TaskListElements/BP_TaskListWidgetDay141` (`WidgetComponent.GetUserWidgetObject` _tasklistw)))
  (`Image.SetBrushFromMaterial` (`/Game/HUD/TaskListElements/BP_TaskListWidgetDay141.Image_195` _asbp_task_list_widget_day_141) "/Game/HUD/TaskListElements/Day_142_Report_1_Blue_Mat.Day_142_Report_1_Blue_Mat")
  (set `/Game/HUD/TaskListElements/BP_TaskListWidgetDay141.bIsDay142?` true _asbp_task_list_widget_day_141)
  (`ActorComponent.SetActive` _tasklistw false false)
  (`SceneComponent.SetVisibility` _tasklistw false false)
  (`|ExecutionSequence`
    (:`then_0`
      (goto _label :!via `Reset`))
    (:`then_1`
      (goto _label_2 :!via `Reset`))))

(event `self.PlayerClick`
  (params (PlayerCharacter :type "/Game/Character/FirstPersonCharacter Object Reference") (TagFunctionality :type Name))
  (bind _returnvalue (`GameplayStatics.GetPlayerController` 0))
  (bind _returnvalue_2 (`GameplayStatics.GetPlayerController` 0))
  (bind _widget (`self.Widget`))
  (bind _tasklistw (`self.TaskListW`))
  (bind (_returnvalue_x _returnvalue_y _returnvalue_z) (`KismetMathLibrary.BreakVector` (`SceneComponent.K2_GetComponentLocation` _widget)))
  (set `self.CurrentTask` TagFunctionality)
  (`parent.PlayerClick` PlayerCharacter TagFunctionality)
  (switch `name` TagFunctionality
    (:`Computer`
      (`|ExecutionSequence`
        (:`then_0`
          (`/Engine/EditorBlueprintResources/StandardMacros.DoOnce` false :!label _label
            (:`Completed`
              (bind _unique_actor (`/Game/MacroLibrary/BML_ActorUtilities.GetActorWithUniqueTag` "ComputerCamera"))
              (`PlayerController.SetViewTargetWithBlend` _returnvalue _unique_actor 0.5 "VTBlend_Linear" 0.0 true)
              (bind _asfirst_person_character (cast `/Game/Character/FirstPersonCharacter` (`GameplayStatics.GetPlayerCharacter` 0)))
              (set `WidgetInteractionComponent.InteractionSource` "Mouse" (`/Game/Character/FirstPersonCharacter.WidgetInteraction` _asfirst_person_character))
              (`WidgetBlueprintLibrary.SetInputMode_GameAndUIEx` _returnvalue (`WidgetComponent.GetUserWidgetObject` (`self.Widget`)) "DoNotLock" false)
              (set `PlayerController.bShowMouseCursor` true _returnvalue)
              (set `PlayerController.bEnableTouchEvents` true _returnvalue))))
        (:`then_1`
          (bind _asbp_test_computer_widget (cast `/Game/HUD/BP_TestComputerWidget` (`WidgetComponent.GetUserWidgetObject` (`self.Widget`))))
          (if (`/Game/HUD/BP_ComputerTasks.bIsComplete?` (`/Game/HUD/BP_TestComputerWidget.BP_ComputerTasks` _asbp_test_computer_widget))
            (`self.TaskFinished`)
            (`ActorComponent.SetActive` _widget false false)
            (`SceneComponent.SetVisibility` _widget false false)
            (`SceneComponent.K2_SetWorldLocation` _widget (`KismetMathLibrary.MakeVector` _returnvalue_x _returnvalue_y (+ _returnvalue_z 300.0)) false false)
            (`ActorComponent.SetActive` _tasklistw true false)
            (`ActorComponent.SetActive` (`self.TaskListW2`) true false)
            (`SceneComponent.SetVisibility` _tasklistw true false)
            (`SceneComponent.SetVisibility` (`self.TaskListW2`) true false)))))
    (:`Mail`
      (`|ExecutionSequence`
        (:`then_0`
          (`/Engine/EditorBlueprintResources/StandardMacros.DoOnce` false :!label _label_2
            (:`Completed`
              (bind _unique_actor_2 (`/Game/MacroLibrary/BML_ActorUtilities.GetActorWithUniqueTag` "ComputerCamera"))
              (`PlayerController.SetViewTargetWithBlend` _returnvalue_2 _unique_actor_2 0.5 "VTBlend_Linear" 0.0 true)
              (bind _asfirst_person_character_2 (cast `/Game/Character/FirstPersonCharacter` (`GameplayStatics.GetPlayerCharacter` 0)))
              (set `WidgetInteractionComponent.InteractionSource` "Mouse" (`/Game/Character/FirstPersonCharacter.WidgetInteraction` _asfirst_person_character_2))
              (`WidgetBlueprintLibrary.SetInputMode_GameAndUIEx` _returnvalue_2 (`WidgetComponent.GetUserWidgetObject` (`self.Widget`)) "DoNotLock" false)
              (set `PlayerController.bShowMouseCursor` true _returnvalue_2)
              (set `PlayerController.bEnableTouchEvents` true _returnvalue_2))))
        (:`then_1`
          (bind _asbp_task_list_widget_day_141 (cast `/Game/HUD/TaskListElements/BP_TaskListWidgetDay141` (`WidgetComponent.GetUserWidgetObject` (`self.TaskListW`))))
          (if (`/Game/HUD/TaskListElements/BP_TaskListWidgetDay141.bIsTaskListFinished?` _asbp_task_list_widget_day_141)
            (`self.TaskFinished`)
            (`self.DeactivateScreen`)
            (`|SpawnActorFromClass` "BP_Computer_C" (`self.GetTransform` self) "Undefined" "OverrideRootScale" null null)
            (`self.K2_DestroyActor`)))))))

(event `self.ReceiveTick`
  (params (DeltaSeconds :type "Float (single-precision)"))
  (bind _returnvalue (`GameplayStatics.GetPlayerController` 0))
  (bind _textrender2 (`self.TextRender2`))
  (bind _widget (`self.Widget`))
  (bind _textrender (`self.TextRender`))
  (bind _tasklistw (`self.TaskListW`))
  (bind (_returnvalue_x _returnvalue_y _returnvalue_z) (`KismetMathLibrary.BreakVector` (`SceneComponent.K2_GetComponentLocation` _widget)))
  (`|ExecutionSequence`
    (:`then_0`
      (switch `name` (`self.CurrentTask`)
        (:`Computer`
          (bind _asbp_test_computer_widget (cast `/Game/HUD/BP_TestComputerWidget` (`WidgetComponent.GetUserWidgetObject` (`self.Widget`))))
          (if (`/Game/HUD/BP_ComputerTasks.bIsComplete?` (`/Game/HUD/BP_TestComputerWidget.BP_ComputerTasks` _asbp_test_computer_widget))
            (`self.TaskFinished`)
            (`ActorComponent.SetActive` _widget false false)
            (`SceneComponent.SetVisibility` _widget false false)
            (`SceneComponent.K2_SetWorldLocation` _widget (`KismetMathLibrary.MakeVector` _returnvalue_x _returnvalue_y (+ _returnvalue_z 300.0)) false false)
            (`ActorComponent.SetActive` _tasklistw true false)
            (`SceneComponent.SetVisibility` _tasklistw true false)
            (set `self.CurrentTask` "Mail")))
        (:`Mail`
          (bind _asbp_task_list_widget_day_141 (cast `/Game/HUD/TaskListElements/BP_TaskListWidgetDay141` (`WidgetComponent.GetUserWidgetObject` (`self.TaskListW`))))
          (if (`/Game/HUD/TaskListElements/BP_TaskListWidgetDay141.bIsTaskListFinished?` _asbp_task_list_widget_day_141)
            (`self.TaskFinished`)
            (`self.DeactivateScreen`)
            (bind _returnvalue_2 (`|SpawnActorFromClass` "BP_Computer_C" (`self.GetTransform` self) "Undefined" "OverrideRootScale" null null))
            (`self.K2_DestroyActor`)
            (bind _asfirst_person_character (cast `/Game/Character/FirstPersonCharacter` (`GameplayStatics.GetPlayerCharacter` 0)))
            (`PlayerController.SetViewTargetWithBlend` _returnvalue _asfirst_person_character 0.5 "VTBlend_Linear" 0.0 true)
            (`WidgetBlueprintLibrary.SetInputMode_GameOnly` _returnvalue)
            (set `PlayerController.bShowMouseCursor` false _returnvalue)
            (`self.K2_DestroyActor`)
            (bind _asbp_task_list_widget_day_141_2 (cast `/Game/HUD/TaskListElements/BP_TaskListWidgetDay141` (`WidgetComponent.GetUserWidgetObject` (`/Game/Mechanics/TaskListObjects/Day1/BP_Computer.TaskListW` _returnvalue_2))))
            (`Image.SetBrushFromMaterial` (`/Game/HUD/TaskListElements/BP_TaskListWidgetDay141.Image_195` _asbp_task_list_widget_day_141_2) "/Game/HUD/TaskListElements/Day_142_Report_1_Blue_Mat.Day_142_Report_1_Blue_Mat")
            (set `/Game/HUD/TaskListElements/BP_TaskListWidgetDay141.bIsDay142?` true _asbp_task_list_widget_day_141_2)
            (bind _asfirst_person_character_2 (cast `/Game/Character/FirstPersonCharacter` (`GameplayStatics.GetPlayerCharacter` 0)))
            (set `WidgetInteractionComponent.InteractionSource` "World" (`/Game/Character/FirstPersonCharacter.WidgetInteraction` _asfirst_person_character_2))
            (if (== (`/Game/Character/FirstPersonCharacter.CurrentDay` _asfirst_person_character_2) 1)
              (bind _unique_actor (`/Game/MacroLibrary/BML_ActorUtilities.GetActorWithUniqueTag` "DeacivateJunctionDay2"))
              (bind _asbp_rail_junction (cast `/Game/Mechanics/GridDirectionLines/BP_RailJunction` _unique_actor :!pure true))
              (set `/Game/Mechanics/GridDirectionLines/BP_RailJunction.bIsActive?` true _asbp_rail_junction)
              (`/Game/Mechanics/GridDirectionLines/BP_RailJunction.DeactivatedChanges` _asbp_rail_junction))))))
    (:`then_1`
      (`|ExecutionSequence`
        (:`then_0`
          (bind _asfirst_person_character_3 (cast `/Game/Character/FirstPersonCharacter` (`GameplayStatics.GetPlayerCharacter` 0)))
          (`SceneComponent.K2_SetWorldRotation` _textrender (`KismetMathLibrary.FindLookAtRotation` (`SceneComponent.K2_GetComponentLocation` _textrender) (`SceneComponent.K2_GetComponentLocation` (`/Game/Character/FirstPersonCharacter.FirstPersonCamera` _asfirst_person_character_3))) false false))
        (:`then_1`
          (bind _asfirst_person_character_4 (cast `/Game/Character/FirstPersonCharacter` (`GameplayStatics.GetPlayerCharacter` 0)))
          (`SceneComponent.K2_SetWorldRotation` _textrender2 (`KismetMathLibrary.FindLookAtRotation` (`SceneComponent.K2_GetComponentLocation` _textrender2) (`SceneComponent.K2_GetComponentLocation` (`/Game/Character/FirstPersonCharacter.FirstPersonCamera` _asfirst_person_character_4))) false false))
        (:`then_2`
          (if (`self.bIsNextTaskInLIst?`)
            (`self.ActivateScreen`)))))))

(event `/Game/HUD/CodeChangeElements/BPI_TaskInterface.TurnComputerOn`
  (bind _widget (`self.Widget`))
  (`ActorComponent.SetActive` _widget true false)
  (`SceneComponent.SetVisibility` _widget true false))

(event `ActivateScreen`
  (`SceneComponent.SetVisibility` (`self.Widget`) true false))

(event `DeactivateScreen`
  (`SceneComponent.SetVisibility` (`self.TaskListW`) false false))

(fn `UserConstructionScript`
  (`parent.UserConstructionScript`))
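; Day 1's eighth task-list object, a child task actor that the player completes by clicking it and waiting through a short timed progress bar.
; A click calls the parent handler, then a DoOnce creates the progress widget and enables Tick for a two-second Delay.
; Tick accumulates scaled delta time on the widget to fill the bar.
; Afterwards it removes the widget, stops ticking and calls TaskFinished, which runs parent logic and resets the DoOnce.
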(event `self.ReceiveBeginPlay`
  (`parent.ReceiveBeginPlay`)
  (`self.SetActorTickEnabled` false))

(event `self.PlayerClick`
  (params (PlayerCharacter :type "/Game/Character/FirstPersonCharacter Object Reference") (TagFunctionality :type Name))
  ;[1 1 1] Check If this is next task, space for any other checks
  (`parent.PlayerClick` PlayerCharacter "None")
  ;[1 1 1] Conditions for finishing task
  (`/Engine/EditorBlueprintResources/StandardMacros.DoOnce` false :!label _label
    (:`Completed`
      (bind _returnvalue (`|CreateWidget` "/Game/Mechanics/TaskListObjects/BP_ProgressBar.BP_ProgressBar_C"))
      (bind _output_get (set `self.Progressbar` _returnvalue))
      (`UserWidget.AddToViewport` _output_get 0)
      (`self.SetActorTickEnabled` true)
      (`KismetSystemLibrary.Delay` 2.0)
      (`Widget.RemoveFromParent` (`self.Progressbar`))
      (`self.SetActorTickEnabled` false)
      (`self.TaskFinished`))))

(event `self.TaskFinished`
  (`parent.TaskFinished`)
  (goto _label :!via `Reset`))

(event `self.ReceiveTick`
  (params (DeltaSeconds :type "Float (single-precision)"))
  (bind _progressbar (`self.Progressbar`))
  (bind _output_get (set `/Game/Mechanics/TaskListObjects/BP_ProgressBar.CompondDeltatime` (+ (/ DeltaSeconds 2.0) (`/Game/Mechanics/TaskListObjects/BP_ProgressBar.CompondDeltatime` _progressbar)) _progressbar))
  (`ProgressBar.SetPercent` (`/Game/Mechanics/TaskListObjects/BP_ProgressBar.TaskCompletionProgressBar` _progressbar) _output_get))

(fn `UserConstructionScript`
  (`parent.UserConstructionScript`))
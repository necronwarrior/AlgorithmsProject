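; BP_WashUpDoor is the Day 1 wash-up task door, which the player clicks to complete the task behind a screen fade.
; A click passes a resettable DoOnce, fades, waits briefly, calls TaskFinished, then fades back.
; Tick advances a progress bar while active, otherwise turns the text render toward the player camera.
; Progress bar creation and removal, plus a garden NPC follow trigger, are disconnected.
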(event `self.ReceiveBeginPlay`
  ;[1 1 1] Disable tick on start
  (`parent.ReceiveBeginPlay`))

(event `self.PlayerClick`
  (params (PlayerCharacter :type "/Game/Character/FirstPersonCharacter Object Reference") (TagFunctionality :type Name))
  ;[1 1 1] Check If this is next task, space for any other checks
  (`parent.PlayerClick` PlayerCharacter TagFunctionality)
  (`/Engine/EditorBlueprintResources/StandardMacros.DoOnce` false :!label _label
    (:`Completed`
      ;[1 1 1] Conditions for finishing task
      (set `self.bIsActivatedYet?` true)
      (`/Game/MacroLibrary/BML_ActorUtilities.FadeInOut` PlayerCharacter true
        (:`Completed`
          (`KismetSystemLibrary.Delay` 1.0)
          (`self.TaskFinished`)
          (`/Game/MacroLibrary/BML_ActorUtilities.FadeInOut` PlayerCharacter))))))

(event `self.TaskFinished`
  ;[1 1 1] Check If this is next task, space for any other checks
  (`parent.TaskFinished`)
  (set `self.bIsActivatedYet?` false)
  (goto _label :!via `Reset`))

(event `self.ReceiveTick`
  (params (DeltaSeconds :type "Float (single-precision)"))
  (bind _progressbar (`self.Progressbar`))
  (bind _textrender (`self.TextRender`))
  (if (`self.bIsActivatedYet?`)
    ;[1 1 1] Fill up the progress bar
    (bind _output_get (set `/Game/Mechanics/TaskListObjects/BP_ProgressBar.CompondDeltatime` (+ DeltaSeconds (`/Game/Mechanics/TaskListObjects/BP_ProgressBar.CompondDeltatime` _progressbar)) _progressbar))
    (`ProgressBar.SetPercent` (`/Game/Mechanics/TaskListObjects/BP_ProgressBar.TaskCompletionProgressBar` _progressbar) _output_get)
    (else
      (bind _asfirst_person_character (cast `/Game/Character/FirstPersonCharacter` (`GameplayStatics.GetPlayerCharacter` 0)))
      (`SceneComponent.K2_SetWorldRotation` _textrender (`KismetMathLibrary.FindLookAtRotation` (`SceneComponent.K2_GetComponentLocation` _textrender) (`SceneComponent.K2_GetComponentLocation` (`/Game/Character/FirstPersonCharacter.FirstPersonCamera` _asfirst_person_character))) false false))))

(fn `UserConstructionScript`
  (`parent.UserConstructionScript`))
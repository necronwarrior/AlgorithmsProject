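; Interactive bed task object that ends the day when the player clicks it.
; On click it disables input, plays the wake-up sequence, teleports the player and controller to a sleep point, marks the task finished and flags the player as lying down.
; After a short delay it restores input and calls the character's day reset.
; Each tick it turns its text label toward the first-person camera.
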(event `self.ReceiveBeginPlay`
  (`parent.ReceiveBeginPlay`))

(event `self.PlayerClick`
  (params (PlayerCharacter :type "/Game/Character/FirstPersonCharacter Object Reference") (TagFunctionality :type Name))
  (bind _returnvalue (`GameplayStatics.GetPlayerController` 0))
  (bind _sequenceplayer (`LevelSequenceActor.SequencePlayer` (`self.WakeUpSequence`)))
  (bind _location (.location (`self.GetTransform` (`self.SleepPoint`))))
  ;[1 1 1] Check If this is next task, space for any other checks
  (`parent.PlayerClick` PlayerCharacter "None")
  (`self.DisableInput` PlayerCharacter (`GameplayStatics.GetPlayerController` 0))
  ;[1 1 1] Conditions for finishing task
  (`MovieSceneSequencePlayer.SetPlaybackPosition` _sequenceplayer 0.0)
  (`MovieSceneSequencePlayer.Play` _sequenceplayer)
  (`/Game/Character/FirstPersonCharacter.Waking up` PlayerCharacter)
  (`self.K2_SetActorLocation` _returnvalue _location false true)
  (`self.K2_SetActorLocation` PlayerCharacter _location false true)
  (`self.K2_SetActorRotation` _returnvalue (.rotation (`self.GetTransform` (`self.SleepPoint`))) false)
  (`self.TaskFinished`)
  (set `/Game/Character/FirstPersonCharacter.bIsLyingDown?` true PlayerCharacter)
  (`KismetSystemLibrary.Delay` 5.0)
  (`self.EnableInput` PlayerCharacter (`GameplayStatics.GetPlayerController` 0))
  (`/Game/Character/FirstPersonCharacter.Reset Day` PlayerCharacter))

(event `self.ReceiveTick`
  (params (DeltaSeconds :type "Float (single-precision)"))
  (bind _textrender (`self.TextRender`))
  (bind _asfirst_person_character (cast `/Game/Character/FirstPersonCharacter` (`GameplayStatics.GetPlayerCharacter` 0)))
  (`SceneComponent.K2_SetWorldRotation` _textrender (`KismetMathLibrary.FindLookAtRotation` (`SceneComponent.K2_GetComponentLocation` _textrender) (`SceneComponent.K2_GetComponentLocation` (`/Game/Character/FirstPersonCharacter.FirstPersonCamera` _asfirst_person_character))) false false))

(fn `UserConstructionScript`
  (`parent.UserConstructionScript`))
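; BP_Plants is the clickable plants object for a Day 1 watering task.
; On player click, it passes its TaskGivingObject to the FirstPersonCharacter as the next task reference and flags watering as finished.
; It then overrides the mesh materials of every actor in TreeList to show the change.
; A handler bound to the character's CallNextDay event resets those materials to the default when the day advances.
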(event `self.ReceiveBeginPlay`
  (bind _asfirst_person_character (cast `/Game/Character/FirstPersonCharacter` (`GameplayStatics.GetPlayerCharacter` 0)))
  (add `/Game/Character/FirstPersonCharacter.CallNextDay` _asfirst_person_character (delegate `NextDayReset`)))

(event `NextDayReset`
  (for _array_element (`self.TreeList`)
    (bind _returnvalue (`self.GetComponentByClass` _array_element "/Script/Engine.StaticMeshComponent"))
    (for _index (range (+ (`PrimitiveComponent.GetNumMaterials` _returnvalue) 1))
      (`PrimitiveComponent.SetMaterial` _returnvalue _index "/Game/Assets/Sign_Board/01_-_Default.01_-_Default"))))

(event `Player Click`
  (bind _taskgivingobject (`self.TaskGivingObject`))
  (if (!= (`self.TaskGivingObject`) null)
    (bind _asfirst_person_character (cast `/Game/Character/FirstPersonCharacter` (`GameplayStatics.GetPlayerCharacter` 0)))
    (set `/Game/Character/FirstPersonCharacter.NextTaskObjectReference` _taskgivingobject _asfirst_person_character)
    (set `/Game/Mechanics/TaskListObjects/Day1/BP_WateringCan.bIsFinishedWatering` true _taskgivingobject)
    (for _array_element (`self.TreeList`)
      (bind _returnvalue (`self.GetComponentByClass` _array_element "/Script/Engine.StaticMeshComponent"))
      (for _index (range (+ (`PrimitiveComponent.GetNumMaterials` _returnvalue) 1))
        (`PrimitiveComponent.SetMaterial` _returnvalue _index "/Engine/MapTemplates/Materials/BasicAsset03.BasicAsset03")))))

(fn `UserConstructionScript`
  (`parent.UserConstructionScript`))
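; Day 1 task-list computer that takes the player through an on-screen computer task, then a mail task list.
; Computer and Mail clicks blend to a tagged camera with mouse UI input, once per day reset; completed computer tasks swap the screen to the task list.
; A finished list restores first-person control and replaces this actor with BP_Computer.
; Tick turns two text labels toward the player and shows the screen when its task is next.
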(event `OnDayReset`
  (bind _returnvalue (`GameplayStatics.GetPlayerController` 0))
  (bind _returnvalue_2 (`GameplayStatics.GetPlayerController` 0))
  (bind _widget (`self.Widget`))
  (bind _tasklistw (`self.TaskListW`))
  (bind (_returnvalue_x _returnvalue_y _returnvalue_z) (`KismetMathLibrary.BreakVector` (`SceneComponent.K2_GetComponentLocation` _widget)))
  (`ActorComponent.SetActive` _widget true false)
  (`SceneComponent.SetVisibility` _widget true false)
  (`SceneComponent.K2_SetWorldLocation` _widget (`KismetMathLibrary.MakeVector` _returnvalue_x _returnvalue_y (- _returnvalue_z 300.0)) false false)
  (`ActorComponent.SetActive` _tasklistw false false)
  (`SceneComponent.SetVisibility` _tasklistw false false)
  (`|ExecutionSequence`
    (:`then_0`
      (goto _label :!via `Reset`))
    (:`then_1`
      (goto _label_2 :!via `Reset`))))

(event `self.PlayerClick`
  (params (PlayerCharacter :type "/Game/Character/FirstPersonCharacter Object Reference") (TagFunctionality :type Name))
  (bind _returnvalue (`GameplayStatics.GetPlayerController` 0))
  (bind _returnvalue_2 (`GameplayStatics.GetPlayerController` 0))
  (bind _returnvalue_3 (`GameplayStatics.GetPlayerController` 0))
  (bind _returnvalue_4 (`GameplayStatics.GetPlayerController` 0))
  (bind _widget (`self.Widget`))
  (bind _tasklistw (`self.TaskListW`))
  (bind (_returnvalue_x _returnvalue_y _returnvalue_z) (`KismetMathLibrary.BreakVector` (`SceneComponent.K2_GetComponentLocation` _widget)))
  (`parent.PlayerClick` PlayerCharacter TagFunctionality)
  (switch `name` TagFunctionality
    (:`Computer`
      (`|ExecutionSequence`
        (:`then_0`
          (`/Engine/EditorBlueprintResources/StandardMacros.DoOnce` false :!label _label
            (:`Completed`
              (bind _unique_actor (`/Game/MacroLibrary/BML_ActorUtilities.GetActorWithUniqueTag` "ComputerCamera"))
              (`PlayerController.SetViewTargetWithBlend` _returnvalue_2 _unique_actor 2.0 "VTBlend_Linear" 0.0 true)
              (bind _asfirst_person_character (cast `/Game/Character/FirstPersonCharacter` (`GameplayStatics.GetPlayerCharacter` 0)))
              (set `WidgetInteractionComponent.InteractionSource` "Mouse" (`/Game/Character/FirstPersonCharacter.WidgetInteraction` _asfirst_person_character))
              (`WidgetBlueprintLibrary.SetInputMode_GameAndUIEx` _returnvalue_2 (`WidgetComponent.GetUserWidgetObject` (`self.Widget`)) "DoNotLock" false)
              (set `PlayerController.bShowMouseCursor` true _returnvalue_2)
              (set `PlayerController.bEnableTouchEvents` true _returnvalue_2))))
        (:`then_1`
          (bind _asbp_test_computer_widget (cast `/Game/HUD/BP_TestComputerWidget` (`WidgetComponent.GetUserWidgetObject` (`self.Widget`))))
          (if (`/Game/HUD/BP_ComputerTasks.bIsComplete?` (`/Game/HUD/BP_TestComputerWidget.BP_ComputerTasks` _asbp_test_computer_widget))
            (`self.TaskFinished`)
            (`ActorComponent.SetActive` _widget false false)
            (`SceneComponent.SetVisibility` _widget false false)
            (`SceneComponent.K2_SetWorldLocation` _widget (`KismetMathLibrary.MakeVector` _returnvalue_x _returnvalue_y (+ _returnvalue_z 300.0)) false false)
            (`ActorComponent.SetActive` _tasklistw true false)
            (`SceneComponent.SetVisibility` _tasklistw true false)
            (bind _unique_actor_2 (`/Game/MacroLibrary/BML_ActorUtilities.GetActorWithUniqueTag` "ComputerCamera"))
            (`PlayerController.SetViewTargetWithBlend` _returnvalue _unique_actor_2 2.0 "VTBlend_Linear" 0.0 true)
            (bind _asfirst_person_character_2 (cast `/Game/Character/FirstPersonCharacter` (`GameplayStatics.GetPlayerCharacter` 0)))
            (set `WidgetInteractionComponent.InteractionSource` "Mouse" (`/Game/Character/FirstPersonCharacter.WidgetInteraction` _asfirst_person_character_2))
            (`WidgetBlueprintLibrary.SetInputMode_GameAndUIEx` _returnvalue (`WidgetComponent.GetUserWidgetObject` (`self.Widget`)) "DoNotLock" false)
            (set `PlayerController.bShowMouseCursor` true _returnvalue)
            (set `PlayerController.bEnableTouchEvents` true _returnvalue)))))
    (:`Mail`
      (`|ExecutionSequence`
        (:`then_0`
          (`/Engine/EditorBlueprintResources/StandardMacros.DoOnce` false :!label _label_2
            (:`Completed`
              (bind _unique_actor_3 (`/Game/MacroLibrary/BML_ActorUtilities.GetActorWithUniqueTag` "ComputerCamera"))
              (`PlayerController.SetViewTargetWithBlend` _returnvalue_3 _unique_actor_3 2.0 "VTBlend_Linear" 0.0 true)
              (bind _asfirst_person_character_3 (cast `/Game/Character/FirstPersonCharacter` (`GameplayStatics.GetPlayerCharacter` 0)))
              (set `WidgetInteractionComponent.InteractionSource` "Mouse" (`/Game/Character/FirstPersonCharacter.WidgetInteraction` _asfirst_person_character_3))
              (`WidgetBlueprintLibrary.SetInputMode_GameAndUIEx` _returnvalue_3 (`WidgetComponent.GetUserWidgetObject` (`self.Widget`)) "DoNotLock" false)
              (set `PlayerController.bShowMouseCursor` true _returnvalue_3)
              (set `PlayerController.bEnableTouchEvents` true _returnvalue_3))))
        (:`then_1`
          (bind _asbp_task_list_widget (cast `/Game/HUD/BP_TaskListWidget` (`WidgetComponent.GetUserWidgetObject` (`self.TaskListW`))))
          (if (`/Game/HUD/BP_TaskListWidget.bIsTaskListFinished?` _asbp_task_list_widget)
            (`self.TaskFinished`)
            (`self.DeactivateScreen`)
            (`|SpawnActorFromClass` "/Game/Mechanics/TaskListObjects/Day1/BP_Computer.BP_Computer_C" (`self.GetTransform` self) "Undefined" "OverrideRootScale" null null)
            (bind _asfirst_person_character_4 (cast `/Game/Character/FirstPersonCharacter` (`GameplayStatics.GetPlayerCharacter` 0)))
            (`PlayerController.SetViewTargetWithBlend` _returnvalue_4 _asfirst_person_character_4 2.0 "VTBlend_Linear" 0.0 true)
            (`WidgetBlueprintLibrary.SetInputMode_GameOnly` _returnvalue_4)
            (set `PlayerController.bShowMouseCursor` false _returnvalue_4)
            (`self.K2_DestroyActor`)))))))

(event `self.ReceiveTick`
  (params (DeltaSeconds :type "Float (single-precision)"))
  (bind _textrender2 (`self.TextRender2`))
  (bind _textrender (`self.TextRender`))
  (`|ExecutionSequence`
    (:`then_0`
      (bind _asfirst_person_character (cast `/Game/Character/FirstPersonCharacter` (`GameplayStatics.GetPlayerCharacter` 0)))
      (`SceneComponent.K2_SetWorldRotation` _textrender (`KismetMathLibrary.FindLookAtRotation` (`SceneComponent.K2_GetComponentLocation` _textrender) (`SceneComponent.K2_GetComponentLocation` (`/Game/Character/FirstPersonCharacter.FirstPersonCamera` _asfirst_person_character))) false false))
    (:`then_1`
      (bind _asfirst_person_character_2 (cast `/Game/Character/FirstPersonCharacter` (`GameplayStatics.GetPlayerCharacter` 0)))
      (`SceneComponent.K2_SetWorldRotation` _textrender2 (`KismetMathLibrary.FindLookAtRotation` (`SceneComponent.K2_GetComponentLocation` _textrender2) (`SceneComponent.K2_GetComponentLocation` (`/Game/Character/FirstPersonCharacter.FirstPersonCamera` _asfirst_person_character_2))) false false))
    (:`then_2`
      (if (`self.bIsNextTaskInLIst?`)
        (`self.ActivateScreen`)
        (set `PlayerController.bShowMouseCursor` false (`GameplayStatics.GetPlayerController` 0))))))

(event `ActivateScreen`
  (`SceneComponent.SetVisibility` (`self.Widget`) true false))

(event `DeactivateScreen`
  (`SceneComponent.SetVisibility` (`self.TaskListW`) false false))

(event `/Game/HUD/CodeChangeElements/BPI_TaskInterface.TurnComputerOn`
  (bind _widget (`self.Widget`))
  (`ActorComponent.SetActive` _widget true false)
  (`SceneComponent.SetVisibility` _widget true false))

(fn `UserConstructionScript`
  (`parent.UserConstructionScript`))
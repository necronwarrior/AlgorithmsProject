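; BP_Day1Task11 is a Day 1 task-list object that relocates the player when clicked.
; On click it calls the parent handler, switches the player's control structure, and releases overlapping rail junctions by disabling input and clearing their player reference.
; It then moves the player to a hardcoded location.
; The next-task check is an empty placeholder, and the task-completion, wake-up sequence and day-end logic are disconnected.
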(event `self.ReceiveBeginPlay`
  (`parent.ReceiveBeginPlay`)
  (set `self.bIsDayOver?` false))

(event `self.PlayerClick`
  (params (PlayerCharacter :type "/Game/Character/FirstPersonCharacter Object Reference") (TagFunctionality :type Name))
  ;[1 1 1] Check If this is next task, space for any other checks
  (`parent.PlayerClick` PlayerCharacter "None")
  (`KismetSystemLibrary.PrintString` "Hello")
  (if (`self.bIsNextTaskInLIst?`)
    _
    (else
      _))
  (`/Game/Character/FirstPersonCharacter.SetControlStructure` PlayerCharacter "NewEnumerator0")
  (for _array_element (`PrimitiveComponent.GetOverlappingActors` (`Character.CapsuleComponent` PlayerCharacter) "/Game/Mechanics/GridDirectionLines/BP_RailJunction.BP_RailJunction_C")
    (`self.DisableInput` _array_element (`GameplayStatics.GetPlayerController` 0))
    (bind _asbp_rail_junction (cast `/Game/Mechanics/GridDirectionLines/BP_RailJunction` _array_element))
    (set `/Game/Mechanics/GridDirectionLines/BP_RailJunction.PlayerCharacter` null _asbp_rail_junction))
  (`self.K2_SetActorLocation` PlayerCharacter (10215.0 -11254.0 1410.0) false false))

(fn `UserConstructionScript`
  (`parent.UserConstructionScript`))
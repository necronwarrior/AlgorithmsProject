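; BP_CodeComputer is a clickable in-world computer that hosts a code-change puzzle on a widget component.
; Clicking it while unsolved blends the view to the computer and switches widget interaction and input to the mouse cursor.
; Tick polls the widget for completion, then notifies influenced objects, returns the view and game input to the player, and updates the related task object.
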(event `PlayerClick`
  (if (not (`self.bIsRelatedPuzzleComplete?`))
    (`self.FocusCamera`)))

(event `self.ReceiveBeginPlay`
  (bind _returnvalue (`|CreateWidget` (`self.CodeChangeWidget`) (`GameplayStatics.GetPlayerController` 0)))
  (`WidgetComponent.SetWidget` (`self.Widget`) _returnvalue))

(event `self.ReceiveTick`
  (params (DeltaSeconds :type "Float (single-precision)"))
  (bind _relatedtaskobject (`self.RelatedTaskObject`))
  (if (not (`self.bIsRelatedPuzzleComplete?`))
    (bind _asbp_code_change_base (cast `/Game/HUD/CodeChangeElements/BP_CodeChange_Base` (`WidgetComponent.GetUserWidgetObject` (`self.Widget`))))
    (if (`/Game/HUD/CodeChangeElements/BP_CodeChange_Base.bIsPuzzleComplete?` _asbp_code_change_base)
      (set `self.bIsRelatedPuzzleComplete?` true)
      (for _array_element (`self.InfluencedObjects`)
        (message `/Game/Mechanics/CodeInjection/BPI_CodeInjectionInterface.PuzzleSolved` _array_element))
      (`self.UnfocusCamera`)
      (bind _asfirst_person_character (cast `/Game/Character/FirstPersonCharacter` (`GameplayStatics.GetPlayerCharacter` 0)))
      (set `/Game/Mechanics/TaskListObjects/BP_PlayerTaskListObjectTemplate.PlayerCharacterReference` _asfirst_person_character _relatedtaskobject)
      (`/Game/Mechanics/TaskListObjects/BP_PlayerTaskListObjectTemplate.computer_task_updated` _relatedtaskobject))))

(event `FocusCamera`
  (bind _returnvalue (`GameplayStatics.GetPlayerController` 0))
  (`PlayerController.SetViewTargetWithBlend` _returnvalue self 0.5 "VTBlend_Linear" 0.0 true)
  (bind _asfirst_person_character (cast `/Game/Character/FirstPersonCharacter` (`GameplayStatics.GetPlayerCharacter` 0)))
  (set `WidgetInteractionComponent.InteractionSource` "Mouse" (`/Game/Character/FirstPersonCharacter.WidgetInteraction` _asfirst_person_character))
  (`WidgetBlueprintLibrary.SetInputMode_GameAndUIEx` _returnvalue (`WidgetComponent.GetUserWidgetObject` (`self.Widget`)) "DoNotLock" false)
  (set `PlayerController.bShowMouseCursor` true _returnvalue)
  (set `PlayerController.bEnableTouchEvents` true _returnvalue))

(event `UnfocusCamera`
  (bind _returnvalue (`GameplayStatics.GetPlayerController` 0))
  (bind _asfirst_person_character (cast `/Game/Character/FirstPersonCharacter` (`GameplayStatics.GetPlayerCharacter` 0)))
  (`PlayerController.SetViewTargetWithBlend` _returnvalue _asfirst_person_character 0.5 "VTBlend_Linear" 0.0 true)
  (`WidgetBlueprintLibrary.SetInputMode_GameOnly` _returnvalue)
  (set `PlayerController.bShowMouseCursor` false _returnvalue))

(fn `UserConstructionScript`)
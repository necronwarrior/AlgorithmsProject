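; BP_Neighbours is a Day 2 task-list object for the neighbours, with a text label that always faces the player.
; On BeginPlay it runs the parent logic and caches a reference to the FirstPersonCharacter.
; Each Tick it casts the player character again and rotates its TextRender toward the first-person camera with a look-at rotation.
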(event `self.ReceiveBeginPlay`
  (`parent.ReceiveBeginPlay`)
  (bind _asfirst_person_character (cast `/Game/Character/FirstPersonCharacter` (`GameplayStatics.GetPlayerCharacter` 0)))
  (set `self.PlayerCharacterReference` _asfirst_person_character))

(event `self.ReceiveTick`
  (params (DeltaSeconds :type "Float (single-precision)"))
  (bind _textrender (`self.TextRender`))
  (bind _asfirst_person_character (cast `/Game/Character/FirstPersonCharacter` (`GameplayStatics.GetPlayerCharacter` 0)))
  (`SceneComponent.K2_SetWorldRotation` _textrender (`KismetMathLibrary.FindLookAtRotation` (`SceneComponent.K2_GetComponentLocation` _textrender) (`SceneComponent.K2_GetComponentLocation` (`/Game/Character/FirstPersonCharacter.FirstPersonCamera` _asfirst_person_character))) false false))

(fn `UserConstructionScript`)
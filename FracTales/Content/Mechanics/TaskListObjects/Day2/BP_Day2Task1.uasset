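; BP_Day2Task1 is the first Day 2 task-list object, linking a player click to partner dialogue.
; On BeginPlay it spawns a BP_PartnerDialogueArea at the world origin and passes it the task's partner dialogue table.
; The first PlayerClick simulates an overlap on that area to call the dialogue, behind a DoOnce that TaskFinished resets after running parent logic.
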(event `self.ReceiveBeginPlay`
  (`parent.ReceiveBeginPlay`)
  (bind _returnvalue (`|SpawnActorFromClass` "/Game/DialogueSystem/PartnerConversations/BP_PartnerDialogueArea.BP_PartnerDialogueArea_C" (`KismetMathLibrary.MakeTransform` (0.0 0.0 0.0)) "Undefined" "OverrideRootScale" null null))
  (bind _output_get (set `self.PartnerDialogueAreaRef` _returnvalue))
  (set `/Game/DialogueSystem/PartnerConversations/BP_PartnerDialogueArea.DialogueToCall` (`self.PartnerDialogueTable`) _output_get))

(event `self.PlayerClick`
  (params (PlayerCharacter :type "/Game/Character/FirstPersonCharacter Object Reference") (TagFunctionality :type Name))
  (`parent.PlayerClick` PlayerCharacter TagFunctionality)
  (`/Engine/EditorBlueprintResources/StandardMacros.DoOnce` false :!label _label
    (:`Completed`
      (`/Game/DialogueSystem/PartnerConversations/BP_PartnerDialogueArea.SimulateOverlap` (`self.PartnerDialogueAreaRef`)))))

(event `self.TaskFinished`
  (`parent.TaskFinished`)
  (goto _label :!via `Reset`))

(fn `TaskFinishedDelegate`
  (`self.TaskFinished`))

(fn `UserConstructionScript`
  (`parent.UserConstructionScript`))
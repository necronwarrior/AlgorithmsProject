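; Parker's computer, a Day 2 task object that the player clicks in two stages as part of a dialogue-driven sequence.
; Events S1_1 and S1_2 switch it on, showing its screen widget and then activating the install state; S1_5 activates a rail.
; The first click stops delayed partner dialogue; the second finishes the task and assigns gate-opening dialogue to NPCs by tag.
; Tick turns its text toward the player camera.
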(event Custom|S1_1
  (Variables|Default|SetbIsComputerOn? true)
  (Rendering|SetVisibility (Variables|Default|GetWidget) true false))

(event Custom|S1_2
  (bind _asbp_parker_computer_interaction (Utilities|Casting|CastToBP_ParkerComputerInteraction (UserInterface|GetUserWidgetObject (Variables|Default|GetWidget))))
  (Variables|/Game/HUD/ParkerComputerTasks/BP_ParkerComputerInteraction.BP_ParkerComputerInteraction_C|SetbIsInstallActive? _asbp_parker_computer_interaction true)
  (Variables|Default|SetbIsComputerOn? true))

(event Custom|S1_5
  (Variables|/Game/Mechanics/GridDirectionLines/BP_RailJunction.BP_RailJunction_C|SetbIsActive? (Variables|Default|GetRailToEnable) true))

(event EventBeginPlay
  (|CallParentFunction))

(event EventTick
  (params (DeltaSeconds :type Float%20%28single-precision%29))
  (bind _textrender (Variables|Default|GetTextRender))
  (bind _asfirst_person_character (Utilities|Casting|CastToFirstPersonCharacter (Game|GetPlayerCharacter 0)))
  (Transformation|SetWorldRotation _textrender (Math|Rotator|FindLookatRotation (Transformation|GetWorldLocation _textrender) (Transformation|GetWorldLocation (Variables|/Game/Character/FirstPersonCharacter.FirstPersonCharacter_C|GetFirstPersonCamera _asfirst_person_character))) false false))

(event EventPlayerClick
  (params (PlayerCharacter :type First%20Person%20Character%20Object%20Reference) (TagFunctionality :type Name :default "None"))
  (if (Variables|Default|GetbIsComputerOn?)
    (|CallParentFunction PlayerCharacter TagFunctionality)
    (switch int (Variables|Default|GetTimesClicked)
      (:0
        (bind _outactors (Actor|GetAllActorsOfClass "/Game/DialogueSystem/PartnerConversations/BP_PartnerDialogueManager.BP_PartnerDialogueManager_C"))
        (Default|StopDelayedDialogue (Utilities|Array|Get(acopy) _outactors))
        (Utilities|PlayDialogue "/Game/DialogueSystem/PartnerConversations/DialogueChanges/Scene_1/S1_2.S1_2")
        (Math|Integer|IncrementInt (Variables|Default|GetTimesClicked)
          (:%20%20
            (Variables|Default|SetbIsComputerOn? false))))
      (:1
        (Utilities|PlayDialogue "/Game/DialogueSystem/PartnerConversations/DialogueChanges/Scene_1/S1_5.S1_5")
        (CallFunction|TaskFinished)
        (Rendering|SetVisibility (Variables|Default|GetWidget) false false)
        (bind _outactors_2 (Actor|GetAllActorsOfClass "/Game/DialogueSystem/PartnerConversations/ControllableNPC/BP_ControlNPCGardenTest.BP_ControlNPCGardenTest_C"))
        (for _array_element _outactors_2
          (switch name (Utilities|Array|Get(acopy) (Variables|/Script/Engine.Actor|GetTags _array_element) 1)
            (:NPC1
              (Variables|/Game/DialogueSystem/PartnerConversations/ControllableNPC/BP_ControlNPCBase.BP_ControlNPCBase_C|SetAttatchedDialogue _array_element "/Game/DialogueSystem/PartnerConversations/Dialogues/GateOpeningDialogue1_1.GateOpeningDialogue1_1"))
            (:NPC2
              (Variables|/Game/DialogueSystem/PartnerConversations/ControllableNPC/BP_ControlNPCBase.BP_ControlNPCBase_C|SetAttatchedDialogue _array_element "/Game/DialogueSystem/PartnerConversations/Dialogues/GateOpeningDialogue1_2.GateOpeningDialogue1_2"))
            (:NPC3
              (Variables|/Game/DialogueSystem/PartnerConversations/ControllableNPC/BP_ControlNPCBase.BP_ControlNPCBase_C|SetAttatchedDialogue _array_element "/Game/DialogueSystem/PartnerConversations/Dialogues/GateOpeningDialogue1_3.GateOpeningDialogue1_3"))
            (:NPC4
              (Variables|/Game/DialogueSystem/PartnerConversations/ControllableNPC/BP_ControlNPCBase.BP_ControlNPCBase_C|SetAttatchedDialogue _array_element "/Game/DialogueSystem/PartnerConversations/Dialogues/GateOpeningDialogue1_4.GateOpeningDialogue1_4"))
            (:NPC5
              (Variables|/Game/DialogueSystem/PartnerConversations/ControllableNPC/BP_ControlNPCBase.BP_ControlNPCBase_C|SetAttatchedDialogue _array_element "/Game/DialogueSystem/PartnerConversations/Dialogues/GateOpeningDialogue1_5.GateOpeningDialogue1_5"))
            (:NPC6
              (Variables|/Game/DialogueSystem/PartnerConversations/ControllableNPC/BP_ControlNPCBase.BP_ControlNPCBase_C|SetAttatchedDialogue _array_element "/Game/DialogueSystem/PartnerConversations/Dialogues/GateOpeningDialogue1_6.GateOpeningDialogue1_6"))))))))

(fn ConstructionScript
  (|CallParentFunction))
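; BP_WallCounter is a clickable task object that shows a calendar widget and advances it to the next day.
; After a five-second delay on BeginPlay it caches the BP_CalendarDisplay widget and sets it to first-person.
; A click advances the day, finishes the task, plays a Wwise click sound at the player and turns on the last BP_Computer found as the next task.
; Tick keeps its text render facing the first-person camera.
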(event `self.ReceiveBeginPlay`
  (`parent.ReceiveBeginPlay`)
  (`KismetSystemLibrary.Delay` 5.0)
  (bind _asbp_calendar_display (cast `/Game/Mechanics/TaskListObjects/Day1/BP_CalendarDisplay` (`WidgetComponent.GetUserWidgetObject` (`self.Widget`))))
  (`/Game/Mechanics/TaskListObjects/Day1/BP_CalendarDisplay.SetFirstPerson` _asbp_calendar_display))

(event `self.PlayerClick`
  (params (PlayerCharacter :type "/Game/Character/FirstPersonCharacter Object Reference") (TagFunctionality :type Name))
  (`parent.PlayerClick` PlayerCharacter TagFunctionality)
  (`/Game/Mechanics/TaskListObjects/Day1/BP_CalendarDisplay.NextDayCalled` (stale `self.ReceiveBeginPlay` _asbp_calendar_display))
  (`self.TaskFinished`)
  (`AkGameplayStatics.PostEventAtLocation` "/Game/Audio/Wwise/Events/sfx/objects/non-destructable/calendar/calendar_click_start.calendar_click_start" (`self.K2_GetActorLocation` (`GameplayStatics.GetPlayerCharacter` 0)))
  (bind _outactors (`GameplayStatics.GetAllActorsOfClass` "/Game/Mechanics/TaskListObjects/Day1/BP_Computer.BP_Computer_C"))
  (bind _output_get (set `self.NextTaskObject` (`|GetArrayItem` _outactors (`KismetArrayLibrary.Array_LastIndex` _outactors))))
  (bind _asbp_computer (cast `/Game/Mechanics/TaskListObjects/Day1/BP_Computer` _output_get))
  (`/Game/Mechanics/TaskListObjects/Day1/BP_Computer.TurnComputerOn` _asbp_computer))

(event `self.ReceiveTick`
  (params (DeltaSeconds :type "Float (single-precision)"))
  (bind _textrender (`self.TextRender`))
  (bind _asfirst_person_character (cast `/Game/Character/FirstPersonCharacter` (`GameplayStatics.GetPlayerCharacter` 0)))
  (`SceneComponent.K2_SetWorldRotation` _textrender (`KismetMathLibrary.FindLookAtRotation` (`SceneComponent.K2_GetComponentLocation` _textrender) (`SceneComponent.K2_GetComponentLocation` (`/Game/Character/FirstPersonCharacter.FirstPersonCamera` _asfirst_person_character))) false false))

(fn `UserConstructionScript`)
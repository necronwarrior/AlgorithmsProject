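; Template actor for an NPC object that runs a task list and opens a task-list widget when clicked.
; On BeginPlay it constructs its own instance of the CurrentTaskList class and starts executing it with itself as the argument.
; PlayerClick disables character input, shows and centers the cursor, then creates and displays CurrentTaskListWidget.
; The widget's TaskListObject is set to None rather than the created task list.
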(event `self.ReceiveBeginPlay`
  ;[1 1 1] When object is created, instantiate a copy of its task list
  (bind _returnvalue (`|GenericCreateObject` (`self.CurrentTaskList`) self))
  (bind _output_get (set `self.CreatedTaskList` _returnvalue))
  ;[1 1 1] Begin executing this object's set tasks
  (`/Game/Mechanics/Mechanic1/TemplateParts/BP_TaskListTemplate.ExecuteTaskList` _output_get self))

(event `PlayerClick`
  (bind _returnvalue (`GameplayStatics.GetPlayerController` 0))
  (bind (_x _y) (`KismetMathLibrary.BreakVector2D` (`WidgetLayoutLibrary.GetViewportSize`)))
  ;[1 1 1] Create widget when player clicks on object
  (`self.DisableInput` (`GameplayStatics.GetPlayerCharacter` 0) _returnvalue)
  (set `PlayerController.bShowMouseCursor` true _returnvalue)
  (`PlayerController.SetMouseLocation` _returnvalue (`KismetMathLibrary.FTrunc` (/ _x 2.0)) (`KismetMathLibrary.FTrunc` (/ _y 2.0)))
  (bind _returnvalue_2 (`|CreateWidget` (`self.CurrentTaskListWidget`)))
  (set `self.TaskListNPCWidget` _returnvalue_2)
  (set `/Game/Mechanics/Mechanic1/TemplateParts/BP_TaskListNPCWidgetTemplate.TaskListObject` null _returnvalue_2)
  (`UserWidget.AddToViewport` _returnvalue_2 0))

(fn `UserConstructionScript`)
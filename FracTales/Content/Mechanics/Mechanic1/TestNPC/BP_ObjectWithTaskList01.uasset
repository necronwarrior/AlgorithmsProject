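; Test NPC task-list object whose head turns during dialogue, building on a parent class's begin-play and click behavior.
; BeginPlay registers its cube as the attached cube and stores the head's resting rotation; a player click sets the dialogue flag.
; Each Tick interpolates the head toward a target derived from the player's rotation while in dialogue, otherwise back to rest, using fixed delta time rather than frame time.
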(event `self.ReceiveBeginPlay`
  (set `self.AttachedCube` (`self.Cube`))
  (set `self.OldRotator` (.rotation (`SceneComponent.GetRelativeTransform` (`self.Head`))))
  (`parent.ReceiveBeginPlay`))

(event `self.PlayerClick`
  (set `self.IsInDialogue?` true)
  (`parent.PlayerClick`))

(event `self.ReceiveTick`
  (params (DeltaSeconds :type "Float (single-precision)"))
  (if (`self.IsInDialogue?`)
    (`SceneComponent.K2_SetRelativeRotation` (`self.Head`) (`KismetMathLibrary.RInterpTo` (.rotation (`SceneComponent.GetRelativeTransform` (`self.Head`))) (`KismetMathLibrary.MakeRotator` (.roll (`self.K2_GetActorRotation` (`GameplayStatics.GetPlayerCharacter` 0))) (.pitch (`self.K2_GetActorRotation` (`GameplayStatics.GetPlayerCharacter` 0))) (+ (.yaw (`self.K2_GetActorRotation` (`GameplayStatics.GetPlayerCharacter` 0))) 90.0)) 0.1 0.1) false false)
    (else
      (`SceneComponent.K2_SetRelativeRotation` (`self.Head`) (`KismetMathLibrary.RInterpTo` (.rotation (`SceneComponent.GetRelativeTransform` (`self.Head`))) (`self.OldRotator`) 0.1 0.1) false false))))

(fn `UserConstructionScript`
  (`parent.UserConstructionScript`))
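; Clickable code-injection terminal that opens a puzzle UI for the player and triggers linked objects once the puzzle is solved.
; Clicking an unsolved, unoccupied terminal nests its configured Puzzle widget inside a CodeInjection base widget, links both to itself, shows the cursor and switches the character's control structure.
; PuzzleSolved posts a Wwise sound, calls TaskFinished and messages every InfluencedObject.
; Line-trace selection and option-list building logic remain unconnected.
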(event `self.ReceiveBeginPlay`
  (`self.EnableInput` (`GameplayStatics.GetPlayerController` 0)))

(event `self.PlayerClick`
  (params (PlayerCharacter :type "/Game/Character/FirstPersonCharacter Object Reference") (TagFunctionality :type Name))
  (bind _returnvalue (`GameplayStatics.GetPlayerController` 0))
  (`parent.PlayerClick` PlayerCharacter TagFunctionality)
  (set `self.PlayerCharacterReference` PlayerCharacter)
  (if (`self.bIsPuzzleSolved?`)
    _
    (elif (not (`self.bIsInTerminal?`))
      (set `self.bIsInTerminal?` true)
      (bind _returnvalue_2 (`|CreateWidget` "/Game/Mechanics/CodeInjection/BP_CodeInjectionBase.BP_CodeInjectionBase_C" _returnvalue))
      (bind _output_get (set `self.CodeInjectionWidget` _returnvalue_2))
      (set `/Game/Mechanics/CodeInjection/BP_CodeInjectionBase.RelatedCodeTerminal` self _output_get)
      (`UserWidget.AddToViewport` _output_get 0)
      (bind _returnvalue_3 (`|CreateWidget` (`self.Puzzle`) _returnvalue))
      (bind _output_get_2 (set `self.RelatedPuzzleWidget` _returnvalue_3))
      (`CanvasPanel.AddChildToCanvas` (`/Game/Mechanics/CodeInjection/BP_CodeInjectionBase.MainCanvas` (`self.CodeInjectionWidget`)) _output_get_2)
      (set `/Game/Mechanics/CodeInjection/BP_CodeInjectionBase.RelatedPuzzleWidget` _returnvalue_3 _output_get)
      (set `/Game/Mechanics/CodeInjection/BP_CodePuzzleBase.RelatedCodeTerminal` self _output_get_2)
      (set `PlayerController.bShowMouseCursor` true _returnvalue)
      (`WidgetBlueprintLibrary.SetInputMode_GameAndUIEx` _returnvalue _output_get_2)
      (bind _asfirst_person_character (cast `/Game/Character/FirstPersonCharacter` (`GameplayStatics.GetPlayerCharacter` 0)))
      (`/Game/Character/FirstPersonCharacter.SetControlStructure` _asfirst_person_character "NewEnumerator1"))))

(event `PuzzleSolved`
  (`AkGameplayStatics.PostEvent` "/Game/Audio/Wwise/Events/player/actions/typing/type_spacebar.type_spacebar" (`GameplayStatics.GetPlayerCharacter` 0))
  (`self.TaskFinished`)
  (for _array_element (`self.InfluencedObjects`)
    (message `/Game/Mechanics/CodeInjection/BPI_CodeInjectionInterface.PuzzleSolved` _array_element)))

(fn `UserConstructionScript`)
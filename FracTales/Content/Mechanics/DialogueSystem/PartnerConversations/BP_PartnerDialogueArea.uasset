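; BP_PartnerDialogueArea is a trigger actor that plays a partner dialogue when the player walks into it.
; On BeginPlay it caches the first BP_PartnerDialogueManager found in the level.
; When a FirstPersonCharacter overlaps it and no dialogue is playing, it passes DialogueToCall to the manager, then destroys itself if DeletedAfterCollision is set.
; An overlap during another dialogue is ignored rather than queued.
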(event `self.ReceiveBeginPlay`
  ;[0.2389 0.2443 1] Find and obtain a reference to the dialogue manager within the scene
  (bind _outactors (`GameplayStatics.GetAllActorsOfClass` "/Game/Mechanics/DialogueSystem/PartnerConversations/BP_PartnerDialogueManager.BP_PartnerDialogueManager_C"))
  (set `self.DialogueManager` (`|GetArrayItem` _outactors)))

(event `self.ReceiveActorBeginOverlap`
  (params (OtherActor :type "Actor Object Reference"))
  ;[0.3932 1 0.2522] When the player enters the collision of this actor, pass the dialogue related to this actor to the dialog manager to be played.
  (if (== (`GameplayStatics.GetObjectClass` OtherActor) "/Game/Character/FirstPersonCharacter.FirstPersonCharacter_C")
    (if (not (`/Game/Mechanics/DialogueSystem/PartnerConversations/BP_PartnerDialogueManager.bIsDialoguePlaying?` (`self.DialogueManager`)))
      (`/Game/Mechanics/DialogueSystem/PartnerConversations/BP_PartnerDialogueManager.CallDialogue` (`self.DialogueManager`) (`self.DialogueToCall`))
      (if (`self.bDeletedAfterCollision?`)
        (`self.K2_DestroyActor`)))))

(fn `UserConstructionScript`)
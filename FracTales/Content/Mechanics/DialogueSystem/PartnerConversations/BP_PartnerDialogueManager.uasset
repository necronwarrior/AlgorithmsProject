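; Manager for partner conversations that plays DataTable dialogue with sounds, timed lines and player choices, and registers itself with every BP_PartnerDialogueArea.
; Tick uses a Delay to pace HandleDialogue, which follows each row's OnEndGoTo until ChoiceMenu or EndDialogue.
; Mouse wheel highlights a choice, and right click stores its variable and jumps to its linked row.
; Rows trigger named events on tagged actors through near-zero SetTimerByFunctionName calls.
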(event `MouseRightClick`
  (bind _dialoguechoicewidgets (`self.DialogueChoiceWidgets`))
  ;[1 0.3181 0.7093] When the choice menu is open, listen for a right mouse click, and then perform the relevant actions based on the current choice
  (if (`self.bIsChoiceMenuOpen?`)
    (bind _returnvalue (`|GetDataTableRow` (`self.CurrentDialogue`) (`KismetStringLibrary.Conv_StringToName` (`KismetStringLibrary.Conv_IntToString` (`|GetArrayItem` (`self.CurrentDialogueChoices`) (`self.SelectedChoice`)))))
      (:`then`
        (bind (_lineid _variablecheck _characterspeaking _characterdialogue _linkedchoices _variableset _onendgoto) (break `/Game/Mechanics/DialogueSystem/PartnerConversations/Dialogues/DialogueStructure` _returnvalue))
        (bind (_variableid _variablename _value) (break `/Game/Mechanics/DialogueSystem/PartnerConversations/Dialogues/ChoiceStructure` _variableset))
        (`BlueprintMapLibrary.Map_Add` (`self.DialogueVariables`) _variablename _value)
        (set `self.bIsChoiceMenuOpen?` false)
        (set `self.DialogueEntryIndex` (`KismetStringLibrary.Conv_StringToName` _onendgoto))
        (for _array_element _dialoguechoicewidgets
          (`Widget.RemoveFromParent` _array_element))
        (`KismetArrayLibrary.Array_Clear` (`self.CurrentDialogueChoices`))
        (`KismetArrayLibrary.Array_Clear` _dialoguechoicewidgets)))))

(event `MouseWheelScrolled`
  (params (AxisValue :type "Float (double-precision)"))
  (bind _selectedchoice (`self.SelectedChoice`))
  (bind _selectedchoice_2 (`self.SelectedChoice`))
  ;[0.3708 0.9302 1] When the choice menu is open, update the player's choice based on how the mouse wheel is being scrolled
  (if (`self.bIsChoiceMenuOpen?`)
    (bind _output_get (set `self.MouseScroll` (+ AxisValue (`self.MouseScroll`))))
    (if (>= _output_get 2.0)
      (if (> _selectedchoice 0)
        (set `self.SelectedChoice` (- _selectedchoice 1)))
      (set `self.MouseScroll` 0.0)
      (elif (<= _output_get -2.0)
        (if (< _selectedchoice_2 (- (`KismetArrayLibrary.Array_Length` (`self.CurrentDialogueChoices`)) 1))
          (set `self.SelectedChoice` (+ _selectedchoice_2 1)))
        (set `self.MouseScroll` 0.0)))))

(event `self.ReceiveTick`
  (params (DeltaSeconds :type "Float (single-precision)"))
  ;[1 0.2187 0.7765] Update all functionality that is required frame by frame
  (if (`self.bIsDialoguePlaying?`)
    (if (`self.bIsChoiceMenuOpen?`)
      (for (_array_element _array_index) (`self.DialogueChoiceWidgets`)
        (if (== _array_index (`self.SelectedChoice`))
          (bind _choicetextwidget (`/Game/Mechanics/DialogueSystem/PartnerConversations/BP_PartnerDialogueChoice.ChoiceTextWidget` _array_element))
          (`TextBlock.SetColorAndOpacity` _choicetextwidget (make `SlateColor` (struct :`R` 1.0 :`G` 0.218 :`A` 1.0)))
          (else
            (`TextBlock.SetColorAndOpacity` _choicetextwidget (make `SlateColor` (struct :`R` 1.0 :`G` 1.0 :`B` 1.0 :`A` 1.0))))))
      (else
        (`KismetSystemLibrary.Delay` (`self.CurrentDelay`))
        (`self.HandleDialogue`)))))

(event `self.ReceiveBeginPlay`
  (bind _outactors (`GameplayStatics.GetAllActorsOfClass` "/Game/Mechanics/DialogueSystem/PartnerConversations/BP_PartnerDialogueArea.BP_PartnerDialogueArea_C"))
  (for _array_element _outactors
    (set `/Game/Mechanics/DialogueSystem/PartnerConversations/BP_PartnerDialogueArea.DialogueManager` self _array_element)))

(fn `CallDialogue`
  (params (DialogueToCall :type "DataTable Object Reference"))
  (bind _dialoguevariables (`self.DialogueVariables`))
  ;[0.2956 0.3941 1] When passed a dialogue from a dialogue actor, prepare all the relevant variables and begin to run the dialogue.
  (set `self.CurrentDialogue` DialogueToCall)
  (set `self.bIsDialoguePlaying?` true)
  (set `self.CurrentDelay` 0.0)
  (set `self.DialogueEntryIndex` "0")
  (`BlueprintMapLibrary.Map_Clear` (`self.DialogueVariables`))
  (bind _outrownames (`DataTableFunctionLibrary.GetDataTableRowNames` (`self.CurrentDialogue`)))
  (for _array_element _outrownames
    (bind _returnvalue (`|GetDataTableRow` (`self.CurrentDialogue`) _array_element)
      (:`then`
        (bind (_variableid _variablename _value) (break `/Game/Mechanics/DialogueSystem/PartnerConversations/Dialogues/ChoiceStructure` (`.VariableSet_15_B28A1423415E66C759C33AA18E7B3634` (break `/Game/Mechanics/DialogueSystem/PartnerConversations/Dialogues/DialogueStructure` _returnvalue))))
        (if (!= _variableid 0)
          (if (not (`BlueprintMapLibrary.Map_Contains` _dialoguevariables _variablename))
            (`BlueprintMapLibrary.Map_Add` _dialoguevariables _variablename _value)
            (set `self.SelectedChoice` 0)))))))

(fn `EndDialogue`
  ;[0 0.7405 1] End the current dialogue
  (set `self.bIsDialoguePlaying?` false))

(fn `HandleDialogue`
  (bind _dialoguewidget (`self.DialogueWidget`))
  (bind _dialoguewidget_2 (`self.DialogueWidget`))
  ;[0.1264 1 0.1388] Branch based on if the choice menu is currently open
  (if (== (`self.DialogueEntryIndex`) "ChoiceMenu")
    ;[0.3372 0.6665 1] If the choice menu is open, prepare the choice menu
    (for _array_element (`self.CurrentDialogueChoices`)
      (bind _returnvalue (`|GetDataTableRow` (`self.CurrentDialogue`) (`KismetStringLibrary.Conv_StringToName` (`KismetStringLibrary.Conv_IntToString` _array_element)))
        (:`then`
          (bind _returnvalue_2 (`|CreateWidget` "/Game/Mechanics/DialogueSystem/PartnerConversations/BP_PartnerDialogueChoice.BP_PartnerDialogueChoice_C" (`GameplayStatics.GetPlayerController` 0)))
          (bind (_lineid _variablecheck _characterspeaking _characterdialogue _linkedchoices _variableset) (break `/Game/Mechanics/DialogueSystem/PartnerConversations/Dialogues/DialogueStructure` _returnvalue))
          (set `/Game/Mechanics/DialogueSystem/PartnerConversations/BP_PartnerDialogueChoice.ChoiceText` _characterdialogue _returnvalue_2)
          (bind (_variableid _variablename _value) (break `/Game/Mechanics/DialogueSystem/PartnerConversations/Dialogues/ChoiceStructure` _variableset))
          (set `/Game/Mechanics/DialogueSystem/PartnerConversations/BP_PartnerDialogueChoice.ChoiceVariableName` _variablename _returnvalue_2)
          (set `/Game/Mechanics/DialogueSystem/PartnerConversations/BP_PartnerDialogueChoice.ChoiceVariableValue` _value _returnvalue_2)
          (`KismetArrayLibrary.Array_Add` (`self.DialogueChoiceWidgets`) _returnvalue_2)
          (`VerticalBox.AddChildToVerticalBox` (`/Game/Mechanics/DialogueSystem/PartnerConversations/BP_PartnerDialogueMain.ChoiceArea` (`self.DialogueWidget`)) _returnvalue_2)
          (set `self.bIsChoiceMenuOpen?` true)
          (set `self.SelectedChoice` 0)
          (set `self.CurrentDelay` 0.0))))
    (else
      ;[1 0.1136 0.1534] Create the next dialogue in the sequence, then set the relevant variables based on it.
      (if (!= _dialoguewidget_2 null)
        (`Widget.RemoveFromParent` _dialoguewidget_2))
      (if (== (`self.DialogueEntryIndex`) "EndDialogue")
        (`self.EndDialogue`)
        (else
          (bind _returnvalue_3 (`|CreateWidget` "/Game/Mechanics/DialogueSystem/PartnerConversations/BP_PartnerDialogueMain.BP_PartnerDialogueMain_C" (`GameplayStatics.GetPlayerController` 0)))
          (bind _output_get (set `self.DialogueWidget` _returnvalue_3))
          (`UserWidget.AddToViewport` _output_get 0)
          (bind _returnvalue_4 (`|GetDataTableRow` (`self.CurrentDialogue`) (`self.DialogueEntryIndex`))
            (:`then`
              (`|ExecutionSequence`
                (:`then_0`
                  (bind (_lineid_2 _variablecheck_2 _characterspeaking_2 _characterdialogue_2 _linkedchoices_2 _variableset_2 _onendgoto _soundevent _timelength _relatedobjecttag _calledeventname _soundtoplay) (break `/Game/Mechanics/DialogueSystem/PartnerConversations/Dialogues/DialogueStructure` _returnvalue_4))
                  (if (!= _soundtoplay null)
                    (`GameplayStatics.PlaySound2D` _soundtoplay)))
                (:`then_1`
                  ;[1 0.3569 0] Call relevant events in other objects
                  (if (`KismetStringLibrary.NotEqual_StrStr` _relatedobjecttag)
                    (bind _outactors (`GameplayStatics.GetAllActorsWithTag` (`KismetStringLibrary.Conv_StringToName` _relatedobjecttag)))
                    (for _array_element_2 _outactors
                      (`KismetSystemLibrary.K2_SetTimer` _array_element_2 _calledeventname 1e-06))))
                (:`then_2`
                  (set `/Game/Mechanics/DialogueSystem/PartnerConversations/BP_PartnerDialogueMain.SpeakerName` _characterspeaking_2 _dialoguewidget)
                  (set `/Game/Mechanics/DialogueSystem/PartnerConversations/BP_PartnerDialogueMain.SpeakerDialogue` _characterdialogue_2 _dialoguewidget)
                  (set `self.CurrentDelay` _timelength)
                  (bind _output_get_2 (set `self.DialogueEntryIndex` (`KismetStringLibrary.Conv_StringToName` _onendgoto)))
                  (if (== _output_get_2 "ChoiceMenu")
                    (set `self.CurrentDialogueChoices` _linkedchoices_2))
                  (return))))))))))

(fn `UserConstructionScript`)
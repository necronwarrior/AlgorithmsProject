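; Passive NPC Blueprint for the dialogue system that handles player interaction and conversation end.
; Important NPCs teleport the player to an optional dialogue spot or turn to face them, then run custom camera setup or standard dialogue.
; Others add ordered or random lines, optionally turning to the player.
; Ending resets camera and widget, resumes patrol and player walking, destroys the actor and notifies FirstPersonCharacter.
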(event `self.OnInteract`
  (params (PlayerChar :type "/Game/Character/FirstPersonCharacter Object Reference"))
  ;[1 1 1] On Interact with Player
  (set `self.PlayerChar` PlayerChar)
  (if (`self.isImportant?`)
    (if (not (`self.isTalking?`))
      (set `self.isTalking?` true)
      (set `self.CurrentDialogueIndex` 0)
      (`/Engine/EditorBlueprintResources/StandardMacros.IsValid` (`self.DialoguePlayerLocation`)
        (:`Is Valid`
          (`self.K2_SetActorLocation` (`self.PlayerChar`) (`self.K2_GetActorLocation` (`self.DialoguePlayerLocation`)) false false)
          (`self.PlayerTurnToNpc`))
        (:`Is Not Valid`
          (`self.TurnToPlayer`)))
      (`SceneComponent.SetVisibility` (`self.NPCWidget`) false false)
      (if (`self.hasCustomBehaviour?`)
        (`self.SwitchToNewCamera` (`self.FirstCameraActor`))
        (`self.AfterConversationSetup`)
        (else
          (`self.HandleCamera`)
          (`self.ShowNextImportantDialogue` 0))))
    (else
      (switch `/Game/Mechanics/DialogueSystem/Blueprints/Enums/e_DialogueSelectionTypes` (`self.selectionType`)
        (:`NewEnumerator0`
          _)
        (:`NewEnumerator1`
          (set `self.CurrentDialogueIndex` (`KismetMathLibrary.RandomIntegerInRange` 0 (`KismetArrayLibrary.Array_LastIndex` (`self.Dialogues`))))))
      (if (not (`self.isTalking?`))
        (`self.AddDialogue`)
        (if (`self.StopMovingWhenTalking?`)
          (`self.TurnToPlayer`))))))

(event `self.EndConversation`
  ;[1 1 1] End Conversation
  (set `self.CurrentDialogueIndex` 0)
  (`SceneComponent.SetVisibility` (`self.NPCWidget`) (`self.isPlayerRadius?`) false)
  (`self.ResetCamera`)
  (`self.MoveToNextPatrolPoint`)
  (`CharacterMovementComponent.SetMovementMode` (`Character.CharacterMovement` (`self.PlayerChar`)) "MOVE_Walking" 0)
  (`self.K2_DestroyActor`)
  (bind _asfirst_person_character (cast `/Game/Character/FirstPersonCharacter` (`GameplayStatics.GetPlayerCharacter` 0)))
  (`/Game/Character/FirstPersonCharacter.PlayerEndConversation` _asfirst_person_character))

(fn `UserConstructionScript`
  (`parent.UserConstructionScript`))
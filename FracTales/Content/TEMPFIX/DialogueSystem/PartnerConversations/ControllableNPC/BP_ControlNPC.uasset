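; BP_ControlNPC is an NPC Blueprint that starts a partner conversation when interacted with.
; On BeginPlay it caches the first BP_PartnerDialogueManager found in the level.
; Interact passes the NPC's AttatchedDialogue to that manager's CallDialogue, but only while no dialogue is already playing.
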(event `self.ReceiveBeginPlay`
  (bind _outactors (`GameplayStatics.GetAllActorsOfClass` "/Game/DialogueSystem/PartnerConversations/BP_PartnerDialogueManager.BP_PartnerDialogueManager_C"))
  (set `self.DialogueManager` (`|GetArrayItem` _outactors)))

(fn `Interact`
  (if (not (`/Game/DialogueSystem/PartnerConversations/BP_PartnerDialogueManager.bIsDialoguePlaying?` (`self.DialogueManager`)))
    (`/Game/DialogueSystem/PartnerConversations/BP_PartnerDialogueManager.CallDialogue` (`self.DialogueManager`) (`self.AttatchedDialogue`))))

(fn `UserConstructionScript`)
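; BP_Plants is a clickable plant object that completes a watering step, apparently for the Day 1 Task 3 content.
; On PlayerClick, after checking TaskGivingObject, it sets that object as the first-person character's next task reference and flags its watering as finished.
; It then swaps every material slot on the static mesh of each TreeList entry to BasicAsset03 as a visual change.
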(event `self.ReceiveBeginPlay`)

(event `Player Click`
  (bind _taskgivingobject (`self.TaskGivingObject`))
  (if (!= (`self.TaskGivingObject`) null)
    (bind _asfirst_person_character (cast `/Game/TestingGrounds/FPTestingZone/Blueprints/FirstPersonCharacter` (`GameplayStatics.GetPlayerCharacter` 0)))
    (set `/Game/TestingGrounds/FPTestingZone/Blueprints/FirstPersonCharacter.NextTaskObjectReference` _taskgivingobject _asfirst_person_character)
    (set `/Game/TestingGrounds/TaskListObjects/Day1/BP_WateringCan.bIsFinishedWatering` true _taskgivingobject)
    (for _array_element (`self.TreeList`)
      (bind _returnvalue (`self.GetComponentByClass` _array_element "/Script/Engine.StaticMeshComponent"))
      (for _index (range (+ (`PrimitiveComponent.GetNumMaterials` _returnvalue) 1))
        (`PrimitiveComponent.SetMaterial` _returnvalue _index "/Engine/MapTemplates/Materials/BasicAsset03.BasicAsset03")))))

(fn `UserConstructionScript`
  (`parent.UserConstructionScript`))
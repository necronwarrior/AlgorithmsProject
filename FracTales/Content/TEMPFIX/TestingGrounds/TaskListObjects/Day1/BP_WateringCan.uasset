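; Watering can task object for Day 1 that the player picks up, uses on a planter and hands back.
; A click saves the player's right-hand object, attaches the can's hand object to the GripPoint socket, and links the Planter as next task, with itself as task giver.
; Once IsFinishedWatering is set externally, a click restores the saved item, detaches the can, resets the flag and calls TaskFinished.
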(event `self.ReceiveBeginPlay`
  (`parent.ReceiveBeginPlay`))

(event `self.PlayerClick`
  (params (PlayerCharacter :type "/Game/TestingGrounds/FPTestingZone/Blueprints/FirstPersonCharacter Object Reference") (TagFunctionality :type Name))
  (bind _righthandobject (`self.RightHandObject`))
  ;[1 1 1] Check If this is next task, space for any other checks
  (if (`self.bIsFinishedWatering`)
    (set `/Game/TestingGrounds/FPTestingZone/Blueprints/FirstPersonCharacter.RightHandObject` (`self.TempHandObject`) PlayerCharacter)
    (`SceneComponent.K2_DetachFromComponent` (`self.RightHandObject`) "KeepRelative" "KeepRelative" "KeepRelative" true)
    (set `self.bIsFinishedWatering` false)
    (`self.TaskFinished`)
    (else
      (`parent.PlayerClick` PlayerCharacter TagFunctionality)
      (set `self.TempHandObject` (`/Game/TestingGrounds/FPTestingZone/Blueprints/FirstPersonCharacter.RightHandObject` PlayerCharacter))
      ;[1 1 1] Conditions for finishing task
      (set `/Game/TestingGrounds/FPTestingZone/Blueprints/FirstPersonCharacter.NextTaskObjectReference` (`self.Planter`) PlayerCharacter)
      (set `/Game/TestingGrounds/FPTestingZone/Blueprints/FirstPersonCharacter.RightHandObject` _righthandobject PlayerCharacter)
      (`SceneComponent.K2_AttachToComponent` _righthandobject (`/Game/TestingGrounds/FPTestingZone/Blueprints/FirstPersonCharacter.Mesh2P` PlayerCharacter) "GripPoint" "SnapToTarget" "SnapToTarget" "SnapToTarget" true)
      (set `/Game/TestingGrounds/TaskListObjects/Day1/Day1Task3Extras/BP_Plants.TaskGivingObject` self (`self.Planter`)))))

(fn `UserConstructionScript`
  (`parent.UserConstructionScript`))
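; BP_signpost runs the game's ending sequence through its PlayEnding event.
; It starts a siren and shows an endgame widget using a dynamic material, whose opacity Tick ramps up while progressively slowing the player's walk speed.
; After a timed delay it changes the player's control structure, removes the task list, silences audio and finishes the alarm effect.
; It then switches to UI-only input, plays Sam's crying dialogue and reveals a button.
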(event `self.ReceiveTick`
  (params (DeltaSeconds :type "Float (single-precision)"))
  (bind _charactermovement (`Character.CharacterMovement` (cast `/Game/Character/FirstPersonCharacter` (`GameplayStatics.GetPlayerCharacter` 0) :!pure true)))
  (if (`self.NewVar_0`)
    (bind _output_get (set `self.DeltaTime` (+ (/ DeltaSeconds 8.0) (`self.DeltaTime`))))
    (`MaterialInstanceDynamic.SetScalarParameterValue` (`self.EndgameRedStatic`) "Opacity" _output_get)
    (set `CharacterMovementComponent.MaxWalkSpeed` (- (`CharacterMovementComponent.MaxWalkSpeed` _charactermovement) (* 10 (`self.DeltaTime`))) _charactermovement)))

(event `PlayEnding`
  (bind _returnvalue (`GameplayStatics.GetPlayerController` 0))
  (bind _endgameredstatic (`self.EndgameRedStatic`))
  (bind _endgameplayerwidget (`self.EndgamePlayerWidget`))
  (bind _endgameredstatic_2 (`self.EndgameRedStatic`))
  (bind _asfirst_person_character (cast `/Game/Character/FirstPersonCharacter` (`GameplayStatics.GetPlayerCharacter` 0) :!pure true))
  (`AkGameplayStatics.PostEventAtLocation` "/Game/Audio/Wwise/Events/sfx/objects/non-destructable/tower/siren_start.siren_start" (`self.K2_GetActorLocation` (`GameplayStatics.GetPlayerCharacter` 0)))
  ;[1 1 1] Begin ending sequence
  ;;[1 1 1] Audio siren
  (set `self.NewVar_0` true)
  (bind _returnvalue_2 (`KismetMaterialLibrary.CreateDynamicMaterialInstance` "/Game/EndgameSequence/EndgamePlayerScreen_mat.EndgamePlayerScreen_mat"))
  (set `self.EndgameRedStatic` _returnvalue_2)
  (bind _returnvalue_3 (`|CreateWidget` "/Game/EndgameSequence/BP_EndgameWidget.BP_EndgameWidget_C"))
  (bind _output_get (set `self.EndgamePlayerWidget` _returnvalue_3))
  (`Image.SetBrushFromMaterial` (`/Game/EndgameSequence/BP_EndgameWidget.Visual_Alarm` _output_get) _endgameredstatic_2)
  (`MaterialInstanceDynamic.SetScalarParameterValue` _endgameredstatic_2 "Opacity" 0.0)
  (`UserWidget.AddToViewport` (`self.EndgamePlayerWidget`) 0)
  (`KismetSystemLibrary.Delay` 10.0)
  (`/Game/Character/FirstPersonCharacter.SetControlStructure` _asfirst_person_character "NewEnumerator1")
  (`TimelineComponent.SetPlayRate` (`/Game/Character/FirstPersonCharacter.Footsteps Timeline` _asfirst_person_character) 0.0)
  (`Widget.RemoveFromParent` (`/Game/Character/FirstPersonCharacter.PlayerTaskListWidget` _asfirst_person_character))
  ;;[1 1 1] Stop all noises
  (`AkGameplayStatics.StopAll`)
  (`self.SetActorTickEnabled` false)
  (`MaterialInstanceDynamic.SetScalarParameterValue` _endgameredstatic "AlarmFinished" 1.0)
  (`MaterialInstanceDynamic.SetScalarParameterValue` _endgameredstatic "Opacity" 1.0)
  (`WidgetBlueprintLibrary.SetInputMode_UIOnlyEx` _returnvalue _endgameplayerwidget)
  (set `PlayerController.bShowMouseCursor` true _returnvalue)
  (`/Game/MacroLibrary/BML_ActorUtilities.PlayDialogue` "/Game/EndgameSequence/EndgameSamCry.EndgameSamCry")
  (`KismetSystemLibrary.Delay` 0.5)
  (`Widget.SetVisibility` (`/Game/EndgameSequence/BP_EndgameWidget.Button_165` _endgameplayerwidget) "Visible"))

(fn `UserConstructionScript`)
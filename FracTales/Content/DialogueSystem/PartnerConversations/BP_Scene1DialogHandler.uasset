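; BP_Scene1DialogHandler sequences partner conversation lines for Scene 1 of the dialogue system.
; Each S1_n event stands for a dialogue beat, and some look up BP_PartnerDialogueManager to schedule follow-up lines after a delay.
; S1_1 queues S1_3 and S1_3 queues S1_4, while S1_5 deactivates Scene 1 dialogue and activates Scene 2.
; S1_2 and S1_4 are empty.
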(event `S1_1`
  (bind _outactors (`GameplayStatics.GetAllActorsOfClass` "/Game/DialogueSystem/PartnerConversations/BP_PartnerDialogueManager.BP_PartnerDialogueManager_C"))
  (`/Game/DialogueSystem/PartnerConversations/BP_PartnerDialogueManager.CallDialogueAfterDelay` (`|GetArrayItem` _outactors) 45.0 "/Game/DialogueSystem/PartnerConversations/DialogueChanges/Scene_1/S1_3.S1_3"))

(event `S1_2`)

(event `S1_3`
  (bind _outactors (`GameplayStatics.GetAllActorsOfClass` "/Game/DialogueSystem/PartnerConversations/BP_PartnerDialogueManager.BP_PartnerDialogueManager_C"))
  (`/Game/DialogueSystem/PartnerConversations/BP_PartnerDialogueManager.CallDialogueAfterDelay` (`|GetArrayItem` _outactors) 30.0 "/Game/DialogueSystem/PartnerConversations/DialogueChanges/Scene_1/S1_4.S1_4"))

(event `S1_4`)

(event `S1_5`
  (bind _outactors (`GameplayStatics.GetAllActorsOfClass` "/Game/DialogueSystem/PartnerConversations/BP_PartnerDialogueManager.BP_PartnerDialogueManager_C"))
  (bind _output (`|GetArrayItem` _outactors))
  (`/Game/DialogueSystem/PartnerConversations/BP_PartnerDialogueManager.DeactivateDialogueByScene` _output 1)
  (`/Game/DialogueSystem/PartnerConversations/BP_PartnerDialogueManager.ActivateDialogueByScene` _output 2))

(fn `UserConstructionScript`)
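; Controllable NPC that patrols waypoints, plays partner dialogue on interaction and carries out a task chosen for the next day.
; Sleep and MainGate queue NextTask; the player's next-day event makes it current, selecting the matching patrol path and setting rotation.
; Patrolling loops by re-calling AIMoveTo on each success.
; While the task is SleepIn, Tick randomizes the actor's rotation every frame.
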(event `self.ReceiveBeginPlay`
  (bind _outactors (`GameplayStatics.GetAllActorsOfClass` "/Game/DialogueSystem/PartnerConversations/BP_PartnerDialogueManager.BP_PartnerDialogueManager_C"))
  (set `self.DialogueManager` (`|GetArrayItem` _outactors))
  (`self.MoveToNextPatrolPoint`)
  (set `self.NextTask` (`self.CurrentTask`)) ; Set next task to current task so that NPC repeats task unless told otherwise
  (bind _asfirst_person_character (cast `/Game/Character/FirstPersonCharacter` (`GameplayStatics.GetPlayerCharacter` 0)))
  (add `/Game/Character/FirstPersonCharacter.CallNextDay` _asfirst_person_character (delegate `CallNextDay`)))

(event `CallNextDay`
  (`self.OnNextDayStart`))

(event `self.ReceiveTick`
  (params (DeltaSeconds :type "Float (single-precision)"))
  (if (`|EnumEquality` (`self.CurrentTask`) "NewEnumerator3")
    (`self.K2_SetActorRotation` (`KismetMathLibrary.MakeRotator` (`KismetMathLibrary.RandomFloatInRange` -180.0 180.0) (`KismetMathLibrary.RandomFloatInRange` -180.0 180.0)))))

(event `MoveToNextPatrolPoint`
  (bind _currentpatrolpoint (`self.CurrentPatrolPoint`))
  (bind _output (`|GetArrayItem` (`self.CurrentWalkingPath`) (`self.CurrentPatrolPoint`)))
  (if (`self.bHasWalkingPath?`)
    (`/Engine/EditorBlueprintResources/StandardMacros.IsValid` _output
      (:`Is Valid`
        (`|AIMoveTo` self self (`self.K2_GetActorLocation` _output)
          (:`OnSuccess`
            (set `self.CurrentPatrolPoint` (select `bool` (== _currentpatrolpoint (`KismetArrayLibrary.Array_LastIndex` (`self.CurrentWalkingPath`))) :`false` (+ _currentpatrolpoint 1)))
            (`self.MoveToNextPatrolPoint`)))))))

(fn `Interact`
  (if (not (`/Game/DialogueSystem/PartnerConversations/BP_PartnerDialogueManager.bIsDialoguePlaying?` (`self.DialogueManager`)))
    (`/Game/DialogueSystem/PartnerConversations/BP_PartnerDialogueManager.CallDialogue` (`self.DialogueManager`) (`self.AttatchedDialogue`))))

(fn `MainGate`
  (set `self.NextTask` "NewEnumerator2"))

(fn `OnNextDayStart`
  (bind _output_get (set `self.CurrentTask` (`self.NextTask`)))
  (for _array_element (`self.NPCPaths`)
    (bind (_relatedtask _patrolpoints) (break `/Game/Structs/SNPCMovePath` _array_element))
    (if (`|EnumEquality` _relatedtask (`self.CurrentTask`))
      (set `self.CurrentWalkingPath` _patrolpoints)))
  (switch `/Game/Enums/ENPCTasks` _output_get
    (:`NewEnumerator2`
      (`self.K2_SetActorRotation` (struct)))
    (:`NewEnumerator3`
      (`self.K2_SetActorRotation` (`KismetMathLibrary.MakeRotator` 0.0 90.0)))))

(fn `Sleep`
  (set `self.NextTask` "NewEnumerator3"))

(fn `UserConstructionScript`)
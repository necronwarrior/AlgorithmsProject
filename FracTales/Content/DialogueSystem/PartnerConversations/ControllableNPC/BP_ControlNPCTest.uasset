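; Test controllable NPC for the dialogue system that visibly reacts to a "Sleep in" task.
; Sleep queues SleepIn as the next task.
; While the current task is Sleep in, Tick randomizes the actor's roll and pitch every frame.
; OnNextDayStart calls the parent implementation, then applies a fixed rotation on its Sleep in case.
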(event `self.ReceiveTick`
  (params (DeltaSeconds :type "Float (single-precision)"))
  (`parent.ReceiveTick` DeltaSeconds)
  (switch `/Game/Enums/ENPCTasks` (`self.CurrentTask`)
    (:`NewEnumerator3`
      (`self.K2_SetActorRotation` (`KismetMathLibrary.MakeRotator` (`KismetMathLibrary.RandomFloatInRange` -180.0 180.0) (`KismetMathLibrary.RandomFloatInRange` -180.0 180.0))))))

(fn `OnNextDayStart`
  (returns (CurTask :type "/Game/Enums/ENPCTasks Enum"))
  (bind _curtask (`parent.OnNextDayStart`))
  (switch `/Game/Enums/ENPCTasks` "NewEnumerator0"
    (:`NewEnumerator0`
      (return _curtask))
    (:`NewEnumerator3`
      (`self.K2_SetActorRotation` (struct :`Pitch` 90.0)))))

(fn `Sleep`
  (set `self.NextTask` "NewEnumerator3"))

(fn `UserConstructionScript`
  (`parent.UserConstructionScript`))
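; Test controllable NPC for the garden that shadows the player's junction-to-junction movement along its own path.
; BeginPlay binds to the player's junction event and collects five tagged garden junctions.
; While following is enabled, the player's chosen junction is matched by index to NPCGardenPath and walked via inherited patrol movement.
; Tick turns its widget toward the player camera; older beam and displacement-mirroring logic is left disconnected.
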(event Custom|StopFollow
  (Variables|Default|SetbCanMoveToNextJunction? false))

(event Custom|MovedToNextJunction
  (if (Variables|Default|GetbCanMoveToNextJunction?)
    (bind _asfirst_person_character (Utilities|Casting|CastToFirstPersonCharacter (Game|GetPlayerCharacter 0)))
    (for (_array_element _array_index) (Variables|Default|GetPlayerGardenPath)
      (if (== (Utilities|Array|Get(acopy) (Variables|/Game/Mechanics/GridDirectionLines/BP_RailJunction.BP_RailJunction_C|GetJunctionList (Variables|/Game/Character/FirstPersonCharacter.FirstPersonCharacter_C|GetCurrentJunction _asfirst_person_character)) (Variables|/Game/Mechanics/GridDirectionLines/BP_RailJunction.BP_RailJunction_C|GetJunctionChoice (Variables|/Game/Character/FirstPersonCharacter.FirstPersonCharacter_C|GetCurrentJunction _asfirst_person_character))) _array_element)
        (Variables|Default|SetCurrentWalkingPath (Utilities|Array|MakeArray (Utilities|Array|Get(acopy) (Variables|Default|GetNPCGardenPath) _array_index)))
        (CallFunction|MovetoNextPatrolPoint)))))

(event Custom|BeginFollow
  (Variables|Default|SetbCanMoveToNextJunction? true))

(event EventBeginPlay
  (bind _charactermovement (Variables|Character|GetCharacterMovement))
  (|CallParentFunction)
  (Variables|/Script/Engine.CharacterMovementComponent|SetMaxAcceleration _charactermovement 9999999999.0)
  (Variables|/Script/Engine.CharacterMovementComponent|SetMaxWalkSpeed _charactermovement 7e+02)
  (bind _asfirst_person_character (Utilities|Casting|CastToFirstPersonCharacter (Game|GetPlayerCharacter 0)))
  (EventDispatchers|BindEventtoMovedtoNextJunction _asfirst_person_character (delegate Custom|MovedToNextJunction))
  (Utilities|FlowControl|Sequence
    (:then_0
      (bind _outactors (Actor|GetAllActorswithTag "GardenJunction1"))
      (bind _asbp_master_patrol_point (Utilities|Casting|CastToBP_MasterPatrolPoint (Utilities|Array|Get(acopy) _outactors)))
      (Utilities|Array|Add (Variables|Default|GetPlayerGardenPath) _asbp_master_patrol_point))
    (:then_1
      (bind _outactors_2 (Actor|GetAllActorswithTag "GardenJunction2"))
      (bind _asbp_master_patrol_point_2 (Utilities|Casting|CastToBP_MasterPatrolPoint (Utilities|Array|Get(acopy) _outactors_2)))
      (Utilities|Array|Add (Variables|Default|GetPlayerGardenPath) _asbp_master_patrol_point_2))
    (:then_2
      (bind _outactors_3 (Actor|GetAllActorswithTag "GardenJunction3"))
      (bind _asbp_master_patrol_point_3 (Utilities|Casting|CastToBP_MasterPatrolPoint (Utilities|Array|Get(acopy) _outactors_3)))
      (Utilities|Array|Add (Variables|Default|GetPlayerGardenPath) _asbp_master_patrol_point_3))
    (:then_3
      (bind _outactors_4 (Actor|GetAllActorswithTag "GardenJunction4"))
      (bind _asbp_master_patrol_point_4 (Utilities|Casting|CastToBP_MasterPatrolPoint (Utilities|Array|Get(acopy) _outactors_4)))
      (Utilities|Array|Add (Variables|Default|GetPlayerGardenPath) _asbp_master_patrol_point_4))
    (:then_4
      (bind _outactors_5 (Actor|GetAllActorswithTag "GardenJunction5"))
      (bind _asbp_master_patrol_point_5 (Utilities|Casting|CastToBP_MasterPatrolPoint (Utilities|Array|Get(acopy) _outactors_5)))
      (Utilities|Array|Add (Variables|Default|GetPlayerGardenPath) _asbp_master_patrol_point_5))))

(event Collision|EventActorBeginOverlap
  (params (OtherActor :type Actor%20Object%20Reference))
  (|CallParentFunction OtherActor))

(event EventTick
  (params (DeltaSeconds :type Float%20%28single-precision%29))
  (bind _widget (Variables|Default|GetWidget))
  (|CallParentFunction DeltaSeconds)
  (bind _asfirst_person_character (Utilities|Casting|CastToFirstPersonCharacter (Game|GetPlayerCharacter 0)))
  (Transformation|SetWorldRotation _widget (Math|Rotator|FindLookatRotation (Transformation|GetWorldLocation _widget) (Transformation|GetWorldLocation (Variables|/Game/Character/FirstPersonCharacter.FirstPersonCharacter_C|GetFirstPersonCamera _asfirst_person_character))) false false))

(event EventMovetoNextPatrolPoint
  (|CallParentFunction))

(fn ConstructionScript
  (|CallParentFunction))

(fn MovetoNextSetOfPatrolPoints)
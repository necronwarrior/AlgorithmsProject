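; BP_GateOpeningNPC is a dialogue NPC that opens a gate as time skips to the next day.
; OpenGate runs a screen fade and, on completion, calls SimulateNextDay on the FirstPersonCharacter.
; It then starts the opposite fade and, without waiting for it to finish, switches its attached dialogue to the completed ControlDialogue01 and calls GateOpening.
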(event `OpenGate`
  (bind _returnvalue (`GameplayStatics.GetPlayerPawn` 0))
  (`/Game/MacroLibrary/BML_ActorUtilities.FadeInOut` _returnvalue true
    (:`Completed`
      (bind _asfirst_person_character (cast `/Game/Character/FirstPersonCharacter` (`GameplayStatics.GetPlayerCharacter` 0)))
      (`/Game/Character/FirstPersonCharacter.SimulateNextDay` _asfirst_person_character)
      (`/Game/MacroLibrary/BML_ActorUtilities.FadeInOut` _returnvalue
        (:`Then`
          (set `self.AttatchedDialogue` "/Game/DialogueSystem/PartnerConversations/ControllableNPC/ControllableDialogues/ControlDialogue01_Complete.ControlDialogue01_Complete")
          (`self.GateOpening`))))))

(fn `UserConstructionScript`
  (`parent.UserConstructionScript`))
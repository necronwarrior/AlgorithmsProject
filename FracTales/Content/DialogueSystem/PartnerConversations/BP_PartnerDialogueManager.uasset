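; Manager for partner conversations that plays DataTable-driven dialogue with timed lines and player choice menus.
; CallDialogue seeds a variable map from the table, then Tick uses a Delay to pace HandleDialogue, which rebuilds the dialogue widget and follows each row's OnEndGoTo.
; ChoiceMenu entries spawn linked choice widgets, highlighted on Tick and navigated by accumulated mouse-wheel input.
; Right-click confirms, stores the choice's variable and jumps to its next row.
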(event `MouseRightClick`
  (bind _dialoguechoicewidgets (`self.DialogueChoiceWidgets`))
  (if (`self.bIsChoiceMenuOpen?`)
    (bind _returnvalue (`|GetDataTableRow` (`self.CurrentDialogue`) (`KismetStringLibrary.Conv_StringToName` (`KismetStringLibrary.Conv_IntToString` (`|GetArrayItem` (`self.CurrentDialogueChoices`) (`self.SelectedChoice`)))))
      (:`then`
        (bind (_lineid _variablecheck _characterspeaking _characterdialogue _linkedchoices _variableset _onendgoto) (break `/Game/DialogueSystem/PartnerConversations/Dialogues/DialogueStructure` _returnvalue))
        (bind (_variableid _variablename _value) (break `/Game/DialogueSystem/PartnerConversations/Dialogues/ChoiceStructure` _variableset))
        (`BlueprintMapLibrary.Map_Add` (`self.DialogueVariables`) _variablename _value)
        (set `self.bIsChoiceMenuOpen?` false)
        (set `self.DialogueEntryIndex` (`KismetStringLibrary.Conv_StringToName` _onendgoto))
        (for _array_element _dialoguechoicewidgets
          (`Widget.RemoveFromParent` _array_element))
        (`KismetArrayLibrary.Array_Clear` (`self.CurrentDialogueChoices`))
        (`KismetArrayLibrary.Array_Clear` _dialoguechoicewidgets)))))

(event `MouseWheelScrolled`
  (params (AxisValue :type "Float (double-precision)"))
  (bind _selectedchoice (`self.SelectedChoice`))
  (bind _selectedchoice_2 (`self.SelectedChoice`))
  (if (`self.bIsChoiceMenuOpen?`)
    (bind _output_get (set `self.MouseScroll` (+ AxisValue (`self.MouseScroll`))))
    (if (>= _output_get 2.0)
      (if (> _selectedchoice 0)
        (set `self.SelectedChoice` (- _selectedchoice 1)))
      (set `self.MouseScroll` 0.0)
      (elif (<= _output_get -2.0)
        (if (< _selectedchoice_2 (- (`KismetArrayLibrary.Array_Length` (`self.CurrentDialogueChoices`)) 1))
          (set `self.SelectedChoice` (+ _selectedchoice_2 1)))
        (set `self.MouseScroll` 0.0)))))

(event `self.ReceiveTick`
  (params (DeltaSeconds :type "Float (single-precision)"))
  (if (`self.bIsDialoguePlaying?`)
    (if (`self.bIsChoiceMenuOpen?`)
      (for (_array_element _array_index) (`self.DialogueChoiceWidgets`)
        (if (== _array_index (`self.SelectedChoice`))
          (bind _choicetextwidget (`/Game/DialogueSystem/PartnerConversations/BP_PartnerDialogueChoice.ChoiceTextWidget` _array_element))
          (`TextBlock.SetColorAndOpacity` _choicetextwidget (make `SlateColor` (struct :`R` 1.0 :`G` 0.218 :`A` 1.0)))
          (else
            (`TextBlock.SetColorAndOpacity` _choicetextwidget (make `SlateColor` (struct :`R` 1.0 :`G` 1.0 :`B` 1.0 :`A` 1.0))))))
      (else
        (`KismetSystemLibrary.Delay` (`self.CurrentDelay`))
        (`self.HandleDialogue`)))))

(fn `CallDialogue`
  (params (DialogueToCall :type "DataTable Object Reference"))
  (bind _dialoguevariables (`self.DialogueVariables`))
  (set `self.CurrentDialogue` DialogueToCall)
  (set `self.bIsDialoguePlaying?` true)
  (set `self.CurrentDelay` 0.0)
  (set `self.DialogueEntryIndex` "0")
  (`BlueprintMapLibrary.Map_Clear` (`self.DialogueVariables`))
  (bind _outrownames (`DataTableFunctionLibrary.GetDataTableRowNames` (`self.CurrentDialogue`)))
  (for _array_element _outrownames
    (bind _returnvalue (`|GetDataTableRow` (`self.CurrentDialogue`) _array_element)
      (:`then`
        (bind (_variableid _variablename _value) (break `/Game/DialogueSystem/PartnerConversations/Dialogues/ChoiceStructure` (`.VariableSet_15_B28A1423415E66C759C33AA18E7B3634` (break `/Game/DialogueSystem/PartnerConversations/Dialogues/DialogueStructure` _returnvalue))))
        (if (!= _variableid 0)
          (if (not (`BlueprintMapLibrary.Map_Contains` _dialoguevariables _variablename))
            (`BlueprintMapLibrary.Map_Add` _dialoguevariables _variablename _value)
            (set `self.SelectedChoice` 0)))))))

(fn `EndDialogue`
  (set `self.bIsDialoguePlaying?` false))

(fn `HandleDialogue`
  (bind _dialoguewidget (`self.DialogueWidget`))
  (bind _dialoguewidget_2 (`self.DialogueWidget`))
  (if (== (`self.DialogueEntryIndex`) "ChoiceMenu")
    (for _array_element (`self.CurrentDialogueChoices`)
      (bind _returnvalue (`|GetDataTableRow` (`self.CurrentDialogue`) (`KismetStringLibrary.Conv_StringToName` (`KismetStringLibrary.Conv_IntToString` _array_element)))
        (:`then`
          (bind _returnvalue_2 (`|CreateWidget` "/Game/DialogueSystem/PartnerConversations/BP_PartnerDialogueChoice.BP_PartnerDialogueChoice_C" (`GameplayStatics.GetPlayerController` 0)))
          (bind (_lineid _variablecheck _characterspeaking _characterdialogue _linkedchoices _variableset) (break `/Game/DialogueSystem/PartnerConversations/Dialogues/DialogueStructure` _returnvalue))
          (set `/Game/DialogueSystem/PartnerConversations/BP_PartnerDialogueChoice.ChoiceText` _characterdialogue _returnvalue_2)
          (bind (_variableid _variablename _value) (break `/Game/DialogueSystem/PartnerConversations/Dialogues/ChoiceStructure` _variableset))
          (set `/Game/DialogueSystem/PartnerConversations/BP_PartnerDialogueChoice.ChoiceVariableName` _variablename _returnvalue_2)
          (set `/Game/DialogueSystem/PartnerConversations/BP_PartnerDialogueChoice.ChoiceVariableValue` _value _returnvalue_2)
          (`KismetArrayLibrary.Array_Add` (`self.DialogueChoiceWidgets`) _returnvalue_2)
          (`VerticalBox.AddChildToVerticalBox` (`/Game/DialogueSystem/PartnerConversations/BP_PartnerDialogueMain.ChoiceArea` (`self.DialogueWidget`)) _returnvalue_2)
          (set `self.bIsChoiceMenuOpen?` true)
          (set `self.SelectedChoice` 0)
          (set `self.CurrentDelay` 0.0))))
    (else
      (if (!= _dialoguewidget_2 null)
        (`Widget.RemoveFromParent` _dialoguewidget_2))
      (if (== (`self.DialogueEntryIndex`) "EndDialogue")
        (`self.EndDialogue`)
        (else
          (bind _returnvalue_3 (`|CreateWidget` "/Game/DialogueSystem/PartnerConversations/BP_PartnerDialogueMain.BP_PartnerDialogueMain_C" (`GameplayStatics.GetPlayerController` 0)))
          (bind _output_get (set `self.DialogueWidget` _returnvalue_3))
          (`UserWidget.AddToViewport` _output_get 0)
          (bind _returnvalue_4 (`|GetDataTableRow` (`self.CurrentDialogue`) (`self.DialogueEntryIndex`))
            (:`then`
              (`|ExecutionSequence`
                (:`then_1`
                  (bind (_lineid_2 _variablecheck_2 _characterspeaking_2 _characterdialogue_2 _linkedchoices_2 _variableset_2 _onendgoto _soundevent _timelength) (break `/Game/DialogueSystem/PartnerConversations/Dialogues/DialogueStructure` _returnvalue_4))
                  (set `/Game/DialogueSystem/PartnerConversations/BP_PartnerDialogueMain.SpeakerName` _characterspeaking_2 _dialoguewidget)
                  (set `/Game/DialogueSystem/PartnerConversations/BP_PartnerDialogueMain.SpeakerDialogue` _characterdialogue_2 _dialoguewidget)
                  (set `self.CurrentDelay` _timelength)
                  (bind _output_get_2 (set `self.DialogueEntryIndex` (`KismetStringLibrary.Conv_StringToName` _onendgoto)))
                  (if (== _output_get_2 "ChoiceMenu")
                    (set `self.CurrentDialogueChoices` _linkedchoices_2))
                  (return))))))))))

(fn `PrepareDialogue`)

(fn `UserConstructionScript`)
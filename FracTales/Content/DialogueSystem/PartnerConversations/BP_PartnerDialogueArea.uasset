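; Trigger-area actor that starts its assigned partner-conversation dialogue when the first-person player walks into it.
; Overlaps from components tagged FrontInteraction are ignored, and only the exact FirstPersonCharacter class qualifies.
; If the player is not already in dialogue, it passes its dialogue to the DialogueManager and optionally destroys itself.
; SimulateOverlap jumps straight to the in-dialogue check, reusing the overlap's cast result and skipping its filters.
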(event `self.TriggerArea.OnComponentBeginOverlap`
  (params (OverlappedComponent :type "PrimitiveComponent Object Reference") (OtherActor :type "Actor Object Reference") (OtherComp :type "PrimitiveComponent Object Reference") (OtherBodyIndex :type Integer) (bFromSweep :type Boolean) (SweepResult :type "HitResult Structure (by ref)"))
  ;[0.3932 1 0.2522] When the player enters the collision of this actor, pass the dialogue related to this actor to the dialog manager to be played.
  (bind _asfirst_person_character (cast `/Game/Character/FirstPersonCharacter` OtherActor))
  (if (`ActorComponent.ComponentHasTag` OtherComp "FrontInteraction")
    _
    (elif (== (`GameplayStatics.GetObjectClass` OtherActor) "/Game/Character/FirstPersonCharacter.FirstPersonCharacter_C")
      (if (not (`/Game/Character/FirstPersonCharacter.bIsInDialogue?` _asfirst_person_character)) :!label _label
        (`/Game/DialogueSystem/PartnerConversations/BP_PartnerDialogueManager.CallDialogue` (`self.DialogueManager`) (`self.DialogueToCall`))
        (if (`self.bDeletedAfterCollision?`)
          (`self.K2_DestroyActor`))))))

(event `SimulateOverlap`
  ;[0.3932 1 0.2522] When the player enters the collision of this actor, pass the dialogue related to this actor to the dialog manager to be played.
  (goto _label))

(fn `UserConstructionScript`)
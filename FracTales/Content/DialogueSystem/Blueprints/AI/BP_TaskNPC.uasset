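; Task-linked NPC that extends a patrolling dialogue NPC, overriding its player-view and dialogue-finished events.
; When the player comes into view while it is idle, it shows its widget and passes the player's task-list state to RelatedTaskObject.
; When dialogue ends, it updates the dialogue index (wrapping in Order mode), resets its UI and resumes patrolling.
; It then marks the task finished if that task is next in the list.
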(event `OnSimpleDialogueFinished`
  (bind _relatedtaskobject (`self.RelatedTaskObject`))
  ;[1 1 1] On Simple Dialogue Finnished (Overide)
  (set `self.CurrentDialogueIndex` (select `/Game/DialogueSystem/Blueprints/Enums/e_DialogueSelectionTypes` (`self.selectionType`) :`NewEnumerator0` (`KismetMathLibrary.SelectInt` 0 (+ (`self.CurrentDialogueIndex`) 1) (== (`self.CurrentDialogueIndex`) (`KismetArrayLibrary.Array_LastIndex` (`self.Dialogues`)))) :`NewEnumerator1` (`self.CurrentDialogueIndex`)))
  (`SceneComponent.SetVisibility` (`self.NPCText`) false false)
  (`SceneComponent.SetVisibility` (`self.NPCWidget`) (`self.isPlayerRadius?`) false)
  (set `self.isTalking?` false)
  (`self.MoveToNextPatrolPoint`)
  (if (`/Game/TestingGrounds/TaskListObjects/BP_PlayerTaskListObjectTemplate.bIsNextTaskInLIst?` _relatedtaskobject)
    (`/Game/TestingGrounds/TaskListObjects/BP_PlayerTaskListObjectTemplate.TaskFinished` _relatedtaskobject)))

(event `OnEnterPlayerView`
  (set `self.isPlayerRadius?` true)
  (if (not (`self.isTalking?`))
    (`SceneComponent.SetVisibility` (`self.NPCWidget`) true false)
    (bind _asfirst_person_character (cast `/Game/TestingGrounds/FPTestingZone/Blueprints/FirstPersonCharacter` (`GameplayStatics.GetPlayerCharacter` 0)))
    (`/Game/TestingGrounds/TaskListObjects/Day1/BP_Day1Task4.InPlayerView` (`self.RelatedTaskObject`) (`/Game/TestingGrounds/FPTestingZone/Blueprints/FirstPersonCharacter.TaskListComplete` _asfirst_person_character) _asfirst_person_character)))

(fn `UserConstructionScript`
  (`parent.UserConstructionScript`))
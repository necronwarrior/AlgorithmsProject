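; BP_VisitTheNeighbour is a task trigger that completes when the player reaches it as the current objective.
; On box overlap, it stores the FirstPersonCharacter and checks for a "Player" component tag and that the character's next task matches its own class.
; A match deactivates PointToDisable and calls TaskFinished.
; Every tick, its TextRender rotates to face the player's first-person camera.
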(event `self.Box.OnComponentBeginOverlap`
  (params (OverlappedComponent :type "PrimitiveComponent Object Reference") (OtherActor :type "Actor Object Reference") (OtherComp :type "PrimitiveComponent Object Reference") (OtherBodyIndex :type Integer) (bFromSweep :type Boolean) (SweepResult :type "HitResult Structure (by ref)"))
  (bind _asfirst_person_character (cast `/Game/Character/FirstPersonCharacter` OtherActor))
  (set `self.PlayerCharacterReference` _asfirst_person_character)
  (if (`ActorComponent.ComponentHasTag` OtherComp "Player")
    (if (== (`/Game/Character/FirstPersonCharacter.NextTaskObjectReference` _asfirst_person_character) (`GameplayStatics.GetObjectClass` self))
      (set `/Game/Mechanics/GridDirectionLines/BP_RailJunction.bIsActive?` false (`self.PointToDisable`))
      (`self.TaskFinished`))))

(event `self.ReceiveTick`
  (params (DeltaSeconds :type "Float (single-precision)"))
  (bind _textrender (`self.TextRender`))
  (bind _asfirst_person_character (cast `/Game/Character/FirstPersonCharacter` (`GameplayStatics.GetPlayerCharacter` 0)))
  (`SceneComponent.K2_SetWorldRotation` _textrender (`KismetMathLibrary.FindLookAtRotation` (`SceneComponent.K2_GetComponentLocation` _textrender) (`SceneComponent.K2_GetComponentLocation` (`/Game/Character/FirstPersonCharacter.FirstPersonCamera` _asfirst_person_character))) false false))

(fn `UserConstructionScript`
  (`parent.UserConstructionScript`))
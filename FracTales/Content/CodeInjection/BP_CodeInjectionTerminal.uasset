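; Terminal actor that displays the code injection UI as soon as play begins.
; On BeginPlay it adds a BP_CodeInjectionBase widget to the viewport and shows player 0's mouse cursor.
; It builds a choice widget for each CodeInjection option, labeled with the selected option and filled with replacement-choice widgets for the available alternatives.
; Selection handling is not in this actor, and its overlap and tick events are unused.
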(event `self.ReceiveBeginPlay`
  (bind _returnvalue (`GameplayStatics.GetPlayerController` 0))
  (bind _returnvalue_2 (`GameplayStatics.GetPlayerController` 0))
  (bind _returnvalue_3 (`|CreateWidget` "/Game/CodeInjection/BP_CodeInjectionBase.BP_CodeInjectionBase_C" _returnvalue))
  (bind _output_get (set `self.CodeInjectionWidget` _returnvalue_3))
  (`UserWidget.AddToViewport` _output_get 0)
  (set `PlayerController.bShowMouseCursor` true _returnvalue)
  (for _array_element (`.Options_4_BE542E9A4FC6A211552ED3B660C15D35` (break `/Game/CodeInjection/SCodeInjection` (`self.CodeInjection`)))
    (bind _returnvalue_4 (`|CreateWidget` "/Game/CodeInjection/BP_CodeInjectionChoice.BP_CodeInjectionChoice_C" _returnvalue_2))
    (bind (_selectedoption _availableoptions) (break `/Game/CodeInjection/SCodeInjectionOptions` _array_element))
    (set `/Game/CodeInjection/BP_CodeInjectionChoice.ChoiceText` _selectedoption _returnvalue_4)
    (for _array_element_2 _availableoptions
      (bind _returnvalue_5 (`|CreateWidget` "/Game/CodeInjection/BP_CodeInjectionReplacementChoice.BP_CodeInjectionReplacementChoice_C" _returnvalue_2))
      (set `/Game/CodeInjection/BP_CodeInjectionReplacementChoice.ChoiceName` _array_element_2 _returnvalue_5)
      (`VerticalBox.AddChildToVerticalBox` (`/Game/CodeInjection/BP_CodeInjectionChoice.VerticalBox_0` _returnvalue_4) _returnvalue_5))
    (`PanelWidget.AddChild` (`/Game/CodeInjection/BP_CodeInjectionBase.VerticalBox` (`self.CodeInjectionWidget`)) _returnvalue_4)))

(fn `UserConstructionScript`)
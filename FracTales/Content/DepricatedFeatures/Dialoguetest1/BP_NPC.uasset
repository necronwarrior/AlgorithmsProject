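; Test NPC actor that opens a dialogue widget when the player interacts with it.
; Pressing E fires a short forward trace from the player; a hit on this NPC creates BP_Dialogue, shows the cursor and disables character input.
; Each tick, the Cube head interpolates toward the player's rotation, or back to its starting rotation when the dialog box is hidden.
; The Dialogue flag toggles on interaction, but only disconnected logic reads it.
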(event `self.ReceiveBeginPlay`
  ;[1 1 1] Get initial rotation of 'Head'
  (set `self.OldRotator` (.rotation (`SceneComponent.GetRelativeTransform` (`self.Cube`)))))

(event `self.ReceiveTick`
  (params (DeltaSeconds :type "Float (single-precision)"))
  (bind _returnvalue (`GameplayStatics.GetPlayerController` 0))
  (bind _returnvalue_2 (`GameplayStatics.GetPlayerCharacter` 0))
  (bind _returnvalue_3 (`self.K2_GetActorLocation` _returnvalue_2))
  (`|ExecutionSequence`
    (:`then_0`
      (if (`/Game/DepricatedFeatures/Dialoguetest1/BP_Dialogue.bIsHidden?` (`self.DialogBox`))
        ;[1 1 1] Reset 'Head' Object of NPC to starting position
        (`SceneComponent.K2_SetRelativeRotation` (`self.Cube`) (`KismetMathLibrary.RInterpTo` (.rotation (`SceneComponent.GetRelativeTransform` (`self.Cube`))) (`self.OldRotator`) 0.1 0.1) false false)
        (else
          ;[1 1 1] Set 'Head' Object of NPC to face player
          (`SceneComponent.K2_SetRelativeRotation` (`self.Cube`) (`KismetMathLibrary.RInterpTo` (.rotation (`SceneComponent.GetRelativeTransform` (`self.Cube`))) (`self.K2_GetActorRotation` (`GameplayStatics.GetPlayerCharacter` 0)) 0.1 0.1) false false)
          (if (== (`GameplayStatics.GetObjectClass` (`self.DialogBox`)) "/Game/DepricatedFeatures/Dialoguetest1/BP_Dialogue.BP_Dialogue_C")
            _))))
    (:`then_1`
      ;[1 1 1] Line Trace from player to detect if this NPC is being selected
      (if (`PlayerController.WasInputKeyJustPressed` (`GameplayStatics.GetPlayerController` 0) "E")
        (bind _outhit (`KismetSystemLibrary.LineTraceSingle` :`Start` _returnvalue_3 :`End` (+ _returnvalue_3 (* (`self.GetActorForwardVector` _returnvalue_2) 300)) :`TraceChannel` "TraceTypeQuery1" :`bIgnoreSelf` false))
        (if (== (`.HitActor` (`GameplayStatics.BreakHitResult` _outhit)) self)
          (set `self.bDialogue` (not (`self.bDialogue`)))
          (bind _returnvalue_4 (`|CreateWidget` "/Game/DepricatedFeatures/Dialoguetest1/BP_Dialogue.BP_Dialogue_C"))
          (bind _output_get (set `self.DialogBox` _returnvalue_4))
          (`UserWidget.AddToViewport` _output_get 0)
          (set `PlayerController.bShowMouseCursor` true _returnvalue)
          (`self.DisableInput` (`GameplayStatics.GetPlayerCharacter` 0) _returnvalue))))))

(fn `UserConstructionScript`)
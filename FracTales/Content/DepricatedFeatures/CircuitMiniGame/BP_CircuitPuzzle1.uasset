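; Circuit puzzle mini-game actor that shows the cursor, orients itself from the player's rotation, and lerps in front of the camera over one second.
; Clicking its three Activatable components toggles their states and recolours child meshes of the wire sequences between yellow, blue and red depthless materials.
; Each click then compares two meshes' material names against the Cylinder's to check the solution, but a match triggers no action.
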(event `self.ReceiveBeginPlay`
  ;[1 1 1] Setting rotation to face player
  (set `PlayerController.bShowMouseCursor` true (`GameplayStatics.GetPlayerController` 0))
  (set `self.StartingPosition` (`KismetMathLibrary.MakeVector` (.x (`self.K2_GetActorLocation`)) (.y (`self.K2_GetActorLocation`)) (- (.z (`self.K2_GetActorLocation`)) 200.0)))
  (`self.K2_SetActorRotation` (`KismetMathLibrary.MakeRotator` (.roll (`self.K2_GetActorRotation` (`GameplayStatics.GetPlayerCharacter` 0))) (.pitch (`self.K2_GetActorRotation` (`GameplayStatics.GetPlayerCharacter` 0))) (+ (.yaw (`self.K2_GetActorRotation` (`GameplayStatics.GetPlayerCharacter` 0))) 90.0))))

(event `self.ReceiveTick`
  (params (DeltaSeconds :type "Float (single-precision)"))
  (bind _returnvalue (`GameplayStatics.GetPlayerCameraManager` 0))
  (bind _lerpdeltatime (`self.LerpDeltaTime`))
  ;[1 1 1] Lerping to in front of player
  (set `self.LerpDeltaTime` (+ DeltaSeconds (`self.LerpDeltaTime`)))
  (if (< _lerpdeltatime 1.0)
    (`self.K2_SetActorLocation` (`KismetMathLibrary.VLerp` (`self.StartingPosition`) (+ (`self.K2_GetActorLocation` _returnvalue) (* (`self.GetActorForwardVector` _returnvalue) 250.0)) _lerpdeltatime))))

(event `self.Activatable1.OnClicked`
  (params (TouchedComponent :type "PrimitiveComponent Object Reference") (ButtonPressed :type "Key Structure"))
  (bind _bactivatable1clicked_ (`self.bActivatable1Clicked?`))
  (set `self.bActivatable1Clicked?` (not _bactivatable1clicked_))
  (if _bactivatable1clicked_
    (`self.ChangeColourOfChildren` (`self.YellowSeq2`) "/Game/Materials/BLUE_Depthless.BLUE_Depthless")
    (`self.ChangeColourOfChildren` (`self.YellowSeq3`) "/Game/Materials/BLUE_Depthless.BLUE_Depthless")
    (else
      (`self.ChangeColourOfChildren` (`self.YellowSeq2`) "/Game/Materials/YELLOW_Depthless.YELLOW_Depthless")
      (`self.ChangeColourOfChildren` (`self.YellowSeq3`) "/Game/Materials/YELLOW_Depthless.YELLOW_Depthless")))
  (`self.CheckFinalResult` :!label _label))

(event `self.Activatable2.OnClicked`
  (params (TouchedComponent :type "PrimitiveComponent Object Reference") (ButtonPressed :type "Key Structure"))
  (bind _bactivatable2clicked_ (`self.bActivatable2Clicked?`))
  (set `self.bActivatable2Clicked?` (not _bactivatable2clicked_))
  (if _bactivatable2clicked_
    (`self.ChangeColourOfChildren` (`self.YellowSeq3`) "/Game/Materials/RED_Depthless.RED_Depthless")
    (goto _label)
    (else
      (`self.ChangeColourOfChildren` (`self.YellowSeq3`) "/Game/Materials/YELLOW_Depthless.YELLOW_Depthless")
      (goto _label))))

(event `self.Activatable3.OnClicked`
  (params (TouchedComponent :type "PrimitiveComponent Object Reference") (ButtonPressed :type "Key Structure"))
  (bind _bactivatable3clicked_ (`self.bActivatable3Clicked?`))
  (set `self.bActivatable3Clicked?` (not _bactivatable3clicked_))
  (if _bactivatable3clicked_
    (`self.ChangeColourOfChildren` (`self.BlueSeq3`) "/Game/Materials/RED_Depthless.RED_Depthless")
    (goto _label)
    (else
      (`self.ChangeColourOfChildren` (`self.BlueSeq3`) "/Game/Materials/BLUE_Depthless.BLUE_Depthless")
      (goto _label))))

(fn `ChangeColourOfChildren`
  (params (ParentObject :type "StaticMeshComponent Object Reference") (NewMaterial :type "Material Object Reference"))
  (for _array_element (`SceneComponent.GetChildrenComponents` ParentObject false)
    (bind _asprimitive_component (cast `PrimitiveComponent` _array_element)
      (:`then`
        _)
      (:`CastFailed`
        _))
    (`PrimitiveComponent.SetMaterial` _asprimitive_component 0 NewMaterial))
  (return))

(fn `CheckFinalResult`
  (bind _returnvalue (`KismetSystemLibrary.GetObjectName` (`PrimitiveComponent.GetMaterial` (`self.Cylinder`) 0)))
  (if (`KismetStringLibrary.EqualEqual_StrStr` (`KismetSystemLibrary.GetObjectName` (`PrimitiveComponent.GetMaterial` (`self.StaticMesh32`) 0)) _returnvalue)
    (if (`KismetStringLibrary.EqualEqual_StrStr` (`KismetSystemLibrary.GetObjectName` (`PrimitiveComponent.GetMaterial` (`self.StaticMesh27`) 0)) _returnvalue)
      _)))

(fn `UserConstructionScript`)
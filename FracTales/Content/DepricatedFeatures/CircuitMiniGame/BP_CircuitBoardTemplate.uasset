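; Template actor for the deprecated circuit board minigame that presents the board in front of the player.
; BeginPlay shows the mouse cursor, stores a start point below the spawn location and sets the board's rotation from the player character's rotation.
; For its first second, Tick lerps the board from that start point to a spot ahead of the camera, re-reading the camera each frame.
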(event `self.ReceiveBeginPlay`
  ;[1 1 1] Setting rotation to face player
  (set `PlayerController.bShowMouseCursor` true (`GameplayStatics.GetPlayerController` 0))
  (set `self.StartingPosition` (`KismetMathLibrary.MakeVector` (.x (`self.K2_GetActorLocation`)) (.y (`self.K2_GetActorLocation`)) (- (.z (`self.K2_GetActorLocation`)) 200.0)))
  (`self.K2_SetActorRotation` (`KismetMathLibrary.MakeRotator` (.roll (`self.K2_GetActorRotation` (`GameplayStatics.GetPlayerCharacter` 0))) (.pitch (`self.K2_GetActorRotation` (`GameplayStatics.GetPlayerCharacter` 0))) (+ (.yaw (`self.K2_GetActorRotation` (`GameplayStatics.GetPlayerCharacter` 0))) 90.0))))

(event `self.ReceiveTick`
  (params (DeltaSeconds :type "Float (single-precision)"))
  (bind _returnvalue (`GameplayStatics.GetPlayerCameraManager` 0))
  (bind _lerpdeltatime (`self.LerpDeltaTime`))
  ;[1 1 1] Lerping to in front of player
  (set `self.LerpDeltaTime` (+ DeltaSeconds (`self.LerpDeltaTime`)))
  (if (< _lerpdeltatime 1.0)
    (`self.K2_SetActorLocation` (`KismetMathLibrary.VLerp` (`self.StartingPosition`) (+ (`self.K2_GetActorLocation` _returnvalue) (* (`self.GetActorForwardVector` _returnvalue) 250.0)) _lerpdeltatime))))

(fn `UserConstructionScript`)
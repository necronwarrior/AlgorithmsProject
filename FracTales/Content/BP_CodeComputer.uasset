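; BP_CodeComputer is a puzzle computer that displays a code-change puzzle and notifies other objects when it is solved.
; On BeginPlay it creates the configured CodeChangeWidget class for the first player controller and places it in its Widget component.
; Until completion, Tick polls that widget as BP_CodeChange_Base for IsPuzzleComplete.
; Once solved, it latches IsRelatedPuzzleComplete and calls PuzzleSolvedMessage on each InfluencedObjects entry.
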(event `self.ReceiveBeginPlay`
  (bind _returnvalue (`|CreateWidget` (`self.CodeChangeWidget`) (`GameplayStatics.GetPlayerController` 0)))
  (`WidgetComponent.SetWidget` (`self.Widget`) _returnvalue))

(event `self.ReceiveTick`
  (params (DeltaSeconds :type "Float (single-precision)"))
  (if (not (`self.bIsRelatedPuzzleComplete?`))
    (bind _asbp_code_change_base (cast `/Game/HUD/CodeChangeElements/BP_CodeChange_Base` (`WidgetComponent.GetUserWidgetObject` (`self.Widget`))))
    (if (`/Game/HUD/CodeChangeElements/BP_CodeChange_Base.bIsPuzzleComplete?` _asbp_code_change_base)
      (set `self.bIsRelatedPuzzleComplete?` true)
      (for _array_element (`self.InfluencedObjects`)
        (message `/Game/Mechanics/CodeInjection/BPI_CodeInjectionInterface.PuzzleSolved` _array_element)))))

(fn `UserConstructionScript`)
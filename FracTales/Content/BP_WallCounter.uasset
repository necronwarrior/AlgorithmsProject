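; BP_WallCounter is a clickable wall-mounted day counter that advances its widget to the next day and completes a task.
; It extends a parent interactable and drives a BP_FONTTEST widget, switched to first-person mode shortly after BeginPlay.
; Clicking blends the view to a tagged calendar camera with UI-only input, then returns to the player after a delay.
; Each tick, its text render turns to face the first-person camera.
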(event `self.ReceiveBeginPlay`
  (`parent.ReceiveBeginPlay`)
  (`KismetSystemLibrary.Delay` 5.0)
  (bind _asbp_fonttest (cast `/Game/BP_FONTTEST` (`WidgetComponent.GetUserWidgetObject` (`self.Widget`))))
  (`/Game/BP_FONTTEST.SetFirstPerson` _asbp_fonttest))

(event `self.PlayerClick`
  (params (PlayerCharacter :type "/Game/Character/FirstPersonCharacter Object Reference") (TagFunctionality :type Name))
  (bind _returnvalue (`GameplayStatics.GetPlayerController` 0))
  (bind _returnvalue_2 (`GameplayStatics.GetPlayerController` 0))
  (`parent.PlayerClick` PlayerCharacter TagFunctionality)
  (`/Game/BP_FONTTEST.NextDayCalled` (stale `self.ReceiveBeginPlay` _asbp_fonttest))
  (`self.TaskFinished`)
  (bind _unique_actor (`/Game/MacroLibrary/BML_ActorUtilities.GetActorWithUniqueTag` "calendarcamera"))
  (`PlayerController.SetViewTargetWithBlend` _returnvalue_2 _unique_actor 2.0 "VTBlend_Linear" 0.0 true)
  (`WidgetBlueprintLibrary.SetInputMode_UIOnlyEx` _returnvalue_2 (`WidgetComponent.GetUserWidgetObject` (`self.Widget`)))
  (set `PlayerController.bShowMouseCursor` true _returnvalue_2)
  (`KismetSystemLibrary.Delay` 5.0)
  (`PlayerController.SetViewTargetWithBlend` _returnvalue (`GameplayStatics.GetPlayerCharacter` 0) 2.0 "VTBlend_Linear" 0.0 true)
  (`WidgetBlueprintLibrary.SetInputMode_GameOnly` _returnvalue))

(event `self.ReceiveTick`
  (params (DeltaSeconds :type "Float (single-precision)"))
  (bind _textrender (`self.TextRender`))
  (bind _asfirst_person_character (cast `/Game/Character/FirstPersonCharacter` (`GameplayStatics.GetPlayerCharacter` 0)))
  (`SceneComponent.K2_SetWorldRotation` _textrender (`KismetMathLibrary.FindLookAtRotation` (`SceneComponent.K2_GetComponentLocation` _textrender) (`SceneComponent.K2_GetComponentLocation` (`/Game/Character/FirstPersonCharacter.FirstPersonCamera` _asfirst_person_character))) false false))

(fn `UserConstructionScript`)
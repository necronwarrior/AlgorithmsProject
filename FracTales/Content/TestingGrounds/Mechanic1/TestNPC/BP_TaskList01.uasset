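; BP_TaskList01 is a test NPC task list that saves a chosen material and applies it to a task list test object.
; Three Option0 choice events each pick a material and write it to a newly created CurrentSaveGame, saved under that object's default slot and user index.
; ExecuteTaskList loads that slot and sets the saved ObjectTestOption0 material on the Cube of the parent BP_TESTTaskListOBJECT.
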(event `self.ExecuteTaskList`
  (params (`Parent Reference` :type "Actor Object Reference"))
  (bind _returnvalue (`GameplayStatics.CreateSaveGameObject` "/Game/TestingGrounds/CurrentSaveGame.CurrentSaveGame_C"))
  (bind _returnvalue_2 (`GameplayStatics.LoadGameFromSlot` (`/Game/TestingGrounds/CurrentSaveGame.SaveSlotName` _returnvalue) (`/Game/TestingGrounds/CurrentSaveGame.UserIndex` _returnvalue)))
  (bind _ascurrent_save_game (cast `/Game/TestingGrounds/CurrentSaveGame` _returnvalue_2))
  (bind _asbp_testtask_list_object (cast `/Game/TestingGrounds/Mechanic2/Test/BP_TESTTaskListOBJECT` `Parent Reference`))
  (`PrimitiveComponent.SetMaterial` (`/Game/TestingGrounds/Mechanic2/Test/BP_TESTTaskListOBJECT.Cube` _asbp_testtask_list_object) 0 (`/Game/TestingGrounds/CurrentSaveGame.ObjectTestOption0` _ascurrent_save_game)))

(event `self.Option0Choice0`
  (params (Parent :type "Actor Object Reference"))
  (set `self.MaterialTest` "/Game/TestingGrounds/FPTestingZone/Tester/creature_guldan_guldan_m2_Geoset_003_Dbl.creature_guldan_guldan_m2_Geoset_003_Dbl")
  (bind _returnvalue (`GameplayStatics.CreateSaveGameObject` "/Game/TestingGrounds/CurrentSaveGame.CurrentSaveGame_C" :!label _label))
  (set `/Game/TestingGrounds/CurrentSaveGame.ObjectTestOption0` (`self.MaterialTest`) _returnvalue)
  (`GameplayStatics.SaveGameToSlot` _returnvalue (`/Game/TestingGrounds/CurrentSaveGame.SaveSlotName` _returnvalue) (`/Game/TestingGrounds/CurrentSaveGame.UserIndex` _returnvalue)))

(event `self.Option0Choice1`
  (params (Parent :type "Actor Object Reference"))
  (set `self.MaterialTest` "/Game/TestingGrounds/FPTestingZone/Tester/creature_guldan_guldan_m2_Geoset_001.creature_guldan_guldan_m2_Geoset_001")
  (goto _label))

(event `self.Option0Choice2`
  (params (Parent :type "Actor Object Reference"))
  (set `self.MaterialTest` "/Game/TestingGrounds/LeveLoading/LoadingScreenMat.LoadingScreenMat")
  (goto _label))
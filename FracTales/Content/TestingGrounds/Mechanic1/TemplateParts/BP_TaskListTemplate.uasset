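; Template Blueprint for a task list that runs tasks when played and handles a three-way option choice from a widget.
; ExecuteTaskList passes a parent reference to Option0Task, which is an empty stub.
; The Option0 event switches on a choice index to one of three per-choice functions, each printing a placeholder string.
; Any other index prints the parent's object name.
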(event `ExecuteTaskList`
  (params (`Parent Reference` :type "Actor Object Reference"))
  ;[1 1 1] Execute tasks when played
  (`self.Option0Task` `Parent Reference`))

(event `Option0`
  (params (O1C :type Integer) (ParentReference :type "Actor Object Reference"))
  ;[1 1 1] Simple framework for accepting one of 3 options through the widget
  (switch `int` O1C
    (:`Default`
      (`KismetSystemLibrary.PrintString` null (`KismetSystemLibrary.GetObjectName` ParentReference)))
    (:`0`
      (`self.Option0Choice0` ParentReference))
    (:`1`
      (`self.Option0Choice1` ParentReference))
    (:`2`
      (`self.Option0Choice2` ParentReference))))

(fn `Option0Choice0`
  (params (Parent :type "Actor Object Reference"))
  (`KismetSystemLibrary.PrintString` null "choice0"))

(fn `Option0Choice1`
  (params (Parent :type "Actor Object Reference"))
  (`KismetSystemLibrary.PrintString` null "choice1"))

(fn `Option0Choice2`
  (params (Parent :type "Actor Object Reference"))
  (`KismetSystemLibrary.PrintString` null "choice2"))

(fn `Option0Task`
  (params (`Parent Reference` :type "Actor Object Reference"))
  (return))
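; Template actor for a clickable task on the player's task list, linked to a nearby rail junction.
; On BeginPlay, IsActive sets its TextRender visibility and collision, then a sphere overlap grows until it finds a BP_RailJunction, cached if it is the only hit.
; PlayerClick stores the player, whose checklist TaskFinished updates at PositionInTaskList.
; ToggleTextVisibility toggles text components tagged with the given task name.
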(event `self.ReceiveBeginPlay`
  (bind _bisactive_ (`self.bIsActive?`))
  (for _array_element (`SceneComponent.GetChildrenComponents` (`self.DefaultSceneRoot`) false)
    (if (`KismetStringLibrary.EqualEqual_StrStr` (`KismetSystemLibrary.GetObjectName` _array_element) "TextRender")
      (`SceneComponent.SetVisibility` _array_element _bisactive_ true)
      (`self.SetActorEnableCollision` _bisactive_)
      (bind (_outactors _returnvalue) (`KismetSystemLibrary.SphereOverlapActors` (`self.K2_GetActorLocation` self) (`self.SphereSize`) (`|MakeArray` "ObjectTypeQuery2" :!type "EObjectTypeQuery Enum") "/Game/TestingGrounds/GridDirectionLines/BP_RailJunction.BP_RailJunction_C" :!label _label))
      (if _returnvalue
        (if (== (`KismetArrayLibrary.Array_Length` _outactors) 1)
          (bind _asbp_rail_junction (cast `/Game/TestingGrounds/GridDirectionLines/BP_RailJunction` (`|GetArrayItem` _outactors)))
          (set `self.ClosestRailJunction` _asbp_rail_junction))
        (else
          (`/Engine/EditorBlueprintResources/StandardMacros.IncrementFloat` (`self.SphereSize`)
            (:`  `
              (goto _label))))))))

(event `PlayerClick`
  (params (PlayerCharacter :type "/Game/TestingGrounds/FPTestingZone/Blueprints/FirstPersonCharacter Object Reference") (TagFunctionality :type Name))
  ;[1 1 1] Check that this task is the next task to perform - at least compared to the last task
  (set `self.PlayerCharacterReference` PlayerCharacter))

(event `TaskFinished`
  ;[1 1 1] When task is completed set its corresponding value in the player's checklist to true and change colour
  (`/Game/TestingGrounds/FPTestingZone/Blueprints/FirstPersonCharacter.SetTaskListComlpeteIndex` (`self.PlayerCharacterReference`) (`self.PositionInTaskList`)))

(event `ToggleTextVisibility`
  (params (TaskName :type Name))
  (for _array_element (`self.K2_GetComponentsByClass` self "/Script/Engine.TextRenderComponent")
    (if (`KismetArrayLibrary.Array_Contains` (`ActorComponent.ComponentTags` _array_element) TaskName)
      (`SceneComponent.ToggleVisibility` _array_element false))))

(fn `UserConstructionScript`)
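; BP_TaskListObjectTemplate is a template actor for one step in an ordered player task list.
; On BeginPlay, IsActive sets its visibility and collision.
; PlayerClick uses neighbouring entries in the player's completion array to flag whether it is the next task, and stores the player reference.
; TaskFinished disables its collision, toggles visibility on itself and the next object, enables that object's collision, and updates the player's checklist.
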(event `self.ReceiveBeginPlay`
  (bind _bisactive_ (`self.bIsActive?`))
  (`SceneComponent.SetVisibility` (`self.DefaultSceneRoot`) _bisactive_ true)
  (`self.SetActorEnableCollision` _bisactive_))

(event `PlayerClick`
  (params (TaskListComplete :type "Array of Boolean") (PlayerCharacter :type "/Game/TestingGrounds/FPTestingZone/Blueprints/FirstPersonCharacter Object Reference"))
  (bind _positionintasklist (`self.PositionInTaskList`))
  ;[1 1 1] Check that this task is the next task to perform - at least compared to the last task
  (`/Engine/EditorBlueprintResources/StandardMacros.CompareInt` _positionintasklist
    (:`>`
      (set `self.bIsNextTaskInLIst?` (`|GetArrayItem` TaskListComplete (- _positionintasklist 1))))
    (:`==`
      (set `self.bIsNextTaskInLIst?` (not (`|GetArrayItem` TaskListComplete (+ _positionintasklist 1))))))
  (set `self.PlayerCharacterReference` PlayerCharacter))

(event `TaskFinished`
  (bind _nextobjectintasklist (`self.NextObjectInTaskList`))
  ;[1 1 1] When task is completed set its corresponding value in the player's checklist to true and change colour
  (`self.SetActorEnableCollision` self false)
  (`SceneComponent.ToggleVisibility` (`self.DefaultSceneRoot`) true)
  (`self.SetActorEnableCollision` _nextobjectintasklist true)
  (`SceneComponent.ToggleVisibility` (`/Game/TestingGrounds/TaskListObjects/BP_TaskListObjectTemplate.DefaultSceneRoot` _nextobjectintasklist) true)
  (`/Game/TestingGrounds/FPTestingZone/Blueprints/FirstPersonCharacter.SetTaskListComlpeteIndex` (`self.PlayerCharacterReference`) (`self.PositionInTaskList`)))

(fn `UserConstructionScript`)
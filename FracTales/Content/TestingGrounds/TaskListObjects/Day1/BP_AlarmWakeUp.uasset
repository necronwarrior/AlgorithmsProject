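; Day 1 alarm clock task object that handles waking the player up and putting them to sleep.
; PlayerClick branches on the functionality tag, finishing the task and replaying the WakeUpSequence in both cases.
; Waking changes control structure, moves the player to WakeupPoint after a delay, clears the lying-down flag and briefly shows a one-time movement widget.
; Setting the alarm moves the player to SleepPoint, changes the task list and sets lying-down.
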(event `self.ReceiveBeginPlay`
  (`parent.ReceiveBeginPlay`))

(event `self.PlayerClick`
  (params (PlayerCharacter :type "/Game/TestingGrounds/FPTestingZone/Blueprints/FirstPersonCharacter Object Reference") (TagFunctionality :type Name))
  (bind _returnvalue (`GameplayStatics.GetPlayerCharacter` 0))
  (bind _sequenceplayer (`LevelSequenceActor.SequencePlayer` (`self.WakeUpSequence`)))
  (bind _sequenceplayer_2 (`LevelSequenceActor.SequencePlayer` (`self.WakeUpSequence`)))
  ;[1 1 1] Check If this is next task, space for any other checks
  (`parent.PlayerClick` PlayerCharacter TagFunctionality)
  (switch `name` TagFunctionality
    (:`WakeUpAlarmClock`
      ;[1 1 1] Conditions for finishing task
      (`self.K2_SetActorRotation` :`self` PlayerCharacter)
      (`/Game/TestingGrounds/FPTestingZone/Blueprints/FirstPersonCharacter.SetControlStructure` PlayerCharacter "NewEnumerator3")
      (`self.TaskFinished`)
      (`MovieSceneSequencePlayer.SetPlaybackPosition` _sequenceplayer_2 0.0)
      (`MovieSceneSequencePlayer.Play` _sequenceplayer_2)
      (`KismetSystemLibrary.Delay` 5.0)
      (`self.K2_SetActorLocation` _returnvalue (.location (`self.GetTransform` (`self.WakeupPoint`))) false false)
      (`Controller.SetControlRotation` (`GameplayStatics.GetPlayerController` 0) (.rotation (`self.GetTransform` (`self.WakeupPoint`))))
      (bind _asfirst_person_character (cast `/Game/TestingGrounds/FPTestingZone/Blueprints/FirstPersonCharacter` _returnvalue))
      (set `/Game/TestingGrounds/FPTestingZone/Blueprints/FirstPersonCharacter.bISTEMPLyingDown` false _asfirst_person_character)
      (`/Engine/EditorBlueprintResources/StandardMacros.DoOnce` false
        (:`Completed`
          (bind _returnvalue_2 (`|CreateWidget` "/Game/TestingGrounds/TutorialTemp/BP_MovementWidget.BP_MovementWidget_C"))
          (`UserWidget.AddToViewport` _returnvalue_2 0)
          (`KismetSystemLibrary.Delay` 5.0)
          (`Widget.RemoveFromParent` _returnvalue_2))))
    (:`SetSleepAlarm`
      (`self.K2_TeleportTo` :`self` PlayerCharacter :`DestLocation` (`self.K2_GetActorLocation` (`self.SleepPoint`)))
      (`self.TaskFinished`)
      (`/Game/TestingGrounds/FPTestingZone/Blueprints/FirstPersonCharacter.Waking up` PlayerCharacter)
      (`/Game/TestingGrounds/FPTestingZone/Blueprints/FirstPersonCharacter.Change Task List` PlayerCharacter)
      (`MovieSceneSequencePlayer.SetPlaybackPosition` _sequenceplayer 0.0)
      (`MovieSceneSequencePlayer.Play` _sequenceplayer)
      (`self.K2_SetActorLocation` PlayerCharacter (.location (`self.GetTransform` (`self.SleepPoint`))) false false)
      (`Controller.SetControlRotation` (`GameplayStatics.GetPlayerController` 0) (.rotation (`self.GetTransform` (`self.SleepPoint`))))
      (set `/Game/TestingGrounds/FPTestingZone/Blueprints/FirstPersonCharacter.bISTEMPLyingDown` true PlayerCharacter))))

(fn `UserConstructionScript`
  (`parent.UserConstructionScript`))
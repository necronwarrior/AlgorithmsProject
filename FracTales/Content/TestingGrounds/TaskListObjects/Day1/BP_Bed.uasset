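; BP_Bed is the bed task object for Day 1 that puts the player to bed and plays a wake-up.
; On a player click it restarts the WakeUpSequence level sequence and calls WakingUp on the character.
; It teleports the character and player controller to the SleepPoint, copies that rotation to the controller, finishes the task and sets a temporary lying-down flag.
; It adds no checks of its own before completing.
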(event `self.ReceiveBeginPlay`
  (`parent.ReceiveBeginPlay`))

(event `self.PlayerClick`
  (params (PlayerCharacter :type "/Game/TestingGrounds/FPTestingZone/Blueprints/FirstPersonCharacter Object Reference") (TagFunctionality :type Name))
  (bind _returnvalue (`GameplayStatics.GetPlayerController` 0))
  (bind _sequenceplayer (`LevelSequenceActor.SequencePlayer` (`self.WakeUpSequence`)))
  (bind _location (.location (`self.GetTransform` (`self.SleepPoint`))))
  ;[1 1 1] Check If this is next task, space for any other checks
  (`parent.PlayerClick` PlayerCharacter "None")
  ;[1 1 1] Conditions for finishing task
  (`MovieSceneSequencePlayer.SetPlaybackPosition` _sequenceplayer 0.0)
  (`MovieSceneSequencePlayer.Play` _sequenceplayer)
  (`/Game/TestingGrounds/FPTestingZone/Blueprints/FirstPersonCharacter.Waking up` PlayerCharacter)
  (`self.K2_SetActorLocation` _returnvalue _location false true)
  (`self.K2_SetActorLocation` PlayerCharacter _location false true)
  (`self.K2_SetActorRotation` _returnvalue (.rotation (`self.GetTransform` (`self.SleepPoint`))) false)
  (`self.TaskFinished`)
  (set `/Game/TestingGrounds/FPTestingZone/Blueprints/FirstPersonCharacter.bISTEMPLyingDown` true PlayerCharacter))

(fn `UserConstructionScript`
  (`parent.UserConstructionScript`))
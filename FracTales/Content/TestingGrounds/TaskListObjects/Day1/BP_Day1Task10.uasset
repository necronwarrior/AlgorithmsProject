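; BP_Day1Task10 is the interactable object for task 10 of Day 1 in the task list, presenting a multiple-choice widget.
; When clicked as the next task in the list, it disables player input, shows and centers the cursor, and opens BP_TaskListWidgetMCQ.
; It passes itself to the widget, and its ExitWidget event marks the task finished.
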(event `self.PlayerClick`
  (params (PlayerCharacter :type "/Game/TestingGrounds/FPTestingZone/Blueprints/FirstPersonCharacter Object Reference") (TagFunctionality :type Name))
  (bind _returnvalue (`GameplayStatics.GetPlayerController` 0))
  (bind (_x _y) (`KismetMathLibrary.BreakVector2D` (`WidgetLayoutLibrary.GetViewportSize`)))
  ;[1 1 1] Check If this is next task, space for any other checks
  (`parent.PlayerClick` PlayerCharacter "None")
  (if (`self.bIsNextTaskInLIst?`)
    ;[1 1 1] Conditions for finishing task
    (`self.DisableInput` (`GameplayStatics.GetPlayerCharacter` 0) _returnvalue)
    (set `PlayerController.bShowMouseCursor` true _returnvalue)
    (`PlayerController.SetMouseLocation` _returnvalue (`KismetMathLibrary.FTrunc` (/ _x 2.0)) (`KismetMathLibrary.FTrunc` (/ _y 2.0)))
    (bind _returnvalue_2 (`|CreateWidget` "/Game/TestingGrounds/TaskListObjects/Day1/Day1Task10Extras/BP_TaskListWidgetMCQ.BP_TaskListWidgetMCQ_C" _returnvalue))
    (bind _output_get (set `self.TaskListMCQNPC` _returnvalue_2))
    (set `/Game/TestingGrounds/TaskListObjects/Day1/Day1Task10Extras/BP_TaskListWidgetMCQ.Day1Task10Object` self _output_get)
    (`UserWidget.AddToViewport` _returnvalue_2 0)))

(event `Exit Widget`
  (`self.TaskFinished`))

(fn `UserConstructionScript`
  (`parent.UserConstructionScript`))
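; BP_Day1Task8 is a clickable task object for the eighth task of Day 1, built on a parent task-list object class.
; When clicked as the next task in the list, it shows a progress bar widget and enables its Tick, which fills the bar over a two-second delay.
; It then removes the widget, disables Tick again and calls TaskFinished.
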(event `self.ReceiveBeginPlay`
  (`parent.ReceiveBeginPlay`)
  (`self.SetActorTickEnabled` false))

(event `self.PlayerClick`
  (params (TaskListComplete :type "Array of Boolean (by ref)") (PlayerCharacter :type "/Game/TestingGrounds/FPTestingZone/Blueprints/FirstPersonCharacter Object Reference"))
  ;[1 1 1] Check If this is next task, space for any other checks
  (`parent.PlayerClick` TaskListComplete PlayerCharacter)
  (if (`self.bIsNextTaskInLIst?`)
    ;[1 1 1] Conditions for finishing task
    (bind _returnvalue (`|CreateWidget` "/Game/TestingGrounds/TaskListObjects/BP_ProgressBar.BP_ProgressBar_C"))
    (bind _output_get (set `self.Progressbar` _returnvalue))
    (`UserWidget.AddToViewport` _output_get 0)
    (`self.SetActorTickEnabled` true)
    (`KismetSystemLibrary.Delay` 2.0)
    (`Widget.RemoveFromParent` (`self.Progressbar`))
    (`self.SetActorTickEnabled` false)
    (`self.TaskFinished`)))

(event `self.ReceiveTick`
  (params (DeltaSeconds :type "Float (single-precision)"))
  (bind _progressbar (`self.Progressbar`))
  (bind _output_get (set `/Game/TestingGrounds/TaskListObjects/BP_ProgressBar.CompondDeltatime` (+ (/ DeltaSeconds 2.0) (`/Game/TestingGrounds/TaskListObjects/BP_ProgressBar.CompondDeltatime` _progressbar)) _progressbar))
  (`ProgressBar.SetPercent` (`/Game/TestingGrounds/TaskListObjects/BP_ProgressBar.TaskCompletionProgressBar` _progressbar) _output_get))

(fn `UserConstructionScript`
  (`parent.UserConstructionScript`))
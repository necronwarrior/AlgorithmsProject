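; BP_Day1Task1 is the first Day 1 task object, a clickable task that plays a wake-up sequence when completed.
; On player click it runs the parent logic and, if it is the next task in the list, resets player rotation, updates the control structure and finishes the task.
; It then restarts the WakeUpSequence and moves the player to a hard-coded position and view direction.
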(event `self.ReceiveBeginPlay`
  (`parent.ReceiveBeginPlay`))

(event `self.PlayerClick`
  (params (TaskListComplete :type "Array of Boolean (by ref)") (PlayerCharacter :type "/Game/TestingGrounds/FPTestingZone/Blueprints/FirstPersonCharacter Object Reference"))
  (bind _sequenceplayer (`LevelSequenceActor.SequencePlayer` (`self.WakeUpSequence`)))
  ;[1 1 1] Check If this is next task, space for any other checks
  (`parent.PlayerClick` TaskListComplete PlayerCharacter)
  (if (`self.bIsNextTaskInLIst?`)
    ;[1 1 1] Conditions for finishing task
    (`self.K2_SetActorRotation` :`self` PlayerCharacter)
    (setmembers `/Game/TestingGrounds/FPTestingZone/Blueprints/ControlsStructure` :`StructRef` (`/Game/TestingGrounds/FPTestingZone/Blueprints/FirstPersonCharacter.ControlStructure` PlayerCharacter) :`bIsLeftMouseButtonActive` true :`bIsInputAxisMoveForwardActive` true :`bIsInputAxisMoveRightActive` true :`bIsInputAxisTurnRateActive` true :`bIsInputAxisLookUpRateActive` true :`bIsInputActionJumpActive` true :`bIsXKeyActive` true :`bIsQKeyActive` true :`bIsInputActionFireActive` true :`bIsEKeyActive` true :`bIsInteractRadiusBeginOverlapActive` true :`bIsInteractRadiusEndOverlapActive` true :`bIs1KeyActive` true :`bIs2KeyActive` true :`bIs3KeyActive` true :`bIs4KeyActive` true :`bIs5KeyActive` true :`bIs6KeyActive` true :`bIs7KeyActive` true :`bIsUpActive` true :`bIsDownActive` true)
    (`self.TaskFinished`)
    (`MovieSceneSequencePlayer.SetPlaybackPosition` _sequenceplayer 0.0)
    (`MovieSceneSequencePlayer.Play` _sequenceplayer)
    (`self.K2_SetActorLocation` (`GameplayStatics.GetPlayerCharacter` 0) (12642.746094 -16133.611328 1549.907349) false false)
    (`Controller.SetControlRotation` (`GameplayStatics.GetPlayerController` 0) (`KismetMathLibrary.MakeRotator` 0.0 0.0 250.0))))

(fn `UserConstructionScript`
  (`parent.UserConstructionScript`))
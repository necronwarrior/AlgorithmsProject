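; BP_ExerciseBike is a clickable Day 1 task object where the player pedals by alternately pressing A and D.
; Clicking it creates the exercise controls widget, switches the player's control structure and enables Tick.
; Tick polls the expected key, counts each alternation and swaps the widget's key highlight.
; At the pedal target it changes the control structure, removes the widget, disables Tick, resets the count and finishes the task.
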(event `self.ReceiveBeginPlay`
  (`parent.ReceiveBeginPlay`)
  (`self.SetActorTickEnabled` false))

(event `self.PlayerClick`
  (params (PlayerCharacter :type "/Game/TestingGrounds/FPTestingZone/Blueprints/FirstPersonCharacter Object Reference") (TagFunctionality :type Name))
  (bind _exercisecontrolwidget (`self.ExerciseControlWidget`))
  ;[1 1 1] Check If this is next task, space for any other checks
  (`parent.PlayerClick` PlayerCharacter "None")
  ;[1 1 1] Conditions for finishing task
  (bind _returnvalue (`|CreateWidget` "/Game/TestingGrounds/TaskListObjects/Day1/Day1Task5Extras/BP_ExerciseControls.BP_ExerciseControls_C"))
  (bind _output_get (set `self.ExerciseControlWidget` _returnvalue))
  (`UserWidget.AddToViewport` _output_get 0)
  (`/Game/TestingGrounds/FPTestingZone/Blueprints/FirstPersonCharacter.SetControlStructure` PlayerCharacter "NewEnumerator1")
  (`self.SetActorTickEnabled` true)
  (`Border.SetBrushColor` (`/Game/TestingGrounds/TaskListObjects/Day1/Day1Task5Extras/BP_ExerciseControls.A_Border` _exercisecontrolwidget) (struct :`R` 1.0 :`G` 1.0 :`B` 1.0 :`A` 1.0))
  (`Border.SetBrushColor` (`/Game/TestingGrounds/TaskListObjects/Day1/Day1Task5Extras/BP_ExerciseControls.D_Border` _exercisecontrolwidget) (struct :`R` 1.0 :`G` 0.9 :`A` 1.0)))

(event `self.ReceiveTick`
  (params (DeltaSeconds :type "Float (single-precision)"))
  (bind _exercisecontrolwidget (`self.ExerciseControlWidget`))
  (bind _a_border (`/Game/TestingGrounds/TaskListObjects/Day1/Day1Task5Extras/BP_ExerciseControls.A_Border` _exercisecontrolwidget))
  (bind _d_border (`/Game/TestingGrounds/TaskListObjects/Day1/Day1Task5Extras/BP_ExerciseControls.D_Border` _exercisecontrolwidget))
  (if (< (`self.PedalCount`) 20)
    (if (`self.bIsLeftKeyPedalling`)
      (if (`PlayerController.IsInputKeyDown` (`GameplayStatics.GetPlayerController` 0) "D")
        (set `self.bIsLeftKeyPedalling` false)
        (`/Engine/EditorBlueprintResources/StandardMacros.IncrementInt` (`self.PedalCount`)
          (:`  `
            (`Border.SetBrushColor` _d_border (struct :`R` 1.0 :`G` 1.0 :`B` 1.0 :`A` 1.0))
            (`Border.SetBrushColor` _a_border (struct :`R` 1.0 :`G` 0.9 :`A` 1.0)))))
      (elif (`PlayerController.IsInputKeyDown` (`GameplayStatics.GetPlayerController` 0) "A")
        (set `self.bIsLeftKeyPedalling` true)
        (`/Engine/EditorBlueprintResources/StandardMacros.IncrementInt` (`self.PedalCount`)
          (:`  `
            (`Border.SetBrushColor` _d_border (struct :`R` 1.0 :`G` 0.9 :`A` 1.0))
            (`Border.SetBrushColor` _a_border (struct :`R` 1.0 :`G` 1.0 :`B` 1.0 :`A` 1.0))))))
    (else
      (`/Game/TestingGrounds/FPTestingZone/Blueprints/FirstPersonCharacter.SetControlStructure` (stale `self.PlayerClick` PlayerCharacter) "NewEnumerator3")
      (`self.SetActorTickEnabled` false)
      (set `self.PedalCount` 0)
      (`Widget.RemoveFromParent` (`self.ExerciseControlWidget`))
      (`self.TaskFinished`))))

(fn `UserConstructionScript`
  (`parent.UserConstructionScript`))
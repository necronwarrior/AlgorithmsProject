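; BP_Day1Task11 is a clickable Day 1 task object that, when it is next in the task list, moves the player into a wake-up transition.
; On click it runs the parent logic, teleports the player to a level spawn actor, finishes the task and tells the character to wake up and change task list.
; It then restarts the wake-up sequence and overrides the player's position and control rotation with hard-coded values.
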(event `self.PlayerClick`
  (params (TaskListComplete :type "Array of Boolean (by ref)") (PlayerCharacter :type "/Game/TestingGrounds/FPTestingZone/Blueprints/FirstPersonCharacter Object Reference"))
  (bind _sequenceplayer (`LevelSequenceActor.SequencePlayer` (`self.WakeUpSequence`)))
  ;[1 1 1] Check If this is next task, space for any other checks
  (`parent.PlayerClick` TaskListComplete PlayerCharacter)
  (if (`self.bIsNextTaskInLIst?`)
    ;[1 1 1] Conditions for finishing task
    (`self.K2_TeleportTo` :`self` PlayerCharacter :`DestLocation` (`self.K2_GetActorLocation` (`self.LevelSpawnActorReference`)))
    (`self.TaskFinished`)
    (`/Game/TestingGrounds/FPTestingZone/Blueprints/FirstPersonCharacter.Waking up` PlayerCharacter)
    (`/Game/TestingGrounds/FPTestingZone/Blueprints/FirstPersonCharacter.Change Task List` PlayerCharacter)
    (`MovieSceneSequencePlayer.SetPlaybackPosition` _sequenceplayer 0.0)
    (`MovieSceneSequencePlayer.Play` _sequenceplayer)
    (`self.K2_SetActorLocation` PlayerCharacter (12622.637695 -15933.104492 1446.759155) false false)
    (`Controller.SetControlRotation` (`GameplayStatics.GetPlayerController` 0) (`KismetMathLibrary.MakeRotator` 0.0 0.0 250.0))))

(fn `UserConstructionScript`
  (`parent.UserConstructionScript`))
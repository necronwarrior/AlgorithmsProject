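; BP_Day1Task7 is the seventh Day 1 task object in the testing grounds task list, triggered by a player click.
; When it is next in the list, it resets the player's rotation, updates their control structure and plays the wake-up sequence from the start.
; It then teleports the player to a wakeup point, finishes the task and aligns the controller's rotation to that point.
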(event `self.ReceiveBeginPlay`
  (`parent.ReceiveBeginPlay`))

(event `self.PlayerClick`
  (params (TaskListComplete :type "Array of Boolean (by ref)") (PlayerCharacter :type "/Game/TestingGrounds/FPTestingZone/Blueprints/FirstPersonCharacter Object Reference"))
  (bind _sequenceplayer (`LevelSequenceActor.SequencePlayer` (`self.WakeUpSequence`)))
  ;[1 1 1] Check If this is next task, space for any other checks
  (`parent.PlayerClick` TaskListComplete PlayerCharacter)
  (if (`self.bIsNextTaskInLIst?`)
    ;[1 1 1] Conditions for finishing task
    (`self.K2_SetActorRotation` :`self` PlayerCharacter)
    (setmembers `/Game/TestingGrounds/FPTestingZone/Blueprints/ControlsStructure` :`StructRef` (`/Game/TestingGrounds/FPTestingZone/Blueprints/FirstPersonCharacter.ControlStructure` PlayerCharacter) :`bIsLeftMouseButtonActive` true :`bIsInputAxisMoveForwardActive` true :`bIsInputAxisMoveRightActive` true :`bIsInputAxisTurnRateActive` true :`bIsInputAxisLookUpRateActive` true :`bIsInputActionJumpActive` true :`bIsXKeyActive` true :`bIsQKeyActive` true :`bIsInputActionFireActive` true :`bIsEKeyActive` true :`bIsInteractRadiusBeginOverlapActive` true :`bIsInteractRadiusEndOverlapActive` true :`bIs1KeyActive` true :`bIs2KeyActive` true :`bIs3KeyActive` true :`bIs4KeyActive` true :`bIs5KeyActive` true :`bIs6KeyActive` true :`bIs7KeyActive` true :`bIsUpActive` true :`bIsDownActive` true)
    (`MovieSceneSequencePlayer.SetPlaybackPosition` _sequenceplayer 0.0)
    (`MovieSceneSequencePlayer.Play` _sequenceplayer)
    (`self.K2_SetActorLocation` PlayerCharacter (.location (`self.GetTransform` (`self.WakeupPoint`))) false false)
    (`self.TaskFinished`)
    (`Controller.SetControlRotation` (`GameplayStatics.GetPlayerController` 0) (.rotation (`self.GetTransform` (`self.WakeupPoint`))))))

(fn `UserConstructionScript`
  (`parent.UserConstructionScript`))
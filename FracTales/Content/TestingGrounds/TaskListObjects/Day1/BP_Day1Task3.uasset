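; BP_Day1Task3 is the third Day 1 task-list object, a plant-watering task driven by player clicks.
; When it is next in the list, a click saves the player's right-hand object, attaches the watering can to the Mesh2P GripPoint and registers itself with the first "PlantTag" actor.
; A click while IsFinishedWatering is set restores the held-object reference, detaches the can and finishes the task.
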(event `self.ReceiveBeginPlay`
  (`parent.ReceiveBeginPlay`))

(event `self.PlayerClick`
  (params (TaskListComplete :type "Array of Boolean (by ref)") (PlayerCharacter :type "/Game/TestingGrounds/FPTestingZone/Blueprints/FirstPersonCharacter Object Reference"))
  (bind _bp_wateringcan (`self.BP_WateringCan`))
  ;[1 1 1] Check If this is next task, space for any other checks
  (if (`self.bIsFinishedWatering`)
    (set `/Game/TestingGrounds/FPTestingZone/Blueprints/FirstPersonCharacter.RightHandObject` (`self.TempHandObject`) PlayerCharacter)
    (`SceneComponent.K2_DetachFromComponent` _bp_wateringcan "KeepRelative" "KeepRelative" "KeepRelative" true)
    (set `self.bIsFinishedWatering` false)
    (`self.TaskFinished`)
    (else
      (`parent.PlayerClick` TaskListComplete PlayerCharacter)
      (if (`self.bIsNextTaskInLIst?`)
        (set `self.TempHandObject` (`/Game/TestingGrounds/FPTestingZone/Blueprints/FirstPersonCharacter.RightHandObject` PlayerCharacter))
        ;[1 1 1] Conditions for finishing task
        (set `/Game/TestingGrounds/FPTestingZone/Blueprints/FirstPersonCharacter.RightHandObject` _bp_wateringcan PlayerCharacter)
        (`SceneComponent.K2_AttachToComponent` _bp_wateringcan (`/Game/TestingGrounds/FPTestingZone/Blueprints/FirstPersonCharacter.Mesh2P` PlayerCharacter) "GripPoint" "SnapToTarget" "SnapToTarget" "SnapToTarget" true)
        (bind _outactors (`GameplayStatics.GetAllActorsWithTag` "PlantTag"))
        (bind _asbp_plants (cast `/Game/TestingGrounds/TaskListObjects/Day1/Day1Task3Extras/BP_Plants` (`|GetArrayItem` _outactors)))
        (set `/Game/TestingGrounds/TaskListObjects/Day1/Day1Task3Extras/BP_Plants.TaskGivingObject` self _asbp_plants)))))

(fn `UserConstructionScript`
  (`parent.UserConstructionScript`))
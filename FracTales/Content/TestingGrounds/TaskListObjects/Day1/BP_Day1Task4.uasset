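; BP_Day1Task4 is the Day 1, task 4 object in a task list system, with BeginPlay and construction deferring to its parent.
; InPlayerView takes the completion array and player character, then sets whether this task is next in the list.
; Later positions require the previous task to be complete, while position zero requires the following one to be incomplete.
; Both branches also store the player character reference.
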(event `self.ReceiveBeginPlay`
  (`parent.ReceiveBeginPlay`))

(fn `InPlayerView`
  (params (TaskListComplete :type "Array of Boolean") (PlayerCharacter :type "/Game/TestingGrounds/FPTestingZone/Blueprints/FirstPersonCharacter Object Reference"))
  (bind _positionintasklist (`self.PositionInTaskList`))
  (`/Engine/EditorBlueprintResources/StandardMacros.CompareInt` _positionintasklist
    (:`>`
      (set `self.bIsNextTaskInLIst?` (`|GetArrayItem` TaskListComplete (- _positionintasklist 1))))
    (:`==`
      (set `self.bIsNextTaskInLIst?` (not (`|GetArrayItem` TaskListComplete (+ _positionintasklist 1))))))
  (set `self.PlayerCharacterReference` PlayerCharacter))

(fn `UserConstructionScript`
  (`parent.UserConstructionScript`))
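; BP_OpenableDoor is a hinged door that swings open away from whatever actor enters its Box trigger and closes on overlap end.
; The actor's position in the door's local space picks a swing of plus or minus 90 degrees yaw.
; SwingOpen and SwingClosed timelines stop each other and lerp from the Hinge's current rotation each update.
; Overlaps are not filtered by actor type or count.
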(event `self.Box.OnComponentBeginOverlap`
  (params (OverlappedComponent :type "PrimitiveComponent Object Reference") (OtherActor :type "Actor Object Reference") (OtherComp :type "PrimitiveComponent Object Reference") (OtherBodyIndex :type Integer) (bFromSweep :type Boolean) (SweepResult :type "HitResult Structure (by ref)"))
  (bind _hinge (`self.Hinge`))
  ;[1 1 1] Door Open away from player
  (`TimelineComponent.Stop` (`self.Swing Closed`))
  (set `self.OpenDirection` (> (.x (`KismetMathLibrary.LessLess_VectorRotator` (- (`self.K2_GetActorLocation`) (`self.K2_GetActorLocation` OtherActor)) (`self.K2_GetActorRotation`))) 0.0))
  (bind (_direction _rotation) (`Timeline|Swing Open` :!via `PlayFromStart`)
    (:`Update`
      (`SceneComponent.K2_SetRelativeRotation` _hinge (`KismetMathLibrary.RLerp` (.rotation (`SceneComponent.GetRelativeTransform` _hinge)) (`KismetMathLibrary.MakeRotator` 0.0 0.0 (`KismetMathLibrary.SelectFloat` -90.0 90.0 (`self.OpenDirection`))) _rotation true) false false))))

(event `self.Box.OnComponentEndOverlap`
  (params (OverlappedComponent :type "PrimitiveComponent Object Reference") (OtherActor :type "Actor Object Reference") (OtherComp :type "PrimitiveComponent Object Reference") (OtherBodyIndex :type Integer))
  (bind _hinge (`self.Hinge`))
  ;[1 1 1] Door close when player away
  (`TimelineComponent.Stop` (`self.Swing Open`))
  (bind (_direction _rotation) (`Timeline|Swing Closed` :!via `PlayFromStart`)
    (:`Update`
      (`SceneComponent.K2_SetRelativeRotation` _hinge (`KismetMathLibrary.RLerp` (struct) (.rotation (`SceneComponent.GetRelativeTransform` _hinge)) _rotation true) false false))))

(fn `UserConstructionScript`)
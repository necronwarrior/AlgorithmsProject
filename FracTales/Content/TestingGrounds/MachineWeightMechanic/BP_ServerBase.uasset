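; BP_ServerBase is an interactable server actor that opens and closes a task UI when the player clicks it.
; Every Tick it line-traces 250 units from above the player along the control rotation, toggling custom depth on its two meshes as an optional focus outline.
; PlayerClick calls ActivateServer, which either creates a BP_ServerWidgetBase initialized with ServerTasks and shows the cursor, or removes it and restores game-only input.
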(event `self.ReceiveTick`
  (params (DeltaSeconds :type "Float (single-precision)"))
  (`|ExecutionSequence`
    (:`then_0`
      (`self.OnFocus`))))

(event `PlayerClick`
  (`self.ActivateServer`))

(fn `ActivateServer`
  (bind _returnvalue (`GameplayStatics.GetPlayerController` 0))
  (if (`self.bServerActive`)
    (set `self.bServerActive` false)
    (`Widget.RemoveFromParent` (`self.ServerUIWidget`))
    (`WidgetBlueprintLibrary.SetInputMode_GameOnly` _returnvalue)
    (set `PlayerController.bShowMouseCursor` false _returnvalue)
    (else
      (set `self.bServerActive` true)
      (bind _returnvalue_2 (`|CreateWidget` "/Game/TestingGrounds/MachineWeightMechanic/BP_ServerWidgetBase.BP_ServerWidgetBase_C"))
      (bind _output_get (set `self.ServerUIWidget` _returnvalue_2))
      (`/Game/TestingGrounds/MachineWeightMechanic/BP_ServerWidgetBase.Initialize` _output_get (`self.ServerTasks`))
      (`UserWidget.AddToViewport` _output_get 0)
      (set `PlayerController.bShowMouseCursor` true (`GameplayStatics.GetPlayerController` 0)))))

(fn `OnFocus`
  (bind _returnvalue (`GameplayStatics.GetPlayerCharacter` 0))
  (bind _staticmesh1 (`self.StaticMesh1`))
  (bind _staticmesh (`self.StaticMesh`))
  (bind _returnvalue_2 (`KismetMathLibrary.MakeVector` (.x (`self.K2_GetActorLocation` _returnvalue)) (.y (`self.K2_GetActorLocation` _returnvalue)) (+ (.z (`self.K2_GetActorLocation` _returnvalue)) 50.0)))
  (bind _outhit (`KismetSystemLibrary.LineTraceSingle` :`Start` _returnvalue_2 :`End` (+ _returnvalue_2 (* (`KismetMathLibrary.GetForwardVector` (`Pawn.GetControlRotation` _returnvalue)) 250.0)) :`TraceChannel` "TraceTypeQuery1" :`bIgnoreSelf` false))
  (if (== (`.HitActor` (`GameplayStatics.BreakHitResult` _outhit)) self)
    (if (`self.bOutlineOnFocus`)
      (`PrimitiveComponent.SetRenderCustomDepth` _staticmesh1 true)
      (`PrimitiveComponent.SetRenderCustomDepth` _staticmesh true))
    (elif (`self.bOutlineOnFocus`)
      (`PrimitiveComponent.SetRenderCustomDepth` _staticmesh1 false)
      (`PrimitiveComponent.SetRenderCustomDepth` _staticmesh false))))

(fn `UserConstructionScript`)
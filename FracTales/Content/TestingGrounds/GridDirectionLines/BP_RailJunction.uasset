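; Rail junction node that moves the first-person player between linked junctions on a four-way movement network.
; The first point arms on player overlap; W maps junction-to-player yaw difference to one of four JunctionList slots.
; Tick interpolates player XY to that junction, faster inside its box, then snaps and calls its Arrived to hand over input.
; Older line-trace spline-rail logic remains, disconnected.
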(event `self.Box.OnComponentEndOverlap`
  (params (OverlappedComponent :type "PrimitiveComponent Object Reference") (OtherActor :type "Actor Object Reference") (OtherComp :type "PrimitiveComponent Object Reference") (OtherBodyIndex :type Integer)))

(event `Arrived`
  (`self.EnableInput` (`GameplayStatics.GetPlayerController` 0) :!label _label)
  (goto _label_2 :!via `Reset`))

(event `self.Box.OnComponentBeginOverlap`
  (params (OverlappedComponent :type "PrimitiveComponent Object Reference") (OtherActor :type "Actor Object Reference") (OtherComp :type "PrimitiveComponent Object Reference") (OtherBodyIndex :type Integer) (bFromSweep :type Boolean) (SweepResult :type "HitResult Structure (by ref)"))
  (if (`ActorComponent.ComponentHasTag` OtherComp "Player")
    (bind _asfirst_person_character (cast `/Game/TestingGrounds/FPTestingZone/Blueprints/FirstPersonCharacter` OtherActor))
    (set `self.PlayerCharacter` _asfirst_person_character)
    (if (`self.bIsFirstPoint?`)
      (goto _label))))

(event `Key|W`
  (params (Key :type "Key Structure" :default "AnyKey"))
  (bind _yaw (.yaw (`SceneComponent.K2_GetComponentRotation` (`self.DefaultSceneRoot`))))
  (bind _returnvalue (- _yaw (.yaw (`SceneComponent.K2_GetComponentRotation` (`Actor.RootComponent` (`self.PlayerCharacter`))))))
  (:`Pressed`
    (if (`KismetMathLibrary.InRange_FloatFloat` _returnvalue -135.0 -45.0 false)
      (if (!= (`|GetArrayItem` (`self.JunctionList`)) null)
        (set `self.JunctionPreChoice` 0)
        (`/Engine/EditorBlueprintResources/StandardMacros.DoOnce` false :!label _label_2
          (:`Completed`
            (set `self.JunctionChoice` (`self.JunctionPreChoice`))
            (`self.SetActorTickEnabled` true)))
        (else
          (`KismetSystemLibrary.PrintString` "0")))
      (elif (or (`KismetMathLibrary.InRange_FloatFloat` _returnvalue -180.0 -135.0) (`KismetMathLibrary.InRange_FloatFloat` _returnvalue 135.0 360.0))
        (if (!= (`|GetArrayItem` (`self.JunctionList`) 1) null)
          (set `self.JunctionPreChoice` 1)
          (goto _label_2)
          (else
            (`KismetSystemLibrary.PrintString` "1")))
        (elif (`KismetMathLibrary.InRange_FloatFloat` _returnvalue 45.0 135.0 true false)
          (if (!= (`|GetArrayItem` (`self.JunctionList`) 2) null)
            (set `self.JunctionPreChoice` 2)
            (goto _label_2)
            (else
              (`KismetSystemLibrary.PrintString` "2")))
          (elif (or (`KismetMathLibrary.InRange_FloatFloat` _returnvalue 0.0 45.0 true false) (`KismetMathLibrary.InRange_FloatFloat` _returnvalue -45.0 0.0 false))
            (if (!= (`|GetArrayItem` (`self.JunctionList`) 3) null)
              (set `self.JunctionPreChoice` 3)
              (goto _label_2)
              (else
                (`KismetSystemLibrary.PrintString` "3")))
            (else
              (`KismetSystemLibrary.PrintString` "oops")
              (`KismetSystemLibrary.PrintString` (`KismetStringLibrary.Conv_DoubleToString` _yaw))
              (`KismetSystemLibrary.PrintString` (`KismetStringLibrary.Conv_DoubleToString` _returnvalue)))))))))

(event `self.ReceiveBeginPlay`
  (`self.DisableInput` (`GameplayStatics.GetPlayerController` 0))
  (`self.SetActorTickEnabled` false))

(event `self.ReceiveTick`
  (params (DeltaSeconds :type "Float (single-precision)"))
  (bind _playercharacter (`self.PlayerCharacter`))
  (bind _returnvalue (`self.K2_GetActorLocation` _playercharacter))
  (bind _output (`|GetArrayItem` (`self.JunctionList`) (`self.JunctionChoice`)))
  (bind _returnvalue_2 (`self.K2_GetActorLocation` _output))
  (bind _z (.z (`self.K2_GetActorLocation` _playercharacter)))
  (bind _x (.x _returnvalue_2))
  (bind _y (.y _returnvalue_2))
  (bind _returnvalue_3 (`KismetMathLibrary.MakeVector` _x _y _z))
  (if (`PrimitiveComponent.IsOverlappingActor` (`/Game/TestingGrounds/GridDirectionLines/BP_RailJunction.Box` _output) _playercharacter)
    (if (and (`KismetMathLibrary.NearlyEqual_FloatFloat` _x (.x (`self.K2_GetActorLocation` _playercharacter)) 1.0) (`KismetMathLibrary.NearlyEqual_FloatFloat` _y (.y (`self.K2_GetActorLocation` _playercharacter)) 1.0))
      (`self.K2_SetActorLocation` _playercharacter (`KismetMathLibrary.MakeVector` (.x _returnvalue_2) (.y _returnvalue_2) _z) false false)
      (`self.SetActorTickEnabled` false)
      (`self.Arrived` _output)
      (set `self.bIsFirstPoint?` false)
      (`self.DisableInput` (`GameplayStatics.GetPlayerController` 0))
      (else
        (`self.K2_SetActorLocation` _playercharacter (`KismetMathLibrary.VInterpTo` _returnvalue _returnvalue_3 DeltaSeconds 10.0) false false)))
    (else
      (`self.K2_SetActorLocation` _playercharacter (`KismetMathLibrary.VInterpTo` _returnvalue _returnvalue_3 DeltaSeconds 5.0) false false))))

(fn `UserConstructionScript`)
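; BP_TaskListObjectTemplate is a template for world objects that represent ordered steps in the player's task list.
; On a player click it sets whether it is the next task by checking the previous entry in the passed completion array, with the first position always allowed, and stores the player character.
; TaskFinished then marks this object's position complete on that character.
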(event `PlayerClick`
  (params (TaskListComplete :type "Array of Boolean") (PlayerCharacter :type "/Game/TestingGrounds/FPTestingZone/Blueprints/FirstPersonCharacter Object Reference"))
  (bind _positionintasklist (`self.PositionInTaskList`))
  ;[1 1 1] Check that this task is the next task to perform - at least compared to the last task
  (`/Engine/EditorBlueprintResources/StandardMacros.CompareInt` _positionintasklist
    (:`>`
      (set `self.bIsNextTaskInLIst?` (`|GetArrayItem` TaskListComplete (- _positionintasklist 1))))
    (:`==`
      (set `self.bIsNextTaskInLIst?` true)))
  (set `self.PlayerCharacterReference` PlayerCharacter))

(event `TaskFinished`
  ;[1 1 1] When task is completed set its corresponding value in the player's checklist to true and change colour
  (`/Game/TestingGrounds/FPTestingZone/Blueprints/FirstPersonCharacter.SetTaskListComlpeteIndex` (`self.PlayerCharacterReference`) (`self.PositionInTaskList`)))

(fn `UserConstructionScript`)
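; BP_Day1Task5 is the fifth Day 1 task-list object, a pedalling mini-task completed by alternately pressing A and D.
; When clicked as the next task in the list, it disables the player's controls through the ControlStructure and enables its otherwise inactive Tick.
; Tick polls both keys, counting each alternation until ten, then updates the control structure, stops ticking, resets the count and calls TaskFinished.
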(event `self.ReceiveBeginPlay`
  (`self.SetActorTickEnabled` false))

(event `self.PlayerClick`
  (params (TaskListComplete :type "Array of Boolean (by ref)") (PlayerCharacter :type "/Game/TestingGrounds/FPTestingZone/Blueprints/FirstPersonCharacter Object Reference"))
  ;[1 1 1] Check If this is next task, space for any other checks
  (`parent.PlayerClick` TaskListComplete PlayerCharacter)
  (if (`self.bIsNextTaskInLIst?`)
    (setmembers `/Game/TestingGrounds/FPTestingZone/Blueprints/ControlsStructure` :`StructRef` (`/Game/TestingGrounds/FPTestingZone/Blueprints/FirstPersonCharacter.ControlStructure` PlayerCharacter) :`bIsLeftMouseButtonActive` false :`bIsInputAxisMoveForwardActive` false :`bIsInputAxisMoveRightActive` false :`bIsInputAxisTurnRateActive` false :`bIsInputAxisLookUpRateActive` false :`bIsInputActionJumpActive` false :`bIsXKeyActive` false :`bIsQKeyActive` false :`bIsInputActionFireActive` false :`bIsEKeyActive` false :`bIsInteractRadiusBeginOverlapActive` false :`bIsInteractRadiusEndOverlapActive` false :`bIs1KeyActive` false :`bIs2KeyActive` false :`bIs3KeyActive` false :`bIs4KeyActive` false :`bIs5KeyActive` false :`bIs6KeyActive` false :`bIs7KeyActive` false :`bIsUpActive` false :`bIsDownActive` false)
    ;[1 1 1] Conditions for finishing task
    (`self.SetActorTickEnabled` true)))

(event `self.ReceiveTick`
  (params (DeltaSeconds :type "Float (single-precision)"))
  (if (< (`self.PedalCount`) 10)
    (if (`self.bIsLeftKeyPedalling`)
      (if (`PlayerController.IsInputKeyDown` (`GameplayStatics.GetPlayerController` 0) "D")
        (set `self.bIsLeftKeyPedalling` false)
        (`/Engine/EditorBlueprintResources/StandardMacros.IncrementInt` (`self.PedalCount`)))
      (elif (`PlayerController.IsInputKeyDown` (`GameplayStatics.GetPlayerController` 0) "A")
        (set `self.bIsLeftKeyPedalling` true)
        (`/Engine/EditorBlueprintResources/StandardMacros.IncrementInt` (`self.PedalCount`))))
    (else
      (setmembers `/Game/TestingGrounds/FPTestingZone/Blueprints/ControlsStructure` :`StructRef` (`/Game/TestingGrounds/FPTestingZone/Blueprints/FirstPersonCharacter.ControlStructure` (stale `self.PlayerClick` PlayerCharacter)) :`bIsLeftMouseButtonActive` true :`bIsInputAxisMoveForwardActive` true :`bIsInputAxisMoveRightActive` true :`bIsInputAxisTurnRateActive` true :`bIsInputAxisLookUpRateActive` true :`bIsInputActionJumpActive` true :`bIsXKeyActive` true :`bIsQKeyActive` true :`bIsInputActionFireActive` true :`bIsEKeyActive` true :`bIsInteractRadiusBeginOverlapActive` true :`bIsInteractRadiusEndOverlapActive` true :`bIs1KeyActive` true :`bIs2KeyActive` true :`bIs3KeyActive` true :`bIs4KeyActive` true :`bIs5KeyActive` true :`bIs6KeyActive` true :`bIs7KeyActive` true :`bIsUpActive` true :`bIsDownActive` true)
      (`self.SetActorTickEnabled` false)
      (set `self.PedalCount` 0)
      (`self.TaskFinished`))))

(fn `UserConstructionScript`
  (`parent.UserConstructionScript`))
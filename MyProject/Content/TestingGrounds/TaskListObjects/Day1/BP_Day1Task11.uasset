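; BP_Day1Task11 is a clickable task object for Day 1 that moves the player on to a new task list.
; On PlayerClick it runs the parent logic, then proceeds only if this is the next task in the list.
; It then teleports the player to the referenced level spawn actor with zero rotation, calls WakingUp, finishes the task and calls ChangeTaskList on the player.
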(event `self.PlayerClick`
  (params (TaskListComplete :type "Array of Boolean (by ref)") (PlayerCharacter :type "/Game/TestingGrounds/FPTestingZone/Blueprints/FirstPersonCharacter Object Reference"))
  ;[1 1 1] Check If this is next task, space for any other checks
  (`parent.PlayerClick` TaskListComplete PlayerCharacter)
  (if (`self.bIsNextTaskInLIst?`)
    ;[1 1 1] Conditions for finishing task
    (`self.K2_TeleportTo` :`self` PlayerCharacter :`DestLocation` (`self.K2_GetActorLocation` (`self.LevelSpawnActorReference`)))
    (`/Game/TestingGrounds/FPTestingZone/Blueprints/FirstPersonCharacter.Waking up` PlayerCharacter)
    (`self.TaskFinished`)
    (`/Game/TestingGrounds/FPTestingZone/Blueprints/FirstPersonCharacter.Change Task List` PlayerCharacter)))

(fn `UserConstructionScript`
  (`parent.UserConstructionScript`))
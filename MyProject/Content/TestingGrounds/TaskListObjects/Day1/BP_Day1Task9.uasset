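; BP_Day1Task9 is the Day 1 Task 9 task-list object, a checklist the player must fully tick to finish the task.
; A click, when this is the next task in the list, shows the checklist widget and mouse cursor and disables player input.
; Tick is enabled only while the checklist is open, polling its checkboxes until all are checked, then removing the widget, restoring game input and calling TaskFinished.
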(event `self.ReceiveBeginPlay`
  (`self.SetActorTickEnabled` false))

(event `self.PlayerClick`
  (params (TaskListComplete :type "Array of Boolean (by ref)") (PlayerCharacter :type "/Game/TestingGrounds/FPTestingZone/Blueprints/FirstPersonCharacter Object Reference"))
  (bind _returnvalue (`GameplayStatics.GetPlayerController` 0))
  ;[1 1 1] Check If this is next task, space for any other checks
  (`parent.PlayerClick` TaskListComplete PlayerCharacter)
  (if (`self.bIsNextTaskInLIst?`)
    ;[1 1 1] Conditions for finishing task
    (bind _returnvalue_2 (`|CreateWidget` "/Game/TestingGrounds/TaskListObjects/Day1/Day1Task9Extras/BP_Day1Task9Checklist.BP_Day1Task9Checklist_C" _returnvalue))
    (bind _output_get (set `self.Day1Task9ChecklistWidgetInstance` _returnvalue_2))
    (`UserWidget.AddToViewport` _output_get 0)
    (set `PlayerController.bShowMouseCursor` true _returnvalue)
    (`self.DisableInput` PlayerCharacter _returnvalue)
    (`self.SetActorTickEnabled` true)))

(event `self.ReceiveTick`
  (params (DeltaSeconds :type "Float (single-precision)"))
  (bind _returnvalue (`GameplayStatics.GetPlayerController` 0))
  (set `self.bIsAllCheckBoxesChecked` true)
  (for _array_element (`/Game/TestingGrounds/TaskListObjects/Day1/Day1Task9Extras/BP_Day1Task9Checklist.CheckBoxArray` (`self.Day1Task9ChecklistWidgetInstance`))
    (if (not (`CheckBox.IsChecked` _array_element))
      (set `self.bIsAllCheckBoxesChecked` false)))
  (if (`self.bIsAllCheckBoxesChecked`)
    (set `PlayerController.bShowMouseCursor` false _returnvalue)
    (`self.EnableInput` (stale `self.PlayerClick` PlayerCharacter) _returnvalue)
    (`Widget.RemoveFromParent` (`self.Day1Task9ChecklistWidgetInstance`))
    (`self.SetActorTickEnabled` false)
    (`WidgetBlueprintLibrary.SetInputMode_GameOnly` _returnvalue)
    (`self.TaskFinished`)))

(fn `UserConstructionScript`
  (`parent.UserConstructionScript`))
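; BP_TaskList01 is a test task list that stores a three-way material choice and applies it to an object's cube.
; The Option0 choice events each pick a yellow, blue or black material and write it to a newly created CurrentSaveGame, saved to that class's default slot.
; ExecuteTaskList loads that slot and sets the saved material on the AttachedCube of the BP_ObjectWithTaskList01 passed as parent.
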(event `self.ExecuteTaskList`
  (params (`Parent Reference` :type "Actor Object Reference"))
  (bind _returnvalue (`GameplayStatics.CreateSaveGameObject` "/Game/TestingGrounds/CurrentSaveGame.CurrentSaveGame_C"))
  (bind _returnvalue_2 (`GameplayStatics.LoadGameFromSlot` (`/Game/TestingGrounds/CurrentSaveGame.SaveSlotName` _returnvalue) (`/Game/TestingGrounds/CurrentSaveGame.UserIndex` _returnvalue)))
  (bind _ascurrent_save_game (cast `/Game/TestingGrounds/CurrentSaveGame` _returnvalue_2))
  (bind _asbp_object_with_task_list_01 (cast `/Game/TestingGrounds/Mechanic1/TestNPC/BP_ObjectWithTaskList01` `Parent Reference`))
  (`PrimitiveComponent.SetMaterial` (`/Game/TestingGrounds/Mechanic1/TestNPC/BP_ObjectWithTaskList01.AttachedCube` _asbp_object_with_task_list_01) 0 (`/Game/TestingGrounds/CurrentSaveGame.ObjectTestOption0` _ascurrent_save_game)))

(event `self.Option0Choice0`
  (params (Parent :type "Actor Object Reference"))
  (set `self.MaterialTest` "/Game/DepricatedFeatures/CircuitMiniGame/YELLOW_Depthless.YELLOW_Depthless")
  (bind _returnvalue (`GameplayStatics.CreateSaveGameObject` "/Game/TestingGrounds/CurrentSaveGame.CurrentSaveGame_C" :!label _label))
  (set `/Game/TestingGrounds/CurrentSaveGame.ObjectTestOption0` (`self.MaterialTest`) _returnvalue)
  (`GameplayStatics.SaveGameToSlot` _returnvalue (`/Game/TestingGrounds/CurrentSaveGame.SaveSlotName` _returnvalue) (`/Game/TestingGrounds/CurrentSaveGame.UserIndex` _returnvalue)))

(event `self.Option0Choice1`
  (params (Parent :type "Actor Object Reference"))
  (set `self.MaterialTest` "/Game/DepricatedFeatures/CircuitMiniGame/BLUE_Depthless.BLUE_Depthless")
  (goto _label))

(event `self.Option0Choice2`
  (params (Parent :type "Actor Object Reference"))
  (set `self.MaterialTest` "/Game/DepricatedFeatures/CircuitMiniGame/BLACK_Depthless.BLACK_Depthless")
  (goto _label))
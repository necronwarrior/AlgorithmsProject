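; BP_CircuitBoardTemplate is a template actor for a circuit board minigame that presents itself to the player's camera.
; On BeginPlay it shows the cursor, disables player character input, stores its start position and takes the negated player rotation.
; Tick lerps it from that start toward the camera location, with the forward offset zeroed out.
; The lerp alpha is accumulated delta time, never clamped, so it passes the target after one second.
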(event `self.ReceiveBeginPlay`
  (bind _returnvalue (`GameplayStatics.GetPlayerController` 0))
  (set `PlayerController.bShowMouseCursor` true _returnvalue)
  (`self.DisableInput` (`GameplayStatics.GetPlayerCharacter` 0) _returnvalue)
  (set `self.StartingPosition` (`self.K2_GetActorLocation`))
  (`self.K2_SetActorRotation` (`KismetMathLibrary.NegateRotator` (`self.K2_GetActorRotation` (`GameplayStatics.GetPlayerCharacter` 0)))))

(event `self.ReceiveTick`
  (params (DeltaSeconds :type "Float (single-precision)"))
  (bind _returnvalue (`GameplayStatics.GetPlayerCameraManager` 0))
  (set `self.LerpDeltaTime` (+ DeltaSeconds (`self.LerpDeltaTime`)))
  (`self.K2_SetActorLocation` (`KismetMathLibrary.VLerp` (`self.StartingPosition`) (+ (`self.K2_GetActorLocation` _returnvalue) (* (`self.GetActorForwardVector` _returnvalue) 0.0)) (`self.LerpDeltaTime`))))

(fn `UserConstructionScript`)